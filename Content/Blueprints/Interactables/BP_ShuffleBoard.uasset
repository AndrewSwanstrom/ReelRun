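; Interactable shuffleboard that slides its puck to a random target on interact and resets it on the next press.
; Overlapping Box1 shows the interact icon, applies an outline overlay material and enables input; leaving clears the highlight and calls DisableInput.
; A FlipFlop alternates the throw and reset, with a DoOnce guarding the throw.
; A timeline lerps the puck from its BeginPlay position to one of nine targets.
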(event OnComponentBeginOverlap(Box1)
  (params (OverlappedComponent :type Primitive%20Component%20Object%20Reference) (OtherActor :type Actor%20Object%20Reference) (OtherComp :type Primitive%20Component%20Object%20Reference) (OtherBodyIndex :type Integer) (bFromSweep :type Boolean) (SweepResult :type Hit%20Result%20Structure%20%28by%20ref%29))
  (Variables|Default|SetbInRange true)
  (Rendering|SetVisibility (Variables|Default|GetInteractIcon) true false)
  (Rendering|Material|SetOverlayMaterial (Variables|Default|GetStaticMesh) "/Game/Materials/OutlineMat/Mi_OutlineMat_Inst.Mi_OutlineMat_Inst" :!class /Script/Engine.MeshComponent)
  (Input|EnableInput (Game|GetPlayerController 0)))

(event OnComponentEndOverlap(Box1)
  (params (OverlappedComponent :type Primitive%20Component%20Object%20Reference) (OtherActor :type Actor%20Object%20Reference) (OtherComp :type Primitive%20Component%20Object%20Reference) (OtherBodyIndex :type Integer))
  (Variables|Default|SetbInRange false)
  (Rendering|SetVisibility (Variables|Default|GetInteractIcon) false false)
  (Rendering|Material|SetOverlayMaterial (Variables|Default|GetStaticMesh) 0 :!class /Script/Engine.MeshComponent)
  (Input|DisableInput (Game|GetPlayerController 0) 0))

(event Input|EnhancedActionEvents|EnhancedInputActionIA_Interact
  (params (ActionValue :type Boolean) (ElapsedSeconds :type Float%20%28double-precision%29) (TriggeredSeconds :type Float%20%28double-precision%29) (InputAction :type Input%20Action%20Object%20Reference :default "/Game/Blueprints/Input/Actions/IA_Interact.IA_Interact"))
  (Utilities|FlowControl|FlipFlop
    (:A
      (Utilities|FlowControl|DoOnce false :!label _label
        (:Completed
          (Variables|Default|SetEndVector (.OutItem (Utilities|Array|Random (Utilities|Array|MakeArray (Variables|Default|GetTarget7) (Variables|Default|GetTarget1) (Variables|Default|GetTarget8) (Variables|Default|GetTarget6) (Variables|Default|GetTarget5) (Variables|Default|GetTarget2) (Variables|Default|GetTarget) (Variables|Default|GetTarget3) (Variables|Default|GetTarget4)))))
          (bind _move_actor_timeline (Timeline|Timeline_0 PlayFromStart)
            (:Update
              (Transformation|SetWorldLocation (Variables|Default|GetPuck) (Math|Vector|Lerp(Vector) (Variables|Default|GetStartVector) (Transformation|GetWorldLocation (Variables|Default|GetEndVector)) _move_actor_timeline) false false))))))
    (:B
      (Transformation|SetWorldLocation (Variables|Default|GetPuck) (Variables|Default|GetStartVector) false false)
      (goto _label Reset))))

(event EventBeginPlay
  (Variables|Default|SetStartVector (Transformation|GetWorldLocation (Variables|Default|GetPuck))))

(event EventTick
  (params (DeltaSeconds :type Float%20%28single-precision%29))
  (CallFunction|WidgetLookat (Variables|Default|GetInteractIcon) (Variables|Default|GetbInRange)))

(fn ConstructionScript
  (|CallParentFunction))