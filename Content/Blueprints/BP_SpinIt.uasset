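; BP_SpinIt is an actor the player can spin with the mouse by hovering over it and clicking.
; Once clicked, Tick turns mouse delta into world pitch and yaw rotation until the cursor leaves.
; Cursor exit clears both flags and plays the RotateActor timeline, easing the actor toward ActorDefaultTransform.
; The node capturing that transform is unwired, so the variable is never set at runtime; debug prints remain.
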(event EventTick
  (params (DeltaSeconds :type Float%20%28single-precision%29))
  (bind _returnvalue (Game|GetPlayerController 0))
  (bind (_deltax _deltay) (Class|PlayerController|GetInputMouseDelta _returnvalue))
  (if (Variables|Default|GetHovered)
    (if (Variables|Default|GetClicked)
      (Class|Actor|AddActorWorldRotation (Math|Rotator|MakeRotator 0.0 (* _deltay -1e+01) (* _deltax -1e+01))))))

(event MouseInput|EventActorBeginCursorOver
  (Variables|Default|SetHovered true)
  (Development|PrintString "H"))

(event MouseInput|EventActorEndCursorOver
  (Variables|Default|SetHovered false)
  (Variables|Default|SetClicked false)
  (Development|PrintString "UH")
  (bind _actor_rotate (Timeline|Rotate%20Actor PlayFromStart)
    (:Update
      (Transformation|SetActorTransform (Math|Transform|Lerp(Transform) (Transformation|GetActorTransform) (Variables|Default|GetActorDefaultTransform) _actor_rotate)))))

(event MouseInput|EventActorOnClicked
  (params (ButtonPressed :type Key%20Structure :default "None"))
  (bind _output_get (Variables|Default|SetClicked true))
  (Development|PrintString (Utilities|String|ToString(Boolean) _output_get)))

(fn ConstructionScript)