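; Destructible tombstone prop built from geometry collection components for base, body, top and plate.
; On BeginPlay it applies a slight random tilt to the base around a 90-degree yaw, resets TopTransform and destroys the top piece.
; Unconnected graphs hold a randomizer that swaps rest collections or removes pieces for tombstone variants, plus a node to re-add a collection at TopTransform, but neither runs.
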(event EventBeginPlay
  (Utilities|FlowControl|DoOnce false
    (:Completed
      (Transformation|SetRelativeRotation (Variables|Default|GetGC_SM_CBase_01) (Math|Rotator|MakeRotator (Math|Conversions|ToFloat(Integer) (Math|Random|RandomIntegerinRange -5 5)) (Math|Conversions|ToFloat(Integer) (Math|Random|RandomIntegerinRange -5 5)) (+ (Math|Conversions|ToFloat(Integer) (Math|Random|RandomIntegerinRange -5 5)) 9e+01)) false false)
      (bind _output_get (Variables|Default|SetTop_Transform ""))
      (Components|DestroyComponent (Variables|Default|GetGC_SM_CTop_01)))))

(fn ConstructionScript)