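; Heavy enemy character that chases and punches, with AI combat ranges, walk speeds and a proximity check against other Heavies.
; Tick turns it toward the player during attacks, sets speed and runs flag-driven socket traces for right-fist hits and knockback.
; Damage plays hit feedback, takes knockback force from the causer, drives a timeline push alongside blackboard state changes, then subtracts health and destroys it at zero.
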(event EventBeginPlay
  (Utilities|Array|Add (Variables|Default|GetHeavyIgnore) self))

(event Collision|EventActorBeginOverlap
  (params (OtherActor :type Actor%20Object%20Reference))
  (|CallParentFunction OtherActor) ; This node is disabled and will not be called.\nDrag off pins to build functionality.
)

(event Game|Damage|EventAnyDamage
  (params (Damage :type Float%20%28single-precision%29) (DamageType :type Damage%20Type%20Object%20Reference) (InstigatedBy :type Controller%20Object%20Reference) (DamageCauser :type Actor%20Object%20Reference))
  (bind _self self)
  ;[1 0.1892 0.4635] dmg
  (Audio|PlaySoundatLocation "/Game/Art/SFX/RandomHitCue.RandomHitCue" (Transformation|GetActorLocation) "0, 0, 0" 1.0 (Math|Random|RandomFloatinRange 0.5 1.3) 0.0 0 0 0 0)
  ;;[1 1 1] show dmg numbers?
  (if (Variables|Default|GetShowDmgNums?)
    (Game|SpawnActorfromClass "/Game/Art/VFX/Blood_And_Nums/DamageNumbers/BP_DmgNum.BP_DmgNum_C" (Transformation|GetActorTransform _self) "Undefined" "MultiplyWithRoot" _self (* Damage 1e+01) "(R=0.000000,G=0.000000,B=0.000000,A=0.000000)" 0))
  ;[1 0.3318 0.08999] init knockback
  (bind _asbase_character (Utilities|Casting|CastToBase_Character DamageCauser)
    (:then
      (Variables|Default|SetCustom%20Knockback%20Force (Variables|/Game/Blueprints/Characters/Base_Character.Base_Character_C|GetKnockBackForce _asbase_character))
      ;[1 1 1] is dmg causer syd
      (if (Variables|/Game/Blueprints/Characters/Base_Character.Base_Character_C|GetSyd _asbase_character)
        (AddComponent|AddNiagaraComponent false)))
    (:CastFailed
      (bind _asbp_throwable_base_obj (Utilities|Casting|CastToBP_ThrowableBaseObj DamageCauser)
        (:then
          (Variables|Default|SetCustom%20Knockback%20Force (Variables|/Game/Blueprints/Throwables/BP_ThrowableBaseObj.BP_ThrowableBaseObj_C|GetThrowableKnockback _asbp_throwable_base_obj)))
        (:CastFailed
          (Variables|Default|SetCustom%20Knockback%20Force 9e+02)))))
  ;[1 0.239 0.2291] hurt anim
  (Animation|Montage|PlayMontage (Variables|Character|GetMesh) "/Game/Art/Characters/Enemies/Heavy/Animations/Montage/Anim_HeavyEnemyDamage_Montage.Anim_HeavyEnemyDamage_Montage"
    (:then
      ;[1 0.3471 0.7164] Knock Back
      (CallFunction|EnemyKnockback)
      (bind _alpha (Timeline|Timeline_0 PlayFromStart)
        (:Update
          (if (== (Variables|Default|GetCustomTimeDilation) 1.0)
            (CallFunction|StartKnockBack _alpha (Variables|Default|GetCustom%20Knockback%20Force))))
        (:Finished
          (Utilities|FlowControl|Delay 0.2)
          (Variables|Default|SetIsOverlapping false)
          (CallFunction|KnockBackState (AI|GetBlackboard (AI|GetAIController self)) (Variables|Default|GetKey) (Utilities|Enum|LiteralenumLightEnemy "NewEnumerator0"))
          ;[1 0.3075 0.4888] decrease health
          (bind _output_get (Variables|Default|SetHealth (- (Variables|Default|GetHealth) Damage)))
          (if (<= _output_get 0.0)
            (Utilities|FlowControl|Delay 0.2)
            (Actor|DestroyActor)))))))

(event EventTick
  (params (DeltaSeconds :type Float%20%28single-precision%29))
  ;[0.8655 0.4491 1] Event Tick
  (if (Variables|Default|GetRotateAttack)
    (CallFunction|RotateTowardsPlayer))
  (if (Variables|Default|GetStopWalk)
    (CallFunction|SetMovementSpeed "NewEnumerator0")
    (else
      (CallFunction|SetMovementSpeed "NewEnumerator1")))
  (if (Variables|Default|GetIsOverlapping)
    (CallFunction|KnockBackTrace (Variables|Character|GetMesh) (Variables|Default|GetTraceStart) (Variables|Default|GetTraceEnd) 0.0)
    (elif (Variables|Default|GetRightFistAttack)
      (bind _output_get (Variables|Default|SetSocketStart "RightHandStart"))
      (bind _output_get_2 (Variables|Default|SetSocketEnd "RightHandEnd"))
      (CallFunction|AttackTrace (Variables|Character|GetMesh) _output_get _output_get_2 3e+01 1e+03 self 1e+01 "/Game/Art/SFX/InGame/ER_WoodBreaking.ER_WoodBreaking")
      (elif (Variables|Default|GetWalkTrace)
        (CallFunction|KnockBackTrace (Variables|Character|GetMesh) (Variables|Default|GetTraceStart) (Variables|Default|GetTraceEnd) 5e+01 "/Game/Art/SFX/InGame/ER_WoodBreaking.ER_WoodBreaking")))))

(event Custom|RotateTowardsPlayer
  (bind _returnvalue (Transformation|GetActorRotation))
  ;[1 0.3105 0.6202] More Accurate Attack
  (Transformation|SetActorRotation (Math|Rotator|MakeRotator (.roll _returnvalue) (.pitch _returnvalue) (.yaw (Math|Rotator|FindLookatRotation (Transformation|GetActorLocation) (Transformation|GetActorLocation (Game|GetPlayerCharacter 0)))))))

(event Custom|Detection
  ;[0.4419 1 0.3749] Detect if too close to Heavy Enemies
  (bind _returnvalue (Collision|SphereOverlapActors (Transformation|GetActorLocation) 8e+01 (Utilities|Array|MakeArray "ObjectTypeQuery3") "BP_Heavy_C" (Variables|Default|GetHeavyIgnore)))
  (if _returnvalue
    (Variables|Default|SetShouldAdjust true)
    (else
      (Variables|Default|SetShouldAdjust false))))

(event Custom|ResetSoundHeavy
  ;[1 0.739 0.3229] Reset Break Sound
  (Variables|Default|SetBreakSound false))

(event Custom|ClearAttackStackHeavy
  ;[1 0.3181 0.5308] Clear Attack Stack
  (Utilities|Array|Clear (Variables|Default|GetActorsIgnore)))

(event Custom|EnemyKnockback
  ;[1 0.9856 0.3176] Force Enemy Into Knock Back State
  (CallFunction|KnockBackState (AI|GetBlackboard (AI|GetAIController self)) (Variables|Default|GetKey) (Utilities|Enum|LiteralenumLightEnemy "NewEnumerator8")))

(event Custom|AttackAnim
  ;[1 0.3153 0.4658] Attack Anim
  (Animation|Montage|PlayMontage (Variables|Character|GetMesh) "/Game/Art/Characters/Enemies/Heavy/Animations/Montage/Anim_HeavyEnemyAttack_Montage.Anim_HeavyEnemyAttack_Montage"
    (:OnCompleted
      _)
    (:OnInterrupted
      _))
  (Default|CallOnAttackEnd))

(fn ConstructionScript
  (|CallParentFunction))

(fn AttackStart
  (params (AttackTarget :type Actor%20Object%20Reference) (Tokens%20Needed :type Integer))
  (return false))

(fn GetIdealRange
  (return 2e+02 3.5e+02 6e+02))

(fn SetMovementSpeed
  (params (Speed :type E_MovementSpeed%20Enum :default "NewEnumerator0"))
  (bind _output_get (Variables|/Script/Engine.CharacterMovementComponent|SetMaxWalkSpeed (Variables|Character|GetCharacterMovement) (Utilities|Select :Index Speed :NewEnumerator0 0.0 :NewEnumerator1 (Math|Random|RandomFloatinRange 125.0 1.5e+02) :NewEnumerator2 5e+02)))
  (return _output_get))