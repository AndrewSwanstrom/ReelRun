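; Cemetery torch light that can flicker and switch off when a character enters its trigger sphere.
; TurnOff allows this on any overlap, while TurnOff2ndTime delays it until a later overlap, with the first counted before the character cast.
; A one-shot timeline drives point light intensity, then swaps the path light mesh to the lights-off material when finished.
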(event OnComponentBeginOverlap(Sphere)
  (params (OverlappedComponent :type Primitive%20Component%20Object%20Reference) (OtherActor :type Actor%20Object%20Reference) (OtherComp :type Primitive%20Component%20Object%20Reference) (OtherBodyIndex :type Integer) (bFromSweep :type Boolean) (SweepResult :type Hit%20Result%20Structure%20%28by%20ref%29))
  (if (Variables|Default|GetTurnOff?)
    (Utilities|Casting|CastToBase_Character OtherActor :!label _label)
    (Utilities|FlowControl|DoOnce false
      (:Completed
        (bind _light_flicker (Timeline|Light%20Flicker PlayFromStart)
          (:Update
            (Rendering|Components|Light|SetIntensity (Variables|Default|GetPointLight) _light_flicker))
          (:Finished
            (Rendering|Material|SetMaterial (Variables|Default|GetSM_PathLight) 0 "/Game/Materials/Instances/MI_HorrorLightsOff.MI_HorrorLightsOff")))))
    (elif (Variables|Default|Get2ndTime)
      (if (Variables|Default|GetTurnOff2ndTime?)
        (goto _label))
      (else
        (Variables|Default|Set2ndTime true)))))

(fn ConstructionScript)