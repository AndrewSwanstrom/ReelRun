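; Ranged shooter enemy that spawns a handgun in its hand and fires at the player through an attack montage.
; A Niagara color parameter and flash timeline telegraph aiming before bullets spawn.
; Damage plays a hit reaction, sets a Blackboard knockback state while a timeline applies causer-specific force, and destroys enemy and gun at zero health.
; AI-facing functions supply ideal ranges and walk speed; the beam trace logic is disconnected.
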(event Custom|ShooterKnockBack
  ;[1 1 1] Force Shooter to Knockback
  (CallFunction|KnockBackState (AI|GetBlackboard (AI|GetAIController self)) (Variables|Default|GetKey) (Utilities|Enum|LiteralenumLightEnemy "NewEnumerator8")))

(event Custom|OnMontageEnded_Event
  (params (Montage :type Anim%20Montage%20Object%20Reference) (bInterrupted :type Boolean))
  (if (== Montage "/Game/Art/Characters/Enemies/Shooter/Animations/Montage/Anim_ShooterAttack_Montage.Anim_ShooterAttack_Montage")
    (Audio|Components|Audio|Stop (Variables|Default|GetWarningFlash))
    (Niagara|SetNiagaraVariable(LinearColor) (Variables|Default|GetNiagara) "Color" (Utilities|Struct|MakeLinearColor 0.0 0.0 0.0 0.0))))

(event Custom|EventAttack
  ;[1 1 1] Shoot Player
  (if (Variables|Default|GetStartStopShooting)
    (bind _notifyname (Animation|Montage|PlayMontage (Variables|Character|GetMesh) "/Game/Art/Characters/Enemies/Shooter/Animations/Montage/Anim_ShooterAttack_Montage.Anim_ShooterAttack_Montage")
      (:OnCompleted
        (Default|CallOnShootEnd :!label _label))
      (:OnInterrupted
        (goto _label))
      (:OnNotifyBegin
        (switch name _notifyname)))))

(event Custom|NormalSpeed)

(event Custom|BulletSpawn
  ;[1 1 1] Spawn Bullet
  (Audio|Components|Audio|Stop (Variables|Default|GetWarningFlash))
  (CallFunction|Bullet self (Variables|Default|GetFlash) (Variables|Character|GetMesh))
  (Niagara|SetNiagaraVariable(LinearColor) (Variables|Default|GetNiagara) "Color" (Utilities|Struct|MakeLinearColor 0.0 0.0 0.0 0.0)))

(event Custom|AimWarning
  (bind _redchannelfloat (Timeline|WarningFlash PlayFromStart)
    (:Update
      (Niagara|SetNiagaraVariable(LinearColor) (Variables|Default|GetNiagara) "Color" (Utilities|Struct|MakeLinearColor _redchannelfloat 0.0 0.0 1.0)))))

(event Custom|TakeAim
  ;[1 1 1] Slow Aim animation down and turn laser on
  (Niagara|SetNiagaraVariable(LinearColor) (Variables|Default|GetNiagara) "Color" (Utilities|Struct|MakeLinearColor 1.0 0.1 0.1 1.0)))

(event Game|Damage|EventAnyDamage
  (params (Damage :type Float%20%28single-precision%29) (DamageType :type Damage%20Type%20Object%20Reference) (InstigatedBy :type Controller%20Object%20Reference) (DamageCauser :type Actor%20Object%20Reference))
  (bind _self self)
  ;[1 1 1] Take Damage & Knockback
  (Audio|PlaySoundatLocation "/Game/Art/SFX/RandomHitCue.RandomHitCue" (Transformation|GetActorLocation) "0, 0, 0" 1.0 (Math|Random|RandomFloatinRange 0.5 1.3) 0.0 0 0 0 0)
  ;;[1 1 1] show dmg numbers?
  (if (Variables|Default|GetShowDmgNums?)
    (Game|SpawnActorfromClass "/Game/Art/VFX/Blood_And_Nums/DamageNumbers/BP_DmgNum.BP_DmgNum_C" (Transformation|GetActorTransform _self) "Undefined" "MultiplyWithRoot" _self Damage "(R=0.000000,G=0.000000,B=0.000000,A=0.000000)" 0))
  ;;[1 1 1] is dmg causer syd
  (if (== (Utilities|String|StringToName (Utilities|GetDisplayName DamageCauser)) "BP_Syd0")
    (AddComponent|AddNiagaraComponent false))
  (Animation|Montage|PlayMontage (Variables|Character|GetMesh) "/Game/Art/Characters/Enemies/Shooter/Animations/Montage/Anim_ShooterDamage_Montage.Anim_ShooterDamage_Montage"
    (:then
      (bind _asbase_character (Utilities|Casting|CastToBase_Character DamageCauser)
        (:then
          (Variables|Default|SetCustomKnockBackForce (Variables|/Game/Blueprints/Characters/Base_Character.Base_Character_C|GetKnockBackForce _asbase_character)))
        (:CastFailed
          (bind _asbp_throwable_base_obj (Utilities|Casting|CastToBP_ThrowableBaseObj DamageCauser)
            (:then
              (Variables|Default|SetCustomKnockBackForce (Variables|/Game/Blueprints/Throwables/BP_ThrowableBaseObj.BP_ThrowableBaseObj_C|GetThrowableKnockback _asbp_throwable_base_obj)))
            (:CastFailed
              (Variables|Default|SetCustomKnockBackForce 9e+02)))))
      (Utilities|FlowControl|Sequence
        (:then_0
          (CallFunction|ShooterKnockBack)
          (bind _alpha (Timeline|Timeline PlayFromStart)
            (:Update
              (if (== (Variables|Default|GetCustomTimeDilation) 1.0)
                (CallFunction|StartKnockBack _alpha (Variables|Default|GetCustomKnockBackForce))))
            (:Finished
              (Utilities|FlowControl|Delay 0.2)
              (Variables|Default|SetIsOverlapping false)
              (CallFunction|KnockBackState (AI|GetBlackboard (AI|GetAIController self)) (Variables|Default|GetKey) (Utilities|Enum|LiteralenumLightEnemy "NewEnumerator0")))))
        (:then_1
          (bind _output_get (Variables|Default|SetHealth (- (Variables|Default|GetHealth) Damage)))
          (if (<= _output_get 0.0)
            (Actor|DestroyActor)
            (Actor|DestroyActor (Variables|Default|GetGunBP_Ref))))))
    (:OnCompleted
      (Development|PrintString "Shooter: OW!"))))

(event EventTick
  (params (DeltaSeconds :type Float%20%28single-precision%29))
  ;[1 1 1] Event Tick KnockBack
)

(event EventBeginPlay
  ;[1 1 1] Spawn Gun in Enemy Hand
  (EventDispatchers|AssignOnMontageEnded (Components|SkeletalMesh|GetAnimInstance (Variables|Character|GetMesh)) (delegate Custom|OnMontageEnded_Event))
  (bind _asbase_character (Utilities|Casting|CastToBase_Character (Game|Player|GetPlayerPawn 0)))
  (Variables|Default|SetChar%20Ref _asbase_character)
  (bind _returnvalue (Game|SpawnActorfromClass (Variables|Default|GetHandGunRef) (Transformation|GetSocketTransform (Variables|Character|GetMesh) "Gun" "RTS_World") "Undefined" "MultiplyWithRoot" 0 0))
  (bind _output_get (Variables|Default|SetGunBP_Ref _returnvalue))
  (Transformation|AttachComponentToComponent _output_get (Variables|Character|GetMesh) "Gun" "SnapToTarget" "SnapToTarget" "SnapToTarget" true))

(fn ConstructionScript)

(fn ShootatPlayer
  (bind _self self)
  (bind _returnvalue (Transformation|GetActorTransform _self))
  (bind _returnvalue_2 (Game|SpawnActorfromClass "/Game/Blueprints/Damaging/BP_Damager.BP_Damager_C" (Math|Transform|MakeTransform (+ (+ (* (Transformation|GetActorForwardVector _self) 1e+02) (.location _returnvalue)) "0.000000,0.000000,50.000000") (.rotation _returnvalue) (.scale _returnvalue)) "Undefined" "MultiplyWithRoot" 0 0))
  (Rendering|SetVisibility (Variables|Default|GetFlash) false false)
  (Niagara|SpawnSystemAttached "/Game/Art/VFX/NS_MuzzleFlash.NS_MuzzleFlash" 0 "None" "0.000000,35.000000,10.000000" "0.000000,45.000000,0.000000" "KeepRelativeOffset" false)
  (bind _asbp_betsy (Utilities|Casting|CastToBP_Betsy (Game|Player|GetPlayerPawn 0)))
  (Physics|AddImpulse (Variables|/Game/Blueprints/Damaging/BP_Damager.BP_Damager_C|GetCollider _returnvalue_2) (* (Math|Vector|GetUnitDirection(Vector) (+ (Transformation|GetActorLocation self) "0.000000,0.000000,50.000000") (Transformation|GetActorLocation _asbp_betsy)) 1e+03) "None" true))

(fn AttackStart
  (params (AttackTarget :type Actor%20Object%20Reference) (Tokens%20Needed :type Integer))
  (return false))

(fn GetIdealRange
  (return 1.5e+03 3e+02 0.0))

(fn SetMovementSpeed
  (params (Speed :type E_MovementSpeed%20Enum :default "NewEnumerator0"))
  (bind _output_get (Variables|/Script/Engine.CharacterMovementComponent|SetMaxWalkSpeed (Variables|Character|GetCharacterMovement) (Utilities|Select :Index Speed :NewEnumerator0 0.0 :NewEnumerator1 2.5e+02 :NewEnumerator2 5e+02 :NewEnumerator4 0.0)))
  (return _output_get))