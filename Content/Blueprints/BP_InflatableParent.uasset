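; Parent Blueprint for inflatable physics props that react to characters hitting or damaging them.
; Damage caused by a Base_Character applies a Z-only impulse to the Sphere, computed from its up vector multiplied by its world location, so strength varies with height.
; A hit from a Base_Character prints a debug "bounce" message and plays a non-spatial light-damage sound, without adding force.
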(event Game|Damage|EventAnyDamage
  (params (Damage :type Float%20%28single-precision%29) (DamageType :type Damage%20Type%20Object%20Reference) (InstigatedBy :type Controller%20Object%20Reference) (DamageCauser :type Actor%20Object%20Reference))
  (bind _self self)
  (bind _sphere (Variables|Default|GetSphere _self))
  (Utilities|Casting|CastToBase_Character DamageCauser)
  (Physics|AddImpulse _sphere (* (* (Math|Vector|GetUpVector _sphere) (Transformation|GetWorldLocation _sphere)) "0.000000,0.000000,300.000000") "None" false))

(event Collision|EventHit
  (params (MyComp :type Primitive%20Component%20Object%20Reference) (Other :type Actor%20Object%20Reference) (OtherComp :type Primitive%20Component%20Object%20Reference) (bSelfMoved :type Boolean) (HitLocation :type Vector :default "0, 0, 0") (HitNormal :type Vector :default "0, 0, 0") (NormalImpulse :type Vector :default "0, 0, 0") (Hit :type Hit%20Result%20Structure%20%28by%20ref%29))
  (Utilities|Casting|CastToBase_Character Other)
  (Development|PrintString "bounce")
  (Audio|PlaySound2D "/Game/Art/Voiceover/Goons/Light/ER_LightDamage_3.ER_LightDamage_3" 1.0 1.0 0.0 0 self))

(fn ConstructionScript)