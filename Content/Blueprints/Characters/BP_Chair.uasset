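; BP_Chair is a playable chair character for melee combat, built on a parent class that supplies most of the logic.
; It sets damage and health, flags the horror level, and passes Enhanced Input to inherited movement, dash, interact and three-montage light and heavy attack functions with chair-specific assets.
; Tick drives the camera boom and target lock with FOV changes, plus an electric mesh overlay at high combo counts.
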(event Input|EnhancedActionEvents|EnhancedInputActionIA_Dash
  (params (ActionValue :type Boolean) (ElapsedSeconds :type Float%20%28double-precision%29) (TriggeredSeconds :type Float%20%28double-precision%29) (InputAction :type Input%20Action%20Object%20Reference :default "/Game/Blueprints/Input/Actions/IA_Dash.IA_Dash"))
  ;[1 1 1] dash
  (:Started
    (CallFunction|Dash 0.3 1.0 "/Game/Art/Characters/Syd/Animations/MontageTypeShii/AM_SydDash.AM_SydDash" 1.0 (Variables|Default|GetCapsuleComponent) "/Game/Art/VFX/NS_Punch.NS_Punch" "/Game/Art/SFX/Wooshes/SW_WooshSlow1.SW_WooshSlow1" (Variables|Default|GetSpeedLines) (Variables|Character|GetCharacterMovement) 8e+02 "None" (Variables|Character|GetMesh) self "Dash Start" "DashEnd" 1e+02 "/Game/Art/SFX/InGame/ER_WoodBreaking.ER_WoodBreaking" 1e+02)))

(event Input|EnhancedActionEvents|EnhancedInputActionIA_Pause
  (params (ActionValue :type Boolean) (ElapsedSeconds :type Float%20%28double-precision%29) (TriggeredSeconds :type Float%20%28double-precision%29) (InputAction :type Input%20Action%20Object%20Reference :default "/Game/Blueprints/Input/Actions/IA_Pause.IA_Pause"))
  ;[0.522 1 0.2235] Pause
  (:Started
    (CallFunction|PausetheGame :!label _label))
  (:Ongoing
    (goto _label)))

(event Input|EnhancedActionEvents|EnhancedInputActionIA_LookH
  (params (ActionValue :type Float%20%28double-precision%29) (ElapsedSeconds :type Float%20%28double-precision%29) (TriggeredSeconds :type Float%20%28double-precision%29) (InputAction :type Input%20Action%20Object%20Reference :default "/Game/Blueprints/Input/Actions/IA_LookH.IA_LookH"))
  ;[1 0.8284 0.2855] Camera Controls
  (CallFunction|YawDirection&Lerp ActionValue))

(event Input|EnhancedActionEvents|EnhancedInputActionIA_LookV
  (params (ActionValue :type Float%20%28double-precision%29) (ElapsedSeconds :type Float%20%28double-precision%29) (TriggeredSeconds :type Float%20%28double-precision%29) (InputAction :type Input%20Action%20Object%20Reference :default "/Game/Blueprints/Input/Actions/IA_LookV.IA_LookV"))
  ;[1 0.8284 0.2855] Camera Controls
  (CallFunction|BoomArmPitch ActionValue))

(event Input|EnhancedActionEvents|EnhancedInputActionIA_LightAttack
  (params (ActionValue :type Boolean) (ElapsedSeconds :type Float%20%28double-precision%29) (TriggeredSeconds :type Float%20%28double-precision%29) (InputAction :type Input%20Action%20Object%20Reference :default "/Game/Blueprints/Input/Actions/IA_LightAttack.IA_LightAttack"))
  (:Started
    (Default|LightAttackStart self "/Game/Art/Characters/Chair/v2/anims/montage/Chair_Light_01_Montage.Chair_Light_01_Montage" "/Game/Art/Characters/Chair/v2/anims/montage/Chair_Light_02_Montage.Chair_Light_02_Montage" "/Game/Art/Characters/Chair/v2/anims/montage/Chair_Light_03_Montage.Chair_Light_03_Montage" 2e+02 3e+02 :!label _label))
  (:Ongoing
    (goto _label)))

(event Input|EnhancedActionEvents|EnhancedInputActionIA_Locomotion
  (params (ActionValue :type Float%20%28double-precision%29) (ElapsedSeconds :type Float%20%28double-precision%29) (TriggeredSeconds :type Float%20%28double-precision%29) (InputAction :type Input%20Action%20Object%20Reference :default "/Game/Blueprints/Input/Actions/IA_Locomotion.IA_Locomotion"))
  (:Triggered
    (Variables|Default|SetXMovementValue ActionValue))
  (:Canceled
    (Variables|Default|SetXMovementValue 0.0 :!label _label))
  (:Completed
    (goto _label)))

(event Input|EnhancedActionEvents|EnhancedInputActionIA_Strafe
  (params (ActionValue :type Float%20%28double-precision%29) (ElapsedSeconds :type Float%20%28double-precision%29) (TriggeredSeconds :type Float%20%28double-precision%29) (InputAction :type Input%20Action%20Object%20Reference :default "/Game/Blueprints/Input/Actions/IA_Strafe.IA_Strafe"))
  (:Triggered
    (Variables|Default|SetYMovementValue ActionValue))
  (:Canceled
    (Variables|Default|SetYMovementValue 0.0 :!label _label))
  (:Completed
    (goto _label)))

(event Input|EnhancedActionEvents|EnhancedInputActionIA_Locomotion
  (params (ActionValue :type Float%20%28double-precision%29) (ElapsedSeconds :type Float%20%28double-precision%29) (TriggeredSeconds :type Float%20%28double-precision%29) (InputAction :type Input%20Action%20Object%20Reference :default "/Game/Blueprints/Input/Actions/IA_Locomotion.IA_Locomotion"))
  (if (Variables|Default|GetCanMove)
    (Default|Locomotion self ActionValue (Variables|Default|GetCameraYawPivot1))))

(event Input|EnhancedActionEvents|EnhancedInputActionIA_Strafe
  (params (ActionValue :type Float%20%28double-precision%29) (ElapsedSeconds :type Float%20%28double-precision%29) (TriggeredSeconds :type Float%20%28double-precision%29) (InputAction :type Input%20Action%20Object%20Reference :default "/Game/Blueprints/Input/Actions/IA_Strafe.IA_Strafe"))
  (if (Variables|Default|GetCanMove)
    (Default|Strafe self ActionValue (Variables|Default|GetCameraYawPivot1))))

(event Input|EnhancedActionEvents|EnhancedInputActionIA_Interact
  (params (ActionValue :type Boolean) (ElapsedSeconds :type Float%20%28double-precision%29) (TriggeredSeconds :type Float%20%28double-precision%29) (InputAction :type Input%20Action%20Object%20Reference :default "/Game/Blueprints/Input/Actions/IA_Interact.IA_Interact"))
  (:Started
    (CallFunction|Interactable 1e+03 1e+02 1.5e+02 (Variables|Character|GetMesh) "BottleSocket" "0.700000,-0.200000,-1.000000" "1.000000,1.000000,1.000000")))

(event Input|EnhancedActionEvents|EnhancedInputActionIA_HeavyAttack
  (params (ActionValue :type Boolean) (ElapsedSeconds :type Float%20%28double-precision%29) (TriggeredSeconds :type Float%20%28double-precision%29) (InputAction :type Input%20Action%20Object%20Reference :default "/Game/Blueprints/Input/Actions/IA_HeavyAttack.IA_HeavyAttack"))
  (:Started
    (Default|HeavyAttackStart self "/Game/Art/Characters/Chair/v2/anims/montage/Chair_Heavy_01_Montage.Chair_Heavy_01_Montage" "/Game/Art/Characters/Chair/v2/anims/montage/Chair_Heavy_02_Montage.Chair_Heavy_02_Montage" "/Game/Art/Characters/Chair/v2/anims/montage/Chair_Heavy_03_Montage.Chair_Heavy_03_Montage" 1e+02 :!label _label))
  (:Ongoing
    (goto _label)))

(event EventBeginPlay
  (|CallParentFunction)
  (Variables|Default|SetBaseKnockback 2e+02)
  (Variables|Default|SetBaseLightDamage 8.0)
  (Variables|Default|SetBaseHeavyDamage 16.0)
  (Variables|Default|SetBaseFinisherDamage 6e+01)
  (Transformation|SetWorldRotation (Variables|Default|GetSpringArm) (Transformation|GetActorRotation) false false)
  (CallFunction|PlayerHealth (Variables|Default|GetMAXHEALTH))
  (CallFunction|InitChairInt)
  (bind _returnvalue (Game|GetCurrentLevelName true))
  (if (Utilities|Enum|Equal(Enum) _returnvalue "LV_Horror")
    (Variables|Default|SetIsHorror true)
    (else
      (Variables|Default|SetIsHorror false))))

(event EventTick
  (params (DeltaSeconds :type Float%20%28single-precision%29))
  (bind _mesh (Variables|Character|GetMesh))
  (bind _camerayawpivot1 (Variables|Default|GetCameraYawPivot1))
  (CallFunction|TickInputVector _camerayawpivot1 (Variables|Default|GetSpringArm))
  (CallFunction|CameraBoomLerp)
  (if (Variables|Default|GetIs%20Targeting)
    (CallFunction|RotateTowardTarget _camerayawpivot1 "0.000000,0.000000,55.000000" 1.0)
    (Utilities|FlowControl|Sequence
      (:then_0
        (CallFunction|UpdateCameraFOV 1.2e+02)
        (if (>= (Variables|Default|GetComboCount) 25.0) :!label _label
          (Rendering|Material|SetOverlayMaterial _mesh "/Game/Materials/Instances/MI_BetsyElectric.MI_BetsyElectric" :!class /Script/Engine.MeshComponent)
          (else
            (Rendering|Material|SetOverlayMaterial _mesh 0 :!class /Script/Engine.MeshComponent))))
      (:then_1
        (goto _label_2 Reset)))
    (else
      (Utilities|FlowControl|Sequence
        (:then_0
          (Timeline|Timeline_1 Reverse
            (:Update
              (CallFunction|EndTarget)
              (goto _label))))
        (:then_1
          (Utilities|FlowControl|DoOnce false :!label _label_2
            (:Completed
              (CallFunction|UpdateCameraFOV 9e+01))))))))

(event Custom|ResetHitSweetSound
  (Variables|Default|SetHitSound false))

(event Custom|ClearEnemies
  (Utilities|Array|Clear (Variables|Default|GetActorsToIgnore)))

(event Custom|ResetFinisher
  (Variables|Default|SetFinisher false))

(event Custom|ResetHit
  (Variables|Default|SetOnHit false))

(event Custom|WoodBreakReset
  (Variables|Default|SetSoundBreak false))

(event Custom|chair%20blud
  (CallFunction|BludThirst (Variables|Character|GetCharacterMovement) 6e+02 8.5e+02 (Variables|Default|GetPostProcess)))

(fn ConstructionScript
  (|CallParentFunction))

(fn CameraBoomLerp
  (CallFunction|CameraLerp (Variables|Default|GetCameraBoomPitchPivot1) (Variables|Default|GetCameraYawPivot1) (Variables|Default|GetActualSpringArm1) (Variables|Default|GetBoomCameraFocusPoint1)))