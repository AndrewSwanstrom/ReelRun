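; BP_Throwable is a one-shot throwable object that the BP_Betsy player picks up and throws with IA_Interact.
; Interacting within MinDistance first sets HasThis, then launches the Sphere along Betsy's forward vector via physics velocity and marks it Used.
; While held, Tick repositions the Sphere in front of Betsy every frame.
; Live pickup never checks or sets Betsy's HoldingItem, only throwing clears it; unconnected older drafts remain.
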(event Input|EnhancedActionEvents|EnhancedInputActionIA_Interact
  (params (ActionValue :type Boolean) (ElapsedSeconds :type Float%20%28double-precision%29) (TriggeredSeconds :type Float%20%28double-precision%29) (InputAction :type Input%20Action%20Object%20Reference :default "/Game/Blueprints/Input/Actions/IA_Interact.IA_Interact"))
  ;[1 1 1] pickup / throw
  (:Started
    (if (not (Variables|Default|GetUsed))
      (bind _asbp_betsy (Utilities|Casting|CastToBP_Betsy (Game|Player|GetPlayerPawn 0)))
      (if (< (Math|Vector|Distance(Vector) (Transformation|GetWorldLocation (Variables|Default|GetSphere)) (Transformation|GetWorldLocation (Variables|/Script/Engine.Actor|GetRootComponent _asbp_betsy))) (Variables|Default|GetMinDistance))
        (if (Variables|Default|GetHasThis)
          (Variables|Default|SetHasThis false)
          (Variables|Default|SetUsed true)
          (Variables|/Game/Blueprints/Characters/BP_Betsy.BP_Betsy_C|SetHoldingItem _asbp_betsy false)
          (Physics|SetPhysicsLinearVelocity (Variables|Default|GetSphere) (* (Transformation|GetActorForwardVector _asbp_betsy) 2e+03) false "None")
          (else
            (Variables|Default|SetHasThis true)))))))

(event Input|EnhancedActionEvents|EnhancedInputActionIA_Interact
  (params (ActionValue :type Boolean) (ElapsedSeconds :type Float%20%28double-precision%29) (TriggeredSeconds :type Float%20%28double-precision%29) (InputAction :type Input%20Action%20Object%20Reference :default "/Game/Blueprints/Input/Actions/IA_Interact.IA_Interact")))

(event Input|EnhancedActionEvents|EnhancedInputActionIA_Interact
  (params (ActionValue :type Boolean) (ElapsedSeconds :type Float%20%28double-precision%29) (TriggeredSeconds :type Float%20%28double-precision%29) (InputAction :type Input%20Action%20Object%20Reference :default "/Game/Blueprints/Input/Actions/IA_Interact.IA_Interact"))
  ;[1 1 1] gay baby jail
)

(event EventBeginPlay
  (Input|EnableInput (Game|GetPlayerController 0)))

(event Collision|EventActorBeginOverlap
  (params (OtherActor :type Actor%20Object%20Reference))
  ;[1 1 1] gay baby jail
)

(event EventTick
  (params (DeltaSeconds :type Float%20%28single-precision%29))
  (bind _returnvalue (Transformation|GetActorTransform))
  ;[1 1 1] Hold in front of player
  (if (Variables|Default|GetHasThis)
    (bind _asbp_betsy (Utilities|Casting|CastToBP_Betsy (Game|Player|GetPlayerPawn 0)))
    (Transformation|SetWorldTransform (Variables|Default|GetSphere) (Math|Transform|MakeTransform (+ (* (Transformation|GetActorForwardVector _asbp_betsy) 1e+02) (.location (Transformation|GetActorTransform _asbp_betsy))) (.rotation _returnvalue) (.scale _returnvalue)) false false)))

(fn ConstructionScript)