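; BP_TestTomb is a tomb Blueprint in the horror destruction folder that varies its look at random when play begins.
; BeginPlay rolls RenderInt from one to three, then makes one of three base components and one of three body components visible.
; Both choices switch on the same RenderInt, so the tomb has three fixed base and body pairings, with mismatched numbering in some.
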(event EventBeginPlay
  (bind _output_get (Variables|Default|SetRenderInt (Math|Random|RandomIntegerinRange 1 3)))
  (switch int _output_get
    (:1
      (Rendering|SetVisibility (Variables|Default|Getbase%202) true false))
    (:2
      (Rendering|SetVisibility (Variables|Default|Getbase%201) true false))
    (:3
      (Rendering|SetVisibility (Variables|Default|Getbase%203) true false)))
  (switch int (Variables|Default|GetRenderInt)
    (:1
      (Rendering|SetVisibility (Variables|Default|Getbody%202) true false))
    (:2
      (Rendering|SetVisibility (Variables|Default|Getbody%203) true false))
    (:3
      (Rendering|SetVisibility (Variables|Default|Getbody%201) true false))))

(fn ConstructionScript)