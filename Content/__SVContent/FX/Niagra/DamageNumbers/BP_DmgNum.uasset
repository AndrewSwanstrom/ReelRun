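; BP_DmgNum is a floating damage number actor that shows a damage amount and removes itself.
; On BeginPlay it passes DmgAmt to its BPW_DmgNum widget component and computes a fixed offset end point from its spawn location.
; A timeline lerps the actor up and diagonally to that point, then destroys it when finished.
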(event EventBeginPlay
  (bind _asbpw_dmg_num (Utilities|Casting|CastToBPW_DmgNum (UserInterface|GetWidget (Variables|Default|GetDmgWidget))))
  (Variables|/Game/__SVContent/FX/Niagra/DamageNumbers/BPW_DmgNum.BPW_DmgNum_C|SetDmgAmt _asbpw_dmg_num (Variables|Default|GetDmgAmt))
  (bind _output_get (Variables|Default|SetStartLocation (Transformation|GetActorLocation)))
  (Variables|Default|SetEndLocation (+ _output_get "-25.000000,-25.000000,50.000000"))
  (bind _movetexttrack (Timeline|MoveTextTimeline Play)
    (:Update
      (Transformation|SetActorLocation (Math|Vector|Lerp(Vector) (Variables|Default|GetStartLocation) (Variables|Default|GetEndLocation) _movetexttrack) false false))
    (:Finished
      (Actor|DestroyActor))))

(fn ConstructionScript)