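; A spline-driven construction-script actor that builds a string of lights hung between poles.
; It adds a pole mesh at each spline point, then spaces bulb meshes and point lights along straight segments, offset vertically by a Gravity-scaled sine.
; A LightsOn flag toggles bulb emissive color and light visibility.
; Cable and spline-mesh rope attempts remain disconnected, so no wire is built.
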(event EventBeginPlay)

(event Collision|EventActorBeginOverlap
  (params (OtherActor :type Actor%20Object%20Reference)))

(event EventTick
  (params (DeltaSeconds :type Float%20%28single-precision%29)))

(fn ConstructionScript
  (bind _spline (Variables|Default|GetSpline))
  ;[1 1 1] Set up spline points and beams
  (for _index (range 0 (- (Spline|GetNumberOfSplinePoints (Variables|Default|GetSpline)) 2))
    (Variables|Default|SetSplineStartPos (Spline|GetLocationatSplinePoint (Variables|Default|GetSpline) _index "Local"))
    (Variables|Default|SetSplineEndPos (Spline|GetLocationatSplinePoint (Variables|Default|GetSpline) (+ _index 1) "Local"))
    (AddComponent|AddStaticMeshComponent false (Math|Conversions|ToTransform(Vector) (Variables|Default|GetSplineStartPos))) ; set up pole mesh
    ;[1 1 1] Place light bulbs
    (for _index_2 (range 0 (Math|Float|Truncate (/ (Math|Vector|Distance(Vector) (Variables|Default|GetSplineStartPos) (Variables|Default|GetSplineEndPos)) (Variables|Default|GetDistanceBetweenLights))))
      (bind _returnvalue (AddComponent|AddStaticMeshComponent false (Math|Conversions|ToTransform(Vector) (+ (+ (* (Math|Vector|GetUnitDirection(Vector) (Variables|Default|GetSplineStartPos) (Variables|Default|GetSplineEndPos)) (* _index_2 (Variables|Default|GetDistanceBetweenLights))) (Variables|Default|GetSplineStartPos)) (Math|Vector|MakeVector 0.0 0.0 (* (Math|Trig|Sin(Degrees) (* (/ (* _index_2 (Variables|Default|GetDistanceBetweenLights)) (/ (Math|Vector|Distance(Vector) (Variables|Default|GetSplineStartPos) (Variables|Default|GetSplineEndPos)) (Variables|Default|GetDistanceBetweenLights))) (Variables|Default|Getdebugsine))) (Variables|Default|GetGravity))))))) ; set up light bulb mesh
      (Rendering|Material|SetVectorParameterValueonMaterials _returnvalue "ColorVector" (Math|Vector|SelectVector (Math|Conversions|ToVector(LinearColor) (Variables|Default|GetMaterialColorVector)) "0, 0, 0" (Variables|Default|GetLightsOn)))
      (bind _returnvalue_2 (AddComponent|AddPointLightComponent false (Math|Conversions|ToTransform(Vector) (+ (+ (* (Math|Vector|GetUnitDirection(Vector) (Variables|Default|GetSplineStartPos) (Variables|Default|GetSplineEndPos)) (* _index_2 (Variables|Default|GetDistanceBetweenLights))) (Variables|Default|GetSplineStartPos)) (Math|Vector|MakeVector 0.0 0.0 (* (Math|Trig|Sin(Degrees) (* (/ (* _index_2 (Variables|Default|GetDistanceBetweenLights)) (/ (Math|Vector|Distance(Vector) (Variables|Default|GetSplineStartPos) (Variables|Default|GetSplineEndPos)) (Variables|Default|GetDistanceBetweenLights))) (Variables|Default|Getdebugsine))) (Variables|Default|GetGravity)))))))
      (Rendering|Components|Light|SetLightColor _returnvalue_2 (Variables|Default|GetLightColorVector) true)
      ;[1 1 1] point lights on/off
      (if (Variables|Default|GetLightsOn)
        (Rendering|SetVisibility _returnvalue_2 true false)
        (else
          (Rendering|SetVisibility _returnvalue_2 false false)))))
  (AddComponent|AddStaticMeshComponent false (Math|Conversions|ToTransform(Vector) (Spline|GetLocationatSplinePoint _spline (Spline|GetNumberOfSplinePoints _spline) "Local"))) ; place last pole
)