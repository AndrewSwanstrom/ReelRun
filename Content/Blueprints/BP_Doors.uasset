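; BP_Doors is a locked gate that the player opens with an interact input once KeyObtained is true.
; A Box overlap tracks whether something is inside and shows or hides an interact icon when the key is held.
; While inside, Tick rotates the icon to face the player camera.
; Interacting disables mesh collision and destroys the box and both gate components.
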(event OnComponentBeginOverlap(Box)
  (params (OverlappedComponent :type Primitive%20Component%20Object%20Reference) (OtherActor :type Actor%20Object%20Reference) (OtherComp :type Primitive%20Component%20Object%20Reference) (OtherBodyIndex :type Integer) (bFromSweep :type Boolean) (SweepResult :type Hit%20Result%20Structure%20%28by%20ref%29))
  (Variables|Default|SetisIn true)
  (if (Variables|Default|GetKeyObtained)
    (Rendering|SetVisibility (Variables|Default|GetInteract%20Icon) true false)))

(event OnComponentEndOverlap(Box)
  (params (OverlappedComponent :type Primitive%20Component%20Object%20Reference) (OtherActor :type Actor%20Object%20Reference) (OtherComp :type Primitive%20Component%20Object%20Reference) (OtherBodyIndex :type Integer))
  (Variables|Default|SetisIn false)
  (if (Variables|Default|GetKeyObtained)
    (Rendering|SetVisibility (Variables|Default|GetInteract%20Icon) false false)))

(event Input|EnhancedActionEvents|EnhancedInputActionIA_Interact
  (params (ActionValue :type Boolean) (ElapsedSeconds :type Float%20%28double-precision%29) (TriggeredSeconds :type Float%20%28double-precision%29) (InputAction :type Input%20Action%20Object%20Reference :default "/Game/Blueprints/Input/Actions/IA_Interact.IA_Interact"))
  ;[1 1 1] interact
  (:Started
    (if (and (Variables|Default|GetisIn) (Variables|Default|GetKeyObtained))
      (Collision|SetCollisionEnabled (Variables|Debug|GetStaticMeshComponent) "NoCollision")
      (Components|DestroyComponent (Variables|Default|GetBox))
      (Variables|Default|SetisIn false)
      (Components|DestroyComponent (Variables|Default|GetGate1)))))

(event EventTick
  (params (DeltaSeconds :type Float%20%28single-precision%29))
  ;[1 1 1] we can replace these with a UI so we dont have to event Tick
  (if (Variables|Default|GetisIn)
    (Transformation|SetWorldRotation (Variables|Default|GetInteract%20Icon) (Math|Rotator|FindLookatRotation (Transformation|GetWorldLocation (Variables|Default|GetInteract%20Icon)) (Transformation|GetWorldLocation (Variables|/Script/Engine.PlayerCameraManager|GetTransformComponent (Game|GetPlayerCameraManager 0)))) false false)))

(event EventBeginPlay
  (Input|EnableInput (Game|GetPlayerController 0)))

(fn ConstructionScript)