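; Ranged enemy that attacks the player with a handgun spawned into its hand socket, telegraphing shots with a Niagara laser.
; Tick traces the beam toward the player, while aim, warning and bullet events set its color around the attack montage.
; Damage drives a timeline knockback sized by the damage causer, sets blackboard state and runs a collision trace while overlapping.
; At zero health it unpossesses, dissolves and destroys itself and its gun.
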(event Custom|OnMontageEnded_Event
  (params (Montage :type Anim%20Montage%20Object%20Reference) (bInterrupted :type Boolean))
  ;[1 0.3851 0.405] Binded Montage End Event
  (if (== Montage "/Game/Art/Characters/Enemies/Shooter/Animations/Montage/Anim_ShooterAttack_Montage.Anim_ShooterAttack_Montage")
    (Audio|Components|Audio|Stop (Variables|Default|GetWarningFlash))
    (Niagara|SetNiagaraVariable(LinearColor) (Variables|Default|GetNiagara) "Color" (Utilities|Struct|MakeLinearColor 0.0 0.0 0.0 0.0))))

(event Custom|EventAttack
  ;[0.1521 0.3289 1] Shoot Player
  (if (Variables|Default|GetStartStopShooting)
    (Animation|Montage|PlayMontage (Variables|Character|GetMesh) "/Game/Art/Characters/Enemies/Shooter/Animations/Montage/Anim_ShooterAttack_Montage.Anim_ShooterAttack_Montage"
      (:OnCompleted
        _)
      (:OnInterrupted
        _))
    (Default|CallOnShootEnd)))

(event Custom|AimWarning
  ;[1 0.3162 0.2465] Aim Warning
  (bind _redchannelfloat (Timeline|WarningFlash PlayFromStart)
    (:Update
      (Niagara|SetNiagaraVariable(LinearColor) (Variables|Default|GetNiagara) "Color" (Utilities|Struct|MakeLinearColor _redchannelfloat 0.0 0.0 1.0)))))

(event Game|Damage|EventAnyDamage
  (params (Damage :type Float%20%28single-precision%29) (DamageType :type Damage%20Type%20Object%20Reference) (InstigatedBy :type Controller%20Object%20Reference) (DamageCauser :type Actor%20Object%20Reference))
  (bind _returnvalue (Transformation|GetActorLocation))
  (bind _returnvalue_2 (Pawn|GetController))
  (bind _self self)
  (bind _self_2 self)
  (bind _mesh (Variables|Character|GetMesh))
  (bind _returnvalue_3 (Transformation|GetActorTransform _self_2))
  ;[0.2971 1 0.9202] Take Damage & Knockback
  (if (Variables|Default|GetCanBeDamaged)
    (Audio|PlaySoundatLocation "/Game/Art/SFX/RandomHitCue.RandomHitCue" _returnvalue "0, 0, 0" 1.0 (Math|Random|RandomFloatinRange 0.5 1.3) 0.0 0 0 0 0)
    (Audio|PlaySoundatLocation (.OutItem (Utilities|Array|Random (Variables|Default|GetHitSounds))) _returnvalue "0, 0, 0" 1.0 1.0 0.0 0 0 0 0)
    ;;[1 1 1] show dmg numbers?
    (if (Variables|Default|GetShowDmgNums?)
      (Game|SpawnActorfromClass "/Game/Art/VFX/Blood_And_Nums/DamageNumbers/BP_DmgNum.BP_DmgNum_C" (Transformation|GetActorTransform _self) "Undefined" "MultiplyWithRoot" _self (* Damage 1e+01) "(R=0.000000,G=0.000000,B=0.000000,A=0.000000)" 0)
      (bind _asbase_character (Utilities|Casting|CastToBase_Character DamageCauser)
        (:then
          (Variables|Default|SetCustomKnockBackForce (Variables|/Game/Blueprints/Characters/Base_Character.Base_Character_C|GetKnockBackForce _asbase_character))
          ;;[1 1 1] is dmg causer syd
          (if (Variables|/Game/Blueprints/Characters/Base_Character.Base_Character_C|GetSyd _asbase_character)
            (AddComponent|AddNiagaraComponent false)))
        (:CastFailed
          (bind _asbp_throwable_base_obj (Utilities|Casting|CastToBP_ThrowableBaseObj DamageCauser)
            (:then
              (Variables|Default|SetCustomKnockBackForce (Variables|/Game/Blueprints/Throwables/BP_ThrowableBaseObj.BP_ThrowableBaseObj_C|GetThrowableKnockback _asbp_throwable_base_obj)))
            (:CastFailed
              (Variables|Default|SetCustomKnockBackForce 9e+02)))))
      (Animation|Montage|PlayMontage (Variables|Character|GetMesh) "/Game/Art/Characters/Enemies/Shooter/Animations/Montage/Anim_ShooterDamage_Montage.Anim_ShooterDamage_Montage"
        (:then
          (CallFunction|ShooterKnockBack)
          (bind _alpha (Timeline|Timeline PlayFromStart)
            (:Update
              (if (== (Variables|Default|GetCustomTimeDilation) 1.0)
                (CallFunction|StartKnockBack _alpha (Variables|Default|GetCustomKnockBackForce))))
            (:Finished
              (Utilities|FlowControl|Delay 0.2)
              (Variables|Default|SetIsOverlapping false)
              (CallFunction|KnockBackState (AI|GetBlackboard (AI|GetAIController self)) (Variables|Default|GetKey) (Utilities|Enum|LiteralenumLightEnemy "NewEnumerator0"))
              (bind _output_get (Variables|Default|SetHealth (- (Variables|Default|GetHealth) Damage)))
              (if (<= _output_get 0.0)
                (Variables|Default|SetCanBeDamaged false)
                (Utilities|IsValid _returnvalue_2
                  (:Is%20Valid
                    (Pawn|UnPossess _returnvalue_2)
                    (Animation|PlayAnimMontage 0 0.2 "None")
                    (Niagara|SpawnSystematLocation "/Game/Art/VFX/MeshSprites/ShooterEnemySprites.ShooterEnemySprites" (.location _returnvalue_3) (.rotation _returnvalue_3) (.scale _returnvalue_3))
                    (bind _slowoff (Timeline|Timeline_0 PlayFromStart)
                      (:Update
                        (bind _returnvalue_4 (Rendering|Material|CreateDynamicMaterialInstance (Variables|Character|GetMesh) 0 "/Game/Art/VFX/NS_EdgeBurnv1/MI_EnemyDissolve.MI_EnemyDissolve" "None" :!class /Script/Engine.PrimitiveComponent))
                        (Rendering|Material|SetScalarParameterValue _returnvalue_4 "Dissolve" (Math|Float|Lerp 5.0 0.0 _slowoff) :!class /Script/Engine.MaterialInstanceDynamic)
                        (Utilities|FlowControl|Delay 0.25)
                        (Physics|SetSimulatePhysics _mesh false)
                        (Collision|SetCollisionProfileName _mesh "Ragdoll" true :!class /Script/Engine.PrimitiveComponent)
                        (Utilities|FlowControl|Delay 1.0)
                        (Actor|DestroyActor)
                        (Actor|DestroyActor (Variables|Default|GetGunBP_Ref))))))))))))))

(event EventTick
  (params (DeltaSeconds :type Float%20%28single-precision%29))
  ;[0.2257 1 0.4545] Event Tick for Knock Back Check
  (bind _outhit (Collision|LineTraceByChannel (Transformation|GetSocketLocation (Variables|Character|GetMesh) "GunSpawn") (Transformation|GetActorLocation (Variables|Default|GetChar%20Ref)) "TraceTypeQuery1" false 0 "None" true "(R=1.000000,G=0.000000,B=0.000000,A=1.000000)" "(R=0.000000,G=1.000000,B=0.000000,A=1.000000)" 3.0))
  (Effects|Components|ParticleSystem|SetVectorParameter (Variables|Default|GetNiagara) "Beam End" (.location _outhit))
  (if (Variables|Default|GetIsOverlapping)
    (CallFunction|KnockBackTrace (Variables|Character|GetMesh) (Variables|Default|GetTraceStart) (Variables|Default|GetTraceEnd) 3e+01 "/Game/Art/SFX/InGame/ER_WoodBreaking.ER_WoodBreaking")))

(event EventBeginPlay
  ;[0.6739 1 0.2482] Spawn Gun in Enemy Hand
  (EventDispatchers|AssignOnMontageEnded (Components|SkeletalMesh|GetAnimInstance (Variables|Character|GetMesh)) (delegate Custom|OnMontageEnded_Event))
  (bind _asbase_character (Utilities|Casting|CastToBase_Character (Game|Player|GetPlayerPawn 0)))
  (Variables|Default|SetChar%20Ref _asbase_character)
  (bind _returnvalue (Game|SpawnActorfromClass (Variables|Default|GetHandGunRef) (Transformation|GetSocketTransform (Variables|Character|GetMesh) "Gun" "RTS_World") "Undefined" "MultiplyWithRoot" 0 0))
  (bind _output_get (Variables|Default|SetGunBP_Ref _returnvalue))
  (Transformation|AttachComponentToComponent _output_get (Variables|Character|GetMesh) "Gun" "SnapToTarget" "SnapToTarget" "SnapToTarget" true))

(event Custom|ShooterKnockBack
  ;[1 0.3229 0.5782] Force Shooter to Knockback
  (CallFunction|KnockBackState (AI|GetBlackboard (AI|GetAIController self)) (Variables|Default|GetKey) (Utilities|Enum|LiteralenumLightEnemy "NewEnumerator8")))

(event Custom|BulletSpawn
  ;[0.6719 1 0.3438] Spawn Bullet
  (Audio|Components|Audio|Stop (Variables|Default|GetWarningFlash))
  (CallFunction|Bullet self (Variables|Default|GetFlash) (Variables|Character|GetMesh))
  (Niagara|SetNiagaraVariable(LinearColor) (Variables|Default|GetNiagara) "Color" (Utilities|Struct|MakeLinearColor 0.0 0.0 0.0 0.0)))

(event Custom|TakeAim
  ;[0.2436 0.7141 1] Slow Aim animation down and turn laser on
  (Niagara|SetNiagaraVariable(LinearColor) (Variables|Default|GetNiagara) "Color" (Utilities|Struct|MakeLinearColor 1.0 0.1 0.1 1.0)))

(fn ConstructionScript)

(fn ShootatPlayer
  (bind _self self)
  (bind _returnvalue (Transformation|GetActorTransform _self))
  (bind _returnvalue_2 (Game|SpawnActorfromClass "/Game/Blueprints/Damaging/BP_Damager.BP_Damager_C" (Math|Transform|MakeTransform (+ (+ (* (Transformation|GetActorForwardVector _self) 1e+02) (.location _returnvalue)) "0.000000,0.000000,50.000000") (.rotation _returnvalue) (.scale _returnvalue)) "Undefined" "MultiplyWithRoot" 0 0))
  (Rendering|SetVisibility (Variables|Default|GetFlash) false false)
  (Niagara|SpawnSystemAttached "/Game/Art/VFX/NS_MuzzleFlash.NS_MuzzleFlash" 0 "None" "0.000000,35.000000,10.000000" "0.000000,45.000000,0.000000" "KeepRelativeOffset" false)
  (bind _asbp_betsy (Utilities|Casting|CastToBP_Betsy (Game|Player|GetPlayerPawn 0)))
  (Physics|AddImpulse (Variables|/Game/Blueprints/Damaging/BP_Damager.BP_Damager_C|GetCollider _returnvalue_2) (* (Math|Vector|GetUnitDirection(Vector) (+ (Transformation|GetActorLocation self) "0.000000,0.000000,50.000000") (Transformation|GetActorLocation _asbp_betsy)) 1e+03) "None" true))

(fn AttackStart
  (params (AttackTarget :type Actor%20Object%20Reference) (Tokens%20Needed :type Integer))
  (return false))

(fn GetIdealRange
  (return 1e+03 3e+02 0.0))

(fn SetMovementSpeed
  (params (Speed :type E_MovementSpeed%20Enum :default "NewEnumerator0"))
  (bind _output_get (Variables|/Script/Engine.CharacterMovementComponent|SetMaxWalkSpeed (Variables|Character|GetCharacterMovement) (Utilities|Select :Index Speed :NewEnumerator0 0.0 :NewEnumerator1 2.5e+02 :NewEnumerator2 5e+02 :NewEnumerator4 0.0)))
  (return _output_get))