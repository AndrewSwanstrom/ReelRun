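; Chandelier Blueprint that animates its pivot between a start and an end transform, presumably as a swaying motion.
; On BeginPlay a random integer picks one of three timelines, so placed instances can move differently.
; The playing timeline's Alpha lerps TransformPivot's world transform between the TransformStart and TransformEnd components on every update.
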(event EventBeginPlay
  (switch int (Math|Random|RandomIntegerinRange 0 2)
    (:Default
      (bind _alpha (Timeline|Timeline_0 Play)
        (:Update
          (Transformation|SetWorldTransform (Variables|Default|GetTransformPivot) (Math|Transform|Lerp(Transform) (Transformation|GetWorldTransform (Variables|Default|GetTransformStart)) (Transformation|GetWorldTransform (Variables|Default|GetTransformEnd)) _alpha) false false))))
    (:0
      (bind _alpha_2 (Timeline|Timeline_1 Play)
        (:Update
          (Transformation|SetWorldTransform (Variables|Default|GetTransformPivot) (Math|Transform|Lerp(Transform) (Transformation|GetWorldTransform (Variables|Default|GetTransformStart)) (Transformation|GetWorldTransform (Variables|Default|GetTransformEnd)) _alpha_2) false false))))
    (:1
      (Timeline|Timeline_0 Play))
    (:2
      (bind _alpha_3 (Timeline|Timeline Play)
        (:Update
          (Transformation|SetWorldTransform (Variables|Default|GetTransformPivot) (Math|Transform|Lerp(Transform) (Transformation|GetWorldTransform (Variables|Default|GetTransformStart)) (Transformation|GetWorldTransform (Variables|Default|GetTransformEnd)) _alpha_3) false false))))))

(fn ConstructionScript)