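; Western boss enemy character that provides attacks, movement speeds and attack range, presumably for its AI.
; Light, heavy and charge events play montages and fire end callbacks when these complete or are interrupted.
; While an attack flag is set, Tick sphere-traces between fist or leg sockets, damaging each actor once until the ignore list clears.
; Damage lowers health, switches the blackboard to a run-away state when low, and destroys the boss at zero.
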(event Custom|AttackLight
  ;[1 1 1] Boss Animation Triggers
  (Animation|Montage|PlayMontage (Variables|Character|GetMesh) "/Game/Art/Characters/Enemies/WesternBoss/Animations/Anim_BossLightAttack_Montage.Anim_BossLightAttack_Montage" 1.5
    (:OnCompleted
      _)
    (:OnInterrupted
      _))
  (Default|CallOnLightAttackEnd))

(event Custom|AttackHeavy
  ;[1 1 1] Boss Animation Triggers
  (Animation|Montage|PlayMontage (Variables|Character|GetMesh) "/Game/Art/Characters/Enemies/WesternBoss/Animations/Anim_BossHeavyAttack_Part1_Montage.Anim_BossHeavyAttack_Part1_Montage" 1.2
    (:OnCompleted
      _)
    (:OnInterrupted
      _))
  (Default|CallOnHeavyAttackEnd))

(event Custom|ClearAttackStack
  ;[1 1 1] Clear Stacks From Line Trace
  (Utilities|Array|Clear (Variables|Default|GetActorsToIgnore)))

(event Custom|Charging
  ;[1 1 1] Boss Animation Triggers
  (Animation|Montage|PlayMontage (Variables|Character|GetMesh) "/Game/Art/Characters/Enemies/WesternBoss/Animations/Boss_Charge_Montage.Boss_Charge_Montage" 0.75
    (:OnCompleted
      _)
    (:OnInterrupted
      _))
  (Default|CallOnChargeEnd))

(event Game|Damage|EventAnyDamage
  (params (Damage :type Float%20%28single-precision%29) (DamageType :type Damage%20Type%20Object%20Reference) (InstigatedBy :type Controller%20Object%20Reference) (DamageCauser :type Actor%20Object%20Reference))
  ;[1 1 1] Damage Boss & Set Run away State
  (bind _output_get (Variables|Default|SetHealth (- (Variables|Default|GetHealth) Damage)))
  (if (<= _output_get 2e+01)
    (AI|Components|Blackboard|SetValueasEnum (Variables|/Script/AIModule.AIController|GetBlackboard (AI|GetAIController self)) (Variables|Default|GetKeyName) (Utilities|Enum|LiteralenumLightEnemy "NewEnumerator6"))
    (if (<= _output_get 0.0)
      (Actor|DestroyActor))))

(event EventTick
  (params (DeltaSeconds :type Float%20%28single-precision%29))
  (bind _mesh (Variables|Character|GetMesh))
  ;[1 1 1] Event Tick Line Trace Damage Logic
  (Variables|Default|SetDelta%20Seconds DeltaSeconds)
  (if (Variables|Default|GetLeftFistAttack)
    (Variables|Default|SetSocketStart "LeftHandStart")
    (Variables|Default|SetSocketEnd "LeftHandEnd")
    (bind _outhits (Collision|MultiSphereTraceForObjects (Transformation|GetSocketLocation _mesh (Variables|Default|GetSocketStart)) (Transformation|GetSocketLocation _mesh (Variables|Default|GetSocketEnd)) 2e+01 (Utilities|Array|MakeArray "ObjectTypeQuery7") false 0 "None" :!label _label))
    (for _array_element _outhits
      (if (not (Utilities|Array|ContainsItem (Variables|Default|GetActorsToIgnore) (.HitActor (Collision|BreakHitResult _array_element))))
        (Game|Damage|ApplyDamage (.HitActor (Collision|BreakHitResult _array_element)) (Variables|Default|GetDamageCalculator) 0 0)
        (Utilities|Array|Add (Variables|Default|GetActorsToIgnore) (.HitActor (Collision|BreakHitResult _array_element)))))
    (elif (Variables|Default|GetRightFistAttack)
      (Variables|Default|SetSocketStart "RightHandStart")
      (Variables|Default|SetSocketEnd "RightHandEnd")
      (goto _label)
      (elif (Variables|Default|GetHeavyAttack)
        (Variables|Default|SetSocketStart "LeftLegStart")
        (Variables|Default|SetSocketEnd "LeftLegEnd")
        (goto _label)))))

(event EventBeginPlay)

(event Collision|EventActorBeginOverlap
  (params (OtherActor :type Actor%20Object%20Reference)))

(fn ConstructionScript)

(fn GetIdealRange
  (return 1.2e+02 0.0))

(fn SetMovementSpeed
  (params (Speed :type E_MovementSpeed%20Enum :default "NewEnumerator0"))
  (bind _output_get (Variables|/Script/Engine.CharacterMovementComponent|SetMaxWalkSpeed (Variables|Character|GetCharacterMovement) (Utilities|Select :Index Speed :NewEnumerator0 0.0 :NewEnumerator1 1e+02 :NewEnumerator2 6e+02)))
  (return _output_get))