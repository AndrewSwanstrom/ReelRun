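; Interactable radio that the player picks up, attaches to their character's radio socket, and that then plays captioned lines.
; A box overlap toggles the interaction prompt, and a one-shot interact picks it up in range and shows a random theatre caption.
; Campfire, cemetery and firewatch events add caption widgets only once held, using random rows except for a fixed cemetery row.
; HideNotifs clears the prompt, highlight, collision, light and static volume.
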(event OnComponentBeginOverlap(Box1)
  (params (OverlappedComponent :type Primitive%20Component%20Object%20Reference) (OtherActor :type Actor%20Object%20Reference) (OtherComp :type Primitive%20Component%20Object%20Reference) (OtherBodyIndex :type Integer) (bFromSweep :type Boolean) (SweepResult :type Hit%20Result%20Structure%20%28by%20ref%29))
  (CallFunction|BeginColliderOverlap OtherActor (Variables|Default|GetInteractIcon) (Variables|Default|GetOverlayMesh)))

(event OnComponentEndOverlap(Box1)
  (params (OverlappedComponent :type Primitive%20Component%20Object%20Reference) (OtherActor :type Actor%20Object%20Reference) (OtherComp :type Primitive%20Component%20Object%20Reference) (OtherBodyIndex :type Integer))
  (CallFunction|EndColliderOverlap OtherActor (Variables|Default|GetInteractIcon) (Variables|Default|GetOverlayMesh)))

(event Custom|cemetary%20lines
  (if (Variables|Default|GetbHasRadio)
    (bind _returnvalue (UserInterface|CreateWidget "/Game/Blueprints/UI/VA/WBP_RadioCaptions.WBP_RadioCaptions_C" (Game|GetPlayerController 0) (Utilities|Struct|MakeDataTableRowHandle "/Game/Blueprints/UI/VA/dataTables/radio/DT_RadioCemetary.DT_RadioCemetary" "1")))
    (UserInterface|Viewport|AddtoViewport _returnvalue 3)))

(event Custom|firewatch%20lines
  (if (Variables|Default|GetbHasRadio)
    (bind _returnvalue (UserInterface|CreateWidget "/Game/Blueprints/UI/VA/WBP_RadioCaptions.WBP_RadioCaptions_C" (Game|GetPlayerController 0) (.OutItem (Utilities|Array|Random (Variables|Default|GetrandomFirewatch)))))
    (UserInterface|Viewport|AddtoViewport _returnvalue 3)))

(event Custom|campfire%20lines
  (if (Variables|Default|GetbHasRadio)
    (bind _returnvalue (UserInterface|CreateWidget "/Game/Blueprints/UI/VA/WBP_RadioCaptions.WBP_RadioCaptions_C" (Game|GetPlayerController 0) (.OutItem (Utilities|Array|Random (Variables|Default|GetrandomCampfire)))))
    (UserInterface|Viewport|AddtoViewport _returnvalue 3)))

(event EventInteractAction
  (Utilities|FlowControl|DoOnce false
    (:Completed
      (if (Variables|Default|GetbInRange)
        (CallFunction|PickupActor (Variables|Default|GetMeshRef) "radioSocket" "0.700000,-0.200000,-1.000000" "0.075000,0.075000,0.075000" (Variables|Default|GetBox1) (Variables|Default|GetStaticMesh) (Variables|Default|GetInteractIcon))
        (bind _returnvalue (UserInterface|CreateWidget "/Game/Blueprints/UI/VA/WBP_RadioCaptions.WBP_RadioCaptions_C" (Game|GetPlayerController 0) (.OutItem (Utilities|Array|Random (Variables|Default|GetrandomTheatre)))))
        (UserInterface|Viewport|AddtoViewport _returnvalue 3)
        (Variables|Default|SetbHasRadio true)))))

(event EventIsInside
  (params (IN :type Boolean)))

(event EventHideNotifs
  (bind _box1 (Variables|Default|GetBox1))
  (Rendering|SetVisibility (Variables|Default|GetInteractIcon) false true)
  (Rendering|Material|SetOverlayMaterial (Variables|Default|GetOverlayMesh) 0 :!class /Script/Engine.MeshComponent)
  (Components|Activation|SetActive _box1 false false)
  (Collision|SetCollisionEnabled _box1 "NoCollision")
  (Components|DestroyComponent (Variables|Default|GetPointLight))
  (Audio|Components|Audio|SetVolumeMultiplier (Variables|Default|GetRadioStatic) 0.0 :!class /Script/Engine.AudioComponent))

(event EventBeginPlay
  (bind _asbase_character (Utilities|Casting|CastToBase_Character (Game|GetPlayerCharacter 0)))
  (Variables|Default|SetMeshRef (Variables|/Script/Engine.Character|GetMesh _asbase_character)))

(fn ConstructionScript
  (|CallParentFunction))