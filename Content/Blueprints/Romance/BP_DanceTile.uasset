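; Dance floor tile actor that switches between random materials and can act as a damaging attack tile with a spike.
; While Active, Tick uses a random delay to trigger TileOff, which plays the EmissiveLerpOff timeline to animate glow, then picks a new material.
; Attack tiles also bounce via a timeline, sphere-checking at the spike for damage, then bounce back when the glow finishes.
; Collider overlaps deal lighter damage while the tile is damaging or flagged as an attack.
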(event OnComponentBeginOverlap(collider)
  (params (OverlappedComponent :type Primitive%20Component%20Object%20Reference) (OtherActor :type Actor%20Object%20Reference) (OtherComp :type Primitive%20Component%20Object%20Reference) (OtherBodyIndex :type Integer) (bFromSweep :type Boolean) (SweepResult :type Hit%20Result%20Structure%20%28by%20ref%29))
  (bind _output_get (Variables|Default|SetOverlappedActor OtherActor))
  (if (or (Variables|Default|GetbCanDmg) (Variables|Default|GetbAnAttack))
    (Development|PrintString "Hello")
    (Game|Damage|ApplyDamage _output_get 1.0 0 self)
    (else
      (Development|PrintString "asdasd"))))

(event OnComponentEndOverlap(collider)
  (params (OverlappedComponent :type Primitive%20Component%20Object%20Reference) (OtherActor :type Actor%20Object%20Reference) (OtherComp :type Primitive%20Component%20Object%20Reference) (OtherBodyIndex :type Integer)))

(event Custom|Change%20Material
  ;[1 1 1] change material
  (Rendering|Material|SetMaterial (Variables|Default|GetCube) 0 (Utilities|Array|Get(acopy) (Variables|Default|GetMaterialArray) (Math|Random|RandomIntegerinRange 0 5))))

(event Custom|TileOff
  (bind _cube (Variables|Default|GetCube))
  ;[0.4688 0.4688 0.4688] tile off
  (if (Variables|Default|GetbAnAttack)
    (CallFunction|Bounce (Variables|Default|GetBounceAmt))
    (bind _slowoff (Timeline|EmissiveLerpOff PlayFromStart)
      (:Update
        (bind _returnvalue (Rendering|Material|CreateDynamicMaterialInstance _cube 0 (Rendering|Material|GetMaterial _cube 0) "None" :!class /Script/Engine.PrimitiveComponent))
        (Rendering|Material|SetScalarParameterValue _returnvalue (Variables|Default|GetEmissiveParamName) (Math|Float|Lerp 0.0 3e+01 _slowoff) :!class /Script/Engine.MaterialInstanceDynamic)
        (Variables|Default|SetbCanDmg true))
      (:Finished
        (CallFunction|ChangeMaterial)
        (Variables|Default|SetbCanDmg false)
        (if (Variables|Default|GetbAnAttack)
          (CallFunction|Bounce (* (Variables|Default|GetBounceAmt) -1.0)))))
    (else
      (Timeline|EmissiveLerpOff PlayFromStart))))

(event Custom|Bounce
  (params (amt :type Float%20%28double-precision%29))
  (bind _returnvalue (Transformation|GetActorLocation))
  (bind _self self)
  (bind _returnvalue_2 (Transformation|GetActorLocation _self))
  (bind (_x _y) (Math|Vector|BreakVector _returnvalue))
  (bind _z (Math|Vector|BreakVector _returnvalue_2))
  ;[1 0.9499 0.006095] bounce for me
  (bind _bounce (Timeline|BounceActor PlayFromStart)
    (:Update
      (Transformation|SetActorLocation (Math|Vector|MakeVector _x _y (Math|Float|Lerp _z (+ _z amt) _bounce)) true false)
      (bind _outactors (Collision|SphereOverlapActors (Transformation|GetWorldLocation (Variables|Default|GetSpikeOfDeath)) 6.0 (Utilities|Array|MakeArray "ObjectTypeQuery7") 0 (Utilities|Array|MakeArray self (Variables|Default|GetBounceHit))))
      (for _array_element _outactors
        (bind _output_get (Variables|Default|SetBounceHit _array_element))
        (bind _returnvalue_3 (Game|Damage|ApplyDamage _output_get 1e+01 0 self))
        (Development|PrintString (Utilities|String|ToString(Float) _returnvalue_3) true true "(R=0.083770,G=0.203125,B=0.059229,A=1.000000)")))
    (:Finished
      (Variables|Default|SetBounceHit 0))))

(event EventBeginPlay
  ;[0.2047 1 0.1752] begin play
  (CallFunction|ChangeMaterial)
  (Components|Timeline|SetPlayRate (Variables|Default|GetEmissiveLerpOff) 6.0)
  (Components|Timeline|SetPlayRate (Variables|Default|GetBounceActor) 6.0))

(event EventTick
  (params (DeltaSeconds :type Float%20%28single-precision%29))
  ;[0 0.6901 1] tick
  (if (Variables|Default|GetbActive)
    (Utilities|FlowControl|Delay (Math|Random|RandomFloatinRange 6.0 11.0))
    (CallFunction|TileOff)))

(fn ConstructionScript)