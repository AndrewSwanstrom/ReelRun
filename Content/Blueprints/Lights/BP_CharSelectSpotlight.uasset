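; BP_CharSelectSpotlight is a spotlight actor, named for character selection, that swings to face a selected index.
; MoveSpotlight captures the light's current relative rotation, then the RotateSpotlight timeline blends it along the shortest path to a fixed downward pitch and a yaw proportional to SelectedInt.
; BeginPlay stores the origin rotation, though the move does not use it.
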(event Custom|MoveSpotlight
  (params (SelectedInt :type Integer))
  (Variables|Default|SetInitialRotation (Variables|/Script/Engine.SceneComponent|GetRelativeRotation (Variables|Default|GetSpotLight))) ; the initial rotation when called
  (bind _alpha (Timeline|RotateSpotlight PlayFromStart)
    (:Update
      (Transformation|SetRelativeRotation (Variables|Default|GetSpotLight) (Math|Rotator|Lerp(Rotator) (Variables|Default|GetInitialRotation) (Math|Rotator|MakeRotator 0.0 -6e+01 (Math|Conversions|ToFloat(Integer) (* SelectedInt 50))) _alpha true) false false))))

(event EventBeginPlay
  (Variables|Default|SetOriginRotation (Variables|/Script/Engine.SceneComponent|GetRelativeRotation (Variables|Default|GetSpotLight))) ; rotates +-30 deg based on origin
)

(fn ConstructionScript)