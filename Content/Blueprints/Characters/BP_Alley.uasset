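; BP_Alley is the playable character Alley, feeding her montages, sounds and tuning into inherited movement, camera, dash, interact and combat functions.
; Tick updates the camera and sphere-traces from foot, leg or body sockets during active attacks, with target lock adjusting rotation and FOV.
; Hits build a combo that, once full, unlocks a health-restoring finisher, signalled by an electric overlay while targeting.
; Level name selects her material, horror flag and footstep sounds.
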(event Custom|InitAlleyCustomLevelMat
  (bind _mesh (Variables|Character|GetMesh))
  (bind _returnvalue (Game|GetCurrentLevelName true))
  (if (Utilities|Array|ContainsItem (Variables|Default|GetMaterialLevelArray) _returnvalue)
    (Rendering|Material|SetMaterial _mesh 1 "/Game/Art/Characters/Alejandro/Materials/MI_Ale1_Western.MI_Ale1_Western")
    (else
      (Rendering|Material|SetMaterial _mesh 1 "/Game/Art/Characters/Alejandro/Materials/MI_Ale1_All.MI_Ale1_All"))))

(event Input|EnhancedActionEvents|EnhancedInputActionIA_Pause
  (params (ActionValue :type Boolean) (ElapsedSeconds :type Float%20%28double-precision%29) (TriggeredSeconds :type Float%20%28double-precision%29) (InputAction :type Input%20Action%20Object%20Reference :default "/Game/Blueprints/Input/Actions/IA_Pause.IA_Pause"))
  ;[0.522 1 0.2235] Pause
  (CallFunction|PausetheGame))

(event Input|EnhancedActionEvents|EnhancedInputActionIA_Dash
  (params (ActionValue :type Boolean) (ElapsedSeconds :type Float%20%28double-precision%29) (TriggeredSeconds :type Float%20%28double-precision%29) (InputAction :type Input%20Action%20Object%20Reference :default "/Game/Blueprints/Input/Actions/IA_Dash.IA_Dash"))
  ;[0.4219 0.3112 1] Dash
  (:Started
    (Variables|Default|SetAttackCount 2)
    (CallFunction|Dash 0.5 1.0 "/Game/Art/Characters/Alejandro/Anims/montage/AM_AleDash.AM_AleDash" 1.1 (Variables|Default|GetCapsuleComponent) "/Game/Art/VFX/NS_Punch.NS_Punch" "/Game/Art/SFX/Wooshes/SW_WooshSlow1.SW_WooshSlow1" (Variables|Default|GetSpeedLines) (Variables|Character|GetCharacterMovement) 8e+02 "None" (Variables|Character|GetMesh) self "Root" "Spine" 8e+01 "/Game/Art/SFX/InGame/ER_WoodBreaking.ER_WoodBreaking" 1.0)))

(event Input|EnhancedActionEvents|EnhancedInputActionIA_HeavyAttack
  (params (ActionValue :type Boolean) (ElapsedSeconds :type Float%20%28double-precision%29) (TriggeredSeconds :type Float%20%28double-precision%29) (InputAction :type Input%20Action%20Object%20Reference :default "/Game/Blueprints/Input/Actions/IA_HeavyAttack.IA_HeavyAttack"))
  ;[1 1 1] attakcs
  (:Started
    (CallFunction|HeavyAttackStart "/Game/Art/Characters/Alejandro/Anims/montage/AM_AleHeavyAttackA.AM_AleHeavyAttackA" "/Game/Art/Characters/Alejandro/Anims/montage/AM_AleHeavyAttackB.AM_AleHeavyAttackB" "/Game/Art/Characters/Alejandro/Anims/montage/AM_AleHeavyAttackC.AM_AleHeavyAttackC" 5.0 :!label _label))
  (:Ongoing
    (goto _label)))

(event Input|EnhancedActionEvents|EnhancedInputActionIA_LookH
  (params (ActionValue :type Float%20%28double-precision%29) (ElapsedSeconds :type Float%20%28double-precision%29) (TriggeredSeconds :type Float%20%28double-precision%29) (InputAction :type Input%20Action%20Object%20Reference :default "/Game/Blueprints/Input/Actions/IA_LookH.IA_LookH"))
  ;[1 0.8284 0.2855] Camera Controls
  (CallFunction|YawDirection&Lerp ActionValue))

(event Input|EnhancedActionEvents|EnhancedInputActionIA_LookV
  (params (ActionValue :type Float%20%28double-precision%29) (ElapsedSeconds :type Float%20%28double-precision%29) (TriggeredSeconds :type Float%20%28double-precision%29) (InputAction :type Input%20Action%20Object%20Reference :default "/Game/Blueprints/Input/Actions/IA_LookV.IA_LookV"))
  ;[1 0.8284 0.2855] Camera Controls
  (CallFunction|BoomArmPitch ActionValue))

(event Input|EnhancedActionEvents|EnhancedInputActionIA_LightAttack
  (params (ActionValue :type Boolean) (ElapsedSeconds :type Float%20%28double-precision%29) (TriggeredSeconds :type Float%20%28double-precision%29) (InputAction :type Input%20Action%20Object%20Reference :default "/Game/Blueprints/Input/Actions/IA_LightAttack.IA_LightAttack"))
  ;[1 1 1] attakcs
  (:Started
    (CallFunction|LightAttackStart "/Game/Art/Characters/Alejandro/Anims/montage/AM_AleLightAttackA.AM_AleLightAttackA" "/Game/Art/Characters/Alejandro/Anims/montage/AM_AleLightAttackB.AM_AleLightAttackB" "/Game/Art/Characters/Alejandro/Anims/montage/AM_AleLightAttackC.AM_AleLightAttackC" 2e+02 3e+02 :!label _label))
  (:Ongoing
    (goto _label)))

(event Input|EnhancedActionEvents|EnhancedInputActionIA_Locomotion
  (params (ActionValue :type Float%20%28double-precision%29) (ElapsedSeconds :type Float%20%28double-precision%29) (TriggeredSeconds :type Float%20%28double-precision%29) (InputAction :type Input%20Action%20Object%20Reference :default "/Game/Blueprints/Input/Actions/IA_Locomotion.IA_Locomotion"))
  ;[1 1 1] vector movement
  (:Triggered
    (Variables|Default|SetXMovementValue ActionValue))
  (:Canceled
    (Variables|Default|SetXMovementValue 0.0 :!label _label))
  (:Completed
    (goto _label)))

(event Input|EnhancedActionEvents|EnhancedInputActionIA_Strafe
  (params (ActionValue :type Float%20%28double-precision%29) (ElapsedSeconds :type Float%20%28double-precision%29) (TriggeredSeconds :type Float%20%28double-precision%29) (InputAction :type Input%20Action%20Object%20Reference :default "/Game/Blueprints/Input/Actions/IA_Strafe.IA_Strafe"))
  ;[1 1 1] vector movement
  (:Triggered
    (Variables|Default|SetYMovementValue ActionValue))
  (:Canceled
    (Variables|Default|SetYMovementValue 0.0 :!label _label))
  (:Completed
    (goto _label)))

(event Input|EnhancedActionEvents|EnhancedInputActionIA_Locomotion
  (params (ActionValue :type Float%20%28double-precision%29) (ElapsedSeconds :type Float%20%28double-precision%29) (TriggeredSeconds :type Float%20%28double-precision%29) (InputAction :type Input%20Action%20Object%20Reference :default "/Game/Blueprints/Input/Actions/IA_Locomotion.IA_Locomotion"))
  ;[1 0.2479 0.6343] Movement
  (if (Variables|Default|GetCanMove)
    (Default|Locomotion self ActionValue (Variables|Default|GetCameraYawPivot1))))

(event Input|EnhancedActionEvents|EnhancedInputActionIA_Strafe
  (params (ActionValue :type Float%20%28double-precision%29) (ElapsedSeconds :type Float%20%28double-precision%29) (TriggeredSeconds :type Float%20%28double-precision%29) (InputAction :type Input%20Action%20Object%20Reference :default "/Game/Blueprints/Input/Actions/IA_Strafe.IA_Strafe"))
  ;[1 0.2479 0.6343] Movement
  (if (Variables|Default|GetCanMove)
    (Default|Strafe self ActionValue (Variables|Default|GetCameraYawPivot1))))

(event Input|EnhancedActionEvents|EnhancedInputActionIA_Interact
  (params (ActionValue :type Boolean) (ElapsedSeconds :type Float%20%28double-precision%29) (TriggeredSeconds :type Float%20%28double-precision%29) (InputAction :type Input%20Action%20Object%20Reference :default "/Game/Blueprints/Input/Actions/IA_Interact.IA_Interact"))
  ;[1 0.2143 0.294] Interact
  (:Started
    (CallFunction|Interactable 1e+03 1e+02 1.5e+02 (Variables|Character|GetMesh) "bottleSocket" "0.700000,-0.200000,-1.000000" "1.000000,1.000000,1.000000")))

(event Input|EnhancedActionEvents|EnhancedInputActionIA_Finisher
  (params (ActionValue :type Boolean) (ElapsedSeconds :type Float%20%28double-precision%29) (TriggeredSeconds :type Float%20%28double-precision%29) (InputAction :type Input%20Action%20Object%20Reference :default "/Game/Blueprints/Input/Actions/IA_Finisher.IA_Finisher"))
  ;[1 1 1] finisher
  (:Started
    (if (>= (Variables|Default|GetComboCount) 25.0)
      (Variables|Default|SetFinisher true)
      (Variables|Default|SetbCanBeDamaged false)
      (Animation|PlayAnimMontage "/Game/Art/Characters/Alejandro/Anims/montage/AM_AlleyFinisher.AM_AlleyFinisher" 1.0 "FinStart")
      (CallFunction|IncrementActualFinisher)
      (Utilities|FlowControl|DoOnce false
        (:Completed
          (Audio|PlaySound2D "/Game/Art/SFX/InGame/closeup-sting.closeup-sting" 0.5 1.0 0.0 0 0)
          (Variables|Default|SetbCanBeDamaged true))))))

(event EventBeginPlay
  ;[0.6674 1 0.3747] Initialized Character
  (|CallParentFunction)
  (Variables|Default|SetBaseKnockback 75.0)
  (Variables|Default|SetBaseLightDamage 8.0)
  (Variables|Default|SetBaseHeavyDamage 12.0)
  (Variables|Default|SetBaseFinisherDamage 35.0)
  (CallFunction|InitAlleyCustomLevelMat)
  (CallFunction|PlayerHealth (Variables|Default|GetMAXHEALTH))
  (Transformation|SetWorldRotation (Variables|Default|GetSpringArm) (Transformation|GetActorRotation) false false)
  (CallFunction|InitAlleyInt)
  (bind _returnvalue (Game|GetCurrentLevelName true))
  (if (Utilities|Enum|Equal(Enum) _returnvalue "LV_Horror")
    (Variables|Default|SetIsHorror true)
    (else
      (Variables|Default|SetIsHorror false))))

(event Collision|EventActorBeginOverlap
  (params (OtherActor :type Actor%20Object%20Reference))
  (|CallParentFunction OtherActor) ; This node is disabled and will not be called.\nDrag off pins to build functionality.
)

(event EventTick
  (params (DeltaSeconds :type Float%20%28single-precision%29))
  (bind _mesh (Variables|Character|GetMesh))
  (bind _camerayawpivot1 (Variables|Default|GetCameraYawPivot1))
  ;[0.7507 1 0.1808] tick
  (CallFunction|TickInputVector _camerayawpivot1 (Variables|Default|GetSpringArm))
  (CallFunction|CameraBoomLerp)
  (CallFunction|AttackDamageTraceAlley)
  (if (Variables|Default|GetIs%20Targeting)
    (CallFunction|RotateTowardTarget _camerayawpivot1 "0.000000,0.000000,55.000000" 1.0)
    (Utilities|FlowControl|Sequence
      (:then_0
        (CallFunction|UpdateCameraFOV 1.2e+02)
        (if (>= (Variables|Default|GetComboCount) 25.0) :!label _label
          (Rendering|Material|SetOverlayMaterial _mesh "/Game/Materials/Instances/MI_BetsyElectric.MI_BetsyElectric" :!class /Script/Engine.MeshComponent)
          (else
            (Rendering|Material|SetOverlayMaterial _mesh 0 :!class /Script/Engine.MeshComponent))))
      (:then_1
        (goto _label_2 Reset)))
    (else
      (Utilities|FlowControl|Sequence
        (:then_0
          (Timeline|Timeline_1 Reverse
            (:Update
              (CallFunction|EndTarget)
              (goto _label))))
        (:then_1
          (Utilities|FlowControl|DoOnce false :!label _label_2
            (:Completed
              (CallFunction|UpdateCameraFOV 9e+01))))))))

(event Game|Damage|EventAnyDamage
  (params (Damage :type Float%20%28single-precision%29) (DamageType :type Damage%20Type%20Object%20Reference) (InstigatedBy :type Controller%20Object%20Reference) (DamageCauser :type Actor%20Object%20Reference))
  (bind _self self)
  ;[1 1 1] any damage
  (CallFunction|GotHit "/Game/JohnVizaria/Sounds/CombatSounds/PunchSounds/punch_1_Cue.punch_1_Cue" "/Game/Art/VFX/NS_Punch.NS_Punch" Damage)
  ;;[1 1 1] show dmg numbers?
  (if (Variables|Default|GetbShowDmgNums)
    (Game|SpawnActorfromClass "/Game/Art/VFX/Blood_And_Nums/DamageNumbers/BP_DmgNum.BP_DmgNum_C" (Transformation|GetActorTransform _self) "Undefined" "MultiplyWithRoot" _self Damage "(R=1.000000,G=0.028639,B=0.000000,A=1.000000)" 0))
  (Development|PrintString "dmged" true true "(R=1.000000,G=0.108663,B=0.000000,A=1.000000)")
  (Animation|PlayAnimMontage (.OutItem (Utilities|Array|Random (Variables|Default|GetHitAnimsBasic))) 1.0 "None"))

(event Custom|FootStepFirst
  (bind _returnvalue (Math|Random|RandomFloatinRange 0.7 1.3))
  (bind _returnvalue_2 (Game|GetCurrentLevelName true))
  ;[1 1 1] needs revision
  (switch string _returnvalue_2
    (:WesternLevel
      (Audio|PlaySound2D "/Game/Art/SFX/Western/SW_Footstep_Wood1.SW_Footstep_Wood1" 4.0 _returnvalue 0.0 0 0))
    (:TrainBlockout
      (Audio|PlaySound2D "/Game/Art/SFX/Western/SW_Footstep_Wood1.SW_Footstep_Wood1" 4.0 _returnvalue 0.0 0 0))
    (:LV_WesternAct3
      (Audio|PlaySound2D "/Game/Art/SFX/InGame/R_Footstep_Stone.R_Footstep_Stone" 1.0 _returnvalue 0.0 0 0))))

(event Custom|FootStepSecond
  (bind _returnvalue (Math|Random|RandomFloatinRange 0.7 1.3))
  (bind _returnvalue_2 (Game|GetCurrentLevelName true))
  ;[1 1 1] needs revision
  (switch string _returnvalue_2
    (:WesternLevel
      (Audio|PlaySound2D "/Game/Art/SFX/Western/SW_Footstep_Wood2.SW_Footstep_Wood2" 4.0 _returnvalue 0.0 0 0))
    (:TrainBlockout
      (Audio|PlaySound2D "/Game/Art/SFX/Western/SW_Footstep_Wood2.SW_Footstep_Wood2" 4.0 _returnvalue 0.0 0 0))
    (:LV_WesternAct3
      (Audio|PlaySound2D "/Game/Art/SFX/InGame/R2_Footstep_Stone.R2_Footstep_Stone" 1.0 _returnvalue 0.0 0 0))))

(event Custom|ResetHitSweetSound
  (Variables|Default|SetHitSound false))

(event Custom|FinisherRestoreHealth
  (if (Variables|Default|GetFinisher)
    (Variables|Default|SetComboCount 0.0)
    (if (Variables|Default|GetOnHit)
      (Audio|PlaySound2D "/Game/Art/SFX/InGame/arcade-ui-3-229508.arcade-ui-3-229508" 1.0 1.0 0.0 0 0)
      (if (> (+ (Variables|Default|GetHealth) 33.0) 1e+02)
        (Variables|Default|SetHealth 1e+02)
        (CallFunction|FinisherNums 33.0)
        (else
          (Variables|Default|SetHealth (+ (Variables|Default|GetHealth) 33.0))
          (CallFunction|FinisherNums 33.0))))
    (else
      (Development|PrintString "false"))))

(event Custom|ClearEnemies
  (Utilities|Array|Clear (Variables|Default|GetActorsToIgnore)))

(event Custom|ResetFinisher
  (Variables|Default|SetFinisher false))

(event Custom|ResetHit
  (Variables|Default|SetOnHit false))

(event Custom|WoodBreakReset
  (Variables|Default|SetSoundBreak false))

(event Custom|Alley%20Blud%20Thirst
  (CallFunction|BludThirst (Variables|Character|GetCharacterMovement) 6e+02 8.5e+02 (Variables|Default|GetBlud)))

(event Custom|SpotlightToggle
  ;[1 1 1] spotlight timer
  (Rendering|SetVisibility (Variables|Default|GetAtkSpotlight) true false)
  (Utilities|Time|SetTimerbyEvent (delegate Custom|OffSpotlight) 1.0))

(event Custom|OffSpotlight
  ;[1 1 1] spotlight timer
  (Rendering|SetVisibility (Variables|Default|GetAtkSpotlight) false false))

(event OnComponentBeginOverlap(bosstargetcollider_0)
  (params (OverlappedComponent :type Primitive%20Component%20Object%20Reference) (OtherActor :type Actor%20Object%20Reference) (OtherComp :type Primitive%20Component%20Object%20Reference) (OtherBodyIndex :type Integer) (bFromSweep :type Boolean) (SweepResult :type Hit%20Result%20Structure%20%28by%20ref%29))
  (CallFunction|StartTarget))

(event OnComponentEndOverlap(bosstargetcollider_0)
  (params (OverlappedComponent :type Primitive%20Component%20Object%20Reference) (OtherActor :type Actor%20Object%20Reference) (OtherComp :type Primitive%20Component%20Object%20Reference) (OtherBodyIndex :type Integer))
  (CallFunction|EndTarget))

(event Input|EnhancedActionEvents|EnhancedInputActionIA_Targetting
  (params (ActionValue :type Boolean) (ElapsedSeconds :type Float%20%28double-precision%29) (TriggeredSeconds :type Float%20%28double-precision%29) (InputAction :type Input%20Action%20Object%20Reference :default "/Game/Blueprints/Input/Actions/IA_Targetting.IA_Targetting"))
  (Utilities|FlowControl|FlipFlop
    (:A
      (CallFunction|StartTarget))
    (:B
      (CallFunction|EndTarget))))

(fn ConstructionScript
  (|CallParentFunction))

(fn CameraBoomLerp
  (CallFunction|CameraLerp (Variables|Default|GetCameraBoomPitchPivot1) (Variables|Default|GetCameraYawPivot1) (Variables|Default|GetActualSpringArm1) (Variables|Default|GetBoomCameraFocusPoint1)))

(fn AttackDamageTraceAlley
  (bind _returnvalue (Game|GetPlayerController 0))
  ;[1 1 1] Multi Trace Damage
  (Utilities|IsValid _returnvalue
    (:Is%20Valid
      (Rendering|Material|SetVectorParameterValue "/Game/Materials/Functions/MPC_GetPlayerPosition.MPC_GetPlayerPosition" "MainCharacterLocation" (Math|Conversions|ToLinearColor(Vector) (Transformation|GetActorLocation _returnvalue)) :!class /Script/Engine.KismetMaterialLibrary)
      (if (Variables|Default|GetFistActive)
        ;;[0.9643 1 0.4549] Define Light Attack & Start Multi Sphere Trace
        (switch int (Variables|Default|GetAttackCount)
          (:0
            (Variables|Default|SetSocketStart "LeftFootStart")
            (Variables|Default|SetSocketEnd "LeftFootEnd"))
          (:1
            (Variables|Default|SetSocketStart "LeftFootStart")
            (Variables|Default|SetSocketEnd "LeftFootEnd"))
          (:2
            (Variables|Default|SetSocketStart "RightLegStart")
            (Variables|Default|SetSocketEnd "RightLegEnd"))
          (:3
            (Variables|Default|SetSocketStart "RightLegStart")
            (Variables|Default|SetSocketEnd "RightLegEnd")))
        (CallFunction|AttackTrace (Variables|Character|GetMesh) (Variables|Default|GetSocketStart) (Variables|Default|GetSocketEnd) 3e+01 "/Game/Art/VFX/NS_Punch.NS_Punch" "/Game/Art/SFX/InGame/ER_WoodBreaking.ER_WoodBreaking" (Variables|Default|GetBaseLightDamage) self "/Game/Blueprints/Damaging/DT_PlayerLightAttack.DT_PlayerLightAttack_C" "/Game/Art/SFX/InGame/SW_HitSweetner3.SW_HitSweetner3" 2.0 3.0)
        (elif (Variables|Default|GetHeavyActive)
          (Variables|Default|SetSocketStart "BodyStart")
          (Variables|Default|SetSocketEnd "BodyEnd")
          (CallFunction|AttackTrace (Variables|Character|GetMesh) (Variables|Default|GetSocketStart) (Variables|Default|GetSocketEnd) (Variables|Default|GetHeavyTraceSize) "/Game/Art/VFX/NS_Punch.NS_Punch" "/Game/Art/SFX/InGame/ER_WoodBreaking.ER_WoodBreaking" (Math|Float|SelectFloat (Variables|Default|GetBaseFinisherDamage) (Variables|Default|GetBaseHeavyDamage) (Variables|Default|GetFinisher)) self "/Game/Blueprints/Damaging/DT_PlayerHeavyAttack.DT_PlayerHeavyAttack_C" "/Game/Art/SFX/InGame/SW_HitSweetner3.SW_HitSweetner3" 1.0 2.0))))))