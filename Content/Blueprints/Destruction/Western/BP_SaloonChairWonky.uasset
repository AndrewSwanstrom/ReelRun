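; BP_SaloonChairWonky is a destructible western saloon chair built on a Chaos geometry collection.
; On a Chaos break event, it fires a transient field from culling, radial falloff and radial vector components at the destruction center, then applies very high internal strain there to force the break apart.
; It also destroys the invisible collision box and moves the debris to another collision object type.
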(event OnChaosBreakEvent(GC_Sm_SaloonChairs_02a)
  (params (BreakEvent :type Chaos%20Break%20Event%20Structure%20%28by%20ref%29))
  (bind _destructioncenter (Variables|Default|GetDestructionCenter))
  (bind _box (Variables|Default|GetBox))
  ;[1 1 1] On Chaos Break Event
  ;;[0.2371 0.3006 1] Add Velocity Field
  (CallFunction|TransientField (Variables|Default|GetFieldSystem) (Variables|Default|GetCullingField) (Variables|Default|GetRadialFalloff) (Variables|Default|GetRadialVector) _destructioncenter (Variables|Default|GetSphere))
  (Class|GeometryCollectionComponent|ApplyInternalStrain (Variables|Default|GetGC_Sm_SaloonChairs_02a) 0 _destructioncenter 1e+02 0 1.0 1e+15)
  ;;[1 0.12 0.2097] Destroy Invisible Collision Box when chaos break happens
  (Utilities|IsValid _box
    (:Is%20Valid
      (Components|DestroyComponent _box)
      ;;[0.214 1 0.2762] Disable Event Tick, change collisoin type
      (Collision|SetCollisionObjectType (Variables|Default|GetGC_Sm_SaloonChairs_02a) "ECC_GameTraceChannel2"))))

(event EventTick
  (params (DeltaSeconds :type Float%20%28single-precision%29)))

(fn ConstructionScript)