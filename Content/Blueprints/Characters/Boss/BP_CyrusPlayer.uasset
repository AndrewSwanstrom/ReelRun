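; Playable Cyrus character that sets its own damage values, montages and effects on top of shared parent combat logic.
; Enhanced Input drives movement, camera, dash, interaction, light/heavy attacks and a finisher unlocked at high combo, signalled by an electric overlay.
; Tick updates camera and lock-on, publishes player location to a material parameter collection, and runs socket-based attack traces.
; Heavy traces use finisher damage rather than heavy damage.
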(event Input|EnhancedActionEvents|EnhancedInputActionIA_Dash
  (params (ActionValue :type Boolean) (ElapsedSeconds :type Float%20%28double-precision%29) (TriggeredSeconds :type Float%20%28double-precision%29) (InputAction :type Input%20Action%20Object%20Reference :default "/Game/Blueprints/Input/Actions/IA_Dash.IA_Dash"))
  (:Started
    (CallFunction|Dash 0.5 1.0 0 1.1 (Variables|Default|GetCapsuleComponent) "/Game/Art/VFX/NS_Punch.NS_Punch" "/Game/Art/SFX/Wooshes/SW_WooshSlow1.SW_WooshSlow1" (Variables|Default|GetSpeedLines) (Variables|Character|GetCharacterMovement) 8e+02 "None" (Variables|Character|GetMesh) self "Root" "Spine" 8e+01 "/Game/Art/SFX/InGame/ER_WoodBreaking.ER_WoodBreaking" 1.0)))

(event Input|EnhancedActionEvents|EnhancedInputActionIA_Pause
  (params (ActionValue :type Boolean) (ElapsedSeconds :type Float%20%28double-precision%29) (TriggeredSeconds :type Float%20%28double-precision%29) (InputAction :type Input%20Action%20Object%20Reference :default "/Game/Blueprints/Input/Actions/IA_Pause.IA_Pause"))
  ;[0.522 1 0.2235] Pause
  (CallFunction|PausetheGame))

(event Input|EnhancedActionEvents|EnhancedInputActionIA_HeavyAttack
  (params (ActionValue :type Boolean) (ElapsedSeconds :type Float%20%28double-precision%29) (TriggeredSeconds :type Float%20%28double-precision%29) (InputAction :type Input%20Action%20Object%20Reference :default "/Game/Blueprints/Input/Actions/IA_HeavyAttack.IA_HeavyAttack"))
  (:Started
    (Default|HeavyAttackStart self "/Game/Art/Characters/Enemies/WesternBoss/Animations/Monmtages/AM_CyrusPlayerHeavy.AM_CyrusPlayerHeavy" "/Game/Art/Characters/Enemies/WesternBoss/Animations/Monmtages/AM_CyrusPlayerHeavy.AM_CyrusPlayerHeavy" "/Game/Art/Characters/Enemies/WesternBoss/Animations/Monmtages/AM_CyrusPlayerHeavy.AM_CyrusPlayerHeavy" 2e+02)
    (CallFunction|DebugNuke)))

(event Input|EnhancedActionEvents|EnhancedInputActionIA_LookH
  (params (ActionValue :type Float%20%28double-precision%29) (ElapsedSeconds :type Float%20%28double-precision%29) (TriggeredSeconds :type Float%20%28double-precision%29) (InputAction :type Input%20Action%20Object%20Reference :default "/Game/Blueprints/Input/Actions/IA_LookH.IA_LookH"))
  (CallFunction|YawDirection&Lerp ActionValue))

(event Input|EnhancedActionEvents|EnhancedInputActionIA_LookV
  (params (ActionValue :type Float%20%28double-precision%29) (ElapsedSeconds :type Float%20%28double-precision%29) (TriggeredSeconds :type Float%20%28double-precision%29) (InputAction :type Input%20Action%20Object%20Reference :default "/Game/Blueprints/Input/Actions/IA_LookV.IA_LookV"))
  (CallFunction|BoomArmPitch ActionValue))

(event Input|EnhancedActionEvents|EnhancedInputActionIA_LightAttack
  (params (ActionValue :type Boolean) (ElapsedSeconds :type Float%20%28double-precision%29) (TriggeredSeconds :type Float%20%28double-precision%29) (InputAction :type Input%20Action%20Object%20Reference :default "/Game/Blueprints/Input/Actions/IA_LightAttack.IA_LightAttack"))
  (:Started
    (Default|LightAttackStart self "/Game/Art/Characters/Enemies/WesternBoss/Animations/Monmtages/AM_CyrusPlayerLight.AM_CyrusPlayerLight" "/Game/Art/Characters/Enemies/WesternBoss/Animations/Monmtages/AM_CyrusPlayerLight.AM_CyrusPlayerLight" "/Game/Art/Characters/Enemies/WesternBoss/Animations/Monmtages/AM_CyrusPlayerLight.AM_CyrusPlayerLight" 2.5e+02 3e+02)
    (CallFunction|DebugNuke)))

(event Input|EnhancedActionEvents|EnhancedInputActionIA_Locomotion
  (params (ActionValue :type Float%20%28double-precision%29) (ElapsedSeconds :type Float%20%28double-precision%29) (TriggeredSeconds :type Float%20%28double-precision%29) (InputAction :type Input%20Action%20Object%20Reference :default "/Game/Blueprints/Input/Actions/IA_Locomotion.IA_Locomotion"))
  (:Triggered
    (Variables|Default|SetXMovementValue ActionValue))
  (:Canceled
    (Variables|Default|SetXMovementValue 0.0 :!label _label))
  (:Completed
    (goto _label)))

(event Input|EnhancedActionEvents|EnhancedInputActionIA_Strafe
  (params (ActionValue :type Float%20%28double-precision%29) (ElapsedSeconds :type Float%20%28double-precision%29) (TriggeredSeconds :type Float%20%28double-precision%29) (InputAction :type Input%20Action%20Object%20Reference :default "/Game/Blueprints/Input/Actions/IA_Strafe.IA_Strafe"))
  (:Triggered
    (Variables|Default|SetYMovementValue ActionValue))
  (:Canceled
    (Variables|Default|SetYMovementValue 0.0 :!label _label))
  (:Completed
    (goto _label)))

(event Input|EnhancedActionEvents|EnhancedInputActionIA_Locomotion
  (params (ActionValue :type Float%20%28double-precision%29) (ElapsedSeconds :type Float%20%28double-precision%29) (TriggeredSeconds :type Float%20%28double-precision%29) (InputAction :type Input%20Action%20Object%20Reference :default "/Game/Blueprints/Input/Actions/IA_Locomotion.IA_Locomotion"))
  (if (Variables|Default|GetCanMove)
    (Default|Locomotion self ActionValue (Variables|Default|GetCameraYawPivot1))))

(event Input|EnhancedActionEvents|EnhancedInputActionIA_Strafe
  (params (ActionValue :type Float%20%28double-precision%29) (ElapsedSeconds :type Float%20%28double-precision%29) (TriggeredSeconds :type Float%20%28double-precision%29) (InputAction :type Input%20Action%20Object%20Reference :default "/Game/Blueprints/Input/Actions/IA_Strafe.IA_Strafe"))
  (if (Variables|Default|GetCanMove)
    (Default|Strafe self ActionValue (Variables|Default|GetCameraYawPivot1))))

(event Input|EnhancedActionEvents|EnhancedInputActionIA_Interact
  (params (ActionValue :type Boolean) (ElapsedSeconds :type Float%20%28double-precision%29) (TriggeredSeconds :type Float%20%28double-precision%29) (InputAction :type Input%20Action%20Object%20Reference :default "/Game/Blueprints/Input/Actions/IA_Interact.IA_Interact"))
  (:Started
    (CallFunction|Interactable 1e+03 1e+02 1.5e+02 (Variables|Character|GetMesh) "bottleSocket" "0.700000,-0.200000,-1.000000" "1.000000,1.000000,1.000000")))

(event Input|EnhancedActionEvents|EnhancedInputActionIA_Finisher
  (params (ActionValue :type Boolean) (ElapsedSeconds :type Float%20%28double-precision%29) (TriggeredSeconds :type Float%20%28double-precision%29) (InputAction :type Input%20Action%20Object%20Reference :default "/Game/Blueprints/Input/Actions/IA_Finisher.IA_Finisher"))
  (:Started
    (if (>= (Variables|Default|GetComboCount) 25.0)
      (Variables|Default|SetFinisher true)
      (Animation|PlayAnimMontage 0 1.0 "FinStart")
      (CallFunction|IncrementActualFinisher)
      (Utilities|FlowControl|DoOnce false
        (:Completed
          (Audio|PlaySound2D "/Game/Art/SFX/InGame/closeup-sting.closeup-sting" 0.5 1.0 0.0 0 0))))))

(event EventBeginPlay
  (|CallParentFunction)
  (Variables|Default|SetBaseKnockback 75.0)
  (Variables|Default|SetBaseLightDamage 16.0)
  (Variables|Default|SetBaseHeavyDamage 35.0)
  (Variables|Default|SetBaseFinisherDamage 1e+02)
  (CallFunction|PlayerHealth (Variables|Default|GetMAXHEALTH))
  (Transformation|SetWorldRotation (Variables|Default|GetSpringArm) (Transformation|GetActorRotation) false false)
  (CallFunction|InitAlleyInt)
  (bind _returnvalue (Game|GetCurrentLevelName true))
  (if (Utilities|Enum|Equal(Enum) _returnvalue "LV_Horror")
    (Variables|Default|SetIsHorror true)
    (else
      (Variables|Default|SetIsHorror false))))

(event EventTick
  (params (DeltaSeconds :type Float%20%28single-precision%29))
  (bind _mesh (Variables|Character|GetMesh))
  (bind _camerayawpivot1 (Variables|Default|GetCameraYawPivot1))
  (CallFunction|TickInputVector _camerayawpivot1 (Variables|Default|GetSpringArm))
  (CallFunction|CameraBoomLerp)
  (CallFunction|AttackDamageTraceCyrus)
  (if (Variables|Default|GetIs%20Targeting)
    (CallFunction|RotateTowardTarget _camerayawpivot1 "0.000000,0.000000,55.000000" 1.0)
    (Utilities|FlowControl|Sequence
      (:then_0
        (CallFunction|UpdateCameraFOV 1.2e+02)
        (if (>= (Variables|Default|GetComboCount) 25.0) :!label _label
          (Rendering|Material|SetOverlayMaterial _mesh "/Game/Materials/Instances/MI_BetsyElectric.MI_BetsyElectric" :!class /Script/Engine.MeshComponent)
          (else
            (Rendering|Material|SetOverlayMaterial _mesh 0 :!class /Script/Engine.MeshComponent))))
      (:then_1
        (goto _label_2 Reset)))
    (else
      (Utilities|FlowControl|Sequence
        (:then_0
          (Timeline|Timeline_6 Reverse
            (:Update
              (CallFunction|EndTarget)
              (goto _label))))
        (:then_1
          (Utilities|FlowControl|DoOnce false :!label _label_2
            (:Completed
              (CallFunction|UpdateCameraFOV 9e+01))))))))

(event Game|Damage|EventAnyDamage
  (params (Damage :type Float%20%28single-precision%29) (DamageType :type Damage%20Type%20Object%20Reference) (InstigatedBy :type Controller%20Object%20Reference) (DamageCauser :type Actor%20Object%20Reference))
  (bind _self self)
  ;[1 1 1] damage
  (CallFunction|GotHit "/Game/JohnVizaria/Sounds/CombatSounds/PunchSounds/punch_1_Cue.punch_1_Cue" "/Game/Art/VFX/NS_Punch.NS_Punch" Damage)
  (if (Variables|Default|GetbShowDmgNums)
    (Game|SpawnActorfromClass "/Game/Art/VFX/Blood_And_Nums/DamageNumbers/BP_DmgNum.BP_DmgNum_C" (Transformation|GetActorTransform _self) "Undefined" "MultiplyWithRoot" _self Damage "(R=1.000000,G=0.028639,B=0.000000,A=1.000000)" 0)))

(fn ConstructionScript
  (|CallParentFunction))

(fn CameraBoomLerp
  (CallFunction|CameraLerp (Variables|Default|GetCameraBoomPitchPivot1) (Variables|Default|GetCameraYawPivot1) (Variables|Default|GetActualSpringArm1) (Variables|Default|GetBoomCameraFocusPoint1)))

(fn AttackDamageTraceCyrus
  (bind _returnvalue (Game|GetPlayerController 0))
  (Utilities|IsValid _returnvalue
    (:Is%20Valid
      (Rendering|Material|SetVectorParameterValue "/Game/Materials/Functions/MPC_GetPlayerPosition.MPC_GetPlayerPosition" "MainCharacterLocation" (Math|Conversions|ToLinearColor(Vector) (Transformation|GetActorLocation _returnvalue)) :!class /Script/Engine.KismetMaterialLibrary)
      (if (Variables|Default|GetFistActive)
        ;[0.9643 1 0.4549] Define Light Attack & Start Multi Sphere Trace
        (switch int (Variables|Default|GetAttackCount)
          (:0
            (Variables|Default|SetSocketStart "LeftFootStart")
            (Variables|Default|SetSocketEnd "LeftFootEnd"))
          (:1
            (Variables|Default|SetSocketStart "LeftFootStart")
            (Variables|Default|SetSocketEnd "LeftFootEnd"))
          (:2
            (Variables|Default|SetSocketStart "RightLegStart")
            (Variables|Default|SetSocketEnd "RightLegEnd"))
          (:3
            (Variables|Default|SetSocketStart "RightLegStart")
            (Variables|Default|SetSocketEnd "RightLegEnd")))
        (CallFunction|AttackTrace (Variables|Character|GetMesh) (Variables|Default|GetSocketStart) (Variables|Default|GetSocketEnd) 3e+01 "/Game/Art/VFX/NS_Punch.NS_Punch" "/Game/Art/SFX/InGame/ER_WoodBreaking.ER_WoodBreaking" (Variables|Default|GetBaseLightDamage) self "/Game/Blueprints/Damaging/DT_PlayerLightAttack.DT_PlayerLightAttack_C" "/Game/Art/SFX/InGame/SW_HitSweetner3.SW_HitSweetner3" 2.0 4.0)
        (elif (Variables|Default|GetHeavyActive)
          (Variables|Default|SetSocketStart "BodyStart")
          (Variables|Default|SetSocketEnd "BodyEnd")
          (CallFunction|AttackTrace (Variables|Character|GetMesh) (Variables|Default|GetSocketStart) (Variables|Default|GetSocketEnd) (Variables|Default|GetHeavyTraceSize) "/Game/Art/VFX/NS_Punch.NS_Punch" "/Game/Art/SFX/InGame/ER_WoodBreaking.ER_WoodBreaking" (Variables|Default|GetBaseFinisherDamage) self "/Game/Blueprints/Damaging/DT_PlayerHeavyAttack.DT_PlayerHeavyAttack_C" "/Game/Art/SFX/InGame/SW_HitSweetner3.SW_HitSweetner3" 1.0 4.0))))))