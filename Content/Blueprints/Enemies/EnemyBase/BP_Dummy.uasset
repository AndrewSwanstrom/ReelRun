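; BP_Dummy is a light melee enemy that takes hits, gets knocked back and attacks with its fists.
; Damage plays sound and montage, then a timeline applies causer-specific knockback before subtracting health and resetting the blackboard state.
; At zero health it unpossesses, dissolves, ragdolls and is destroyed.
; Attacks reserve tokens from the target, while Tick runs socket traces for fist hits and knockback collisions.
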(event Custom|EnemyKnockback
  (bind _self self)
  (bind _returnvalue (AI|GetAIController _self))
  (bind _returnvalue_2 (AI|GetBlackboard _returnvalue))
  ;[1 0.3575 0.5391] Force Enemy Into Knock Back State
  (Utilities|IsValid _returnvalue_2
    (:Is%20Valid
      (CallFunction|KnockBackState _returnvalue_2 (Variables|Default|GetKey) (Utilities|Enum|LiteralenumLightEnemy "NewEnumerator8")))))

(event Custom|AttackAnim
  (params (AttackTarget :type Actor%20Object%20Reference))
  ;[0.1832 1 0.2887] Play Attack Animations
  (bind _success (Class|BPIDamageable|ReserveAttackToken(Message) AttackTarget 1))
  (if _success
    (Animation|Montage|PlayMontage (Variables|Character|GetMesh) "/Game/Art/Characters/Enemies/Light/Animations/Montage/Anim_LightEnemyAttack_Montage.Anim_LightEnemyAttack_Montage"
      (:OnCompleted
        _)
      (:OnInterrupted
        _)))
  (Default|CallOnAttackEnd)
  (Utilities|IsValid AttackTarget
    (:Is%20Valid
      (Class|BPIDamageable|ReturnToken(Message) AttackTarget 1))))

(event Game|Damage|EventAnyDamage
  (params (Damage :type Float%20%28single-precision%29) (DamageType :type Damage%20Type%20Object%20Reference) (InstigatedBy :type Controller%20Object%20Reference) (DamageCauser :type Actor%20Object%20Reference))
  (bind _returnvalue (Transformation|GetActorLocation))
  (bind _returnvalue_2 (Pawn|GetController))
  (bind _self self)
  (bind _self_2 self)
  (bind _self_3 self)
  (bind _mesh (Variables|Character|GetMesh))
  (bind _returnvalue_3 (Transformation|GetActorTransform _self_3))
  (bind _returnvalue_4 (AI|GetAIController _self))
  (bind _returnvalue_5 (AI|GetBlackboard _returnvalue_4))
  ;[0.1357 0.2884 1] Receive Damage
  (Audio|PlaySoundatLocation "/Game/Art/SFX/RandomHitCue.RandomHitCue" _returnvalue "0, 0, 0" 1.0 (Math|Random|RandomFloatinRange 0.5 1.3) 0.0 0 0 0 0)
  (Audio|PlaySoundatLocation (.OutItem (Utilities|Array|Random (Variables|Default|GetHitSounds))) _returnvalue "0, 0, 0" 1.0 1.0 0.0 0 0 0 0)
  ;;[1 1 1] show dmg numbers?
  (if (Variables|Default|GetShowDmgNums?)
    (Game|SpawnActorfromClass "/Game/Art/VFX/Blood_And_Nums/DamageNumbers/BP_DmgNum.BP_DmgNum_C" (Transformation|GetActorTransform _self_2) "Undefined" "MultiplyWithRoot" _self_2 (* Damage 1e+01) "(R=0.000000,G=0.000000,B=0.000000,A=0.000000)" 0))
  (bind _asbase_character (Utilities|Casting|CastToBase_Character DamageCauser)
    (:then
      (Variables|Default|SetCustomKnockbackForce (Variables|/Game/Blueprints/Characters/Base_Character.Base_Character_C|GetKnockBackForce _asbase_character))
      ;;[1 1 1] is dmg causer syd
      (if (Variables|/Game/Blueprints/Characters/Base_Character.Base_Character_C|GetSyd _asbase_character)
        (AddComponent|AddNiagaraComponent false)))
    (:CastFailed
      (bind _asbp_throwable_base_obj (Utilities|Casting|CastToBP_ThrowableBaseObj DamageCauser)
        (:then
          (Variables|Default|SetCustomKnockbackForce (Variables|/Game/Blueprints/Throwables/BP_ThrowableBaseObj.BP_ThrowableBaseObj_C|GetThrowableKnockback _asbp_throwable_base_obj)))
        (:CastFailed
          (Variables|Default|SetCustomKnockbackForce 9e+02)))))
  (Animation|Montage|PlayMontage (Variables|Character|GetMesh) "/Game/Art/Characters/Enemies/Light/Animations/Montage/Anim_LightEnemyDamage_Montage.Anim_LightEnemyDamage_Montage"
    (:then
      (CallFunction|EnemyKnockback)
      (bind _alpha (Timeline|Timeline_0 PlayFromStart)
        (:Update
          (if (== (Variables|Default|GetCustomTimeDilation) 1.0)
            (CallFunction|StartKnockBack _alpha (Variables|Default|GetCustomKnockbackForce))))
        (:Finished
          (Utilities|FlowControl|Delay 0.2)
          (Variables|Default|SetIsOverlapping false)
          (Utilities|IsValid _returnvalue_5
            (:Is%20Valid
              (CallFunction|KnockBackState _returnvalue_5 (Variables|Default|GetKey) (Utilities|Enum|LiteralenumLightEnemy "NewEnumerator0"))
              (bind _output_get (Variables|Default|SetHealth (- (Variables|Default|GetHealth) Damage)))
              (if (<= _output_get 0.0)
                (Variables|Default|SetbECanBeDamaged false)
                (Utilities|IsValid _returnvalue_2
                  (:Is%20Valid
                    (Pawn|UnPossess _returnvalue_2)
                    (Animation|PlayAnimMontage 0 0.2 "None")
                    (Niagara|SpawnSystematLocation "/Game/Art/VFX/MeshSprites/LightEnemySprites.LightEnemySprites" (.location _returnvalue_3) (.rotation _returnvalue_3) (.scale _returnvalue_3))
                    (bind _slowoff (Timeline|Timeline PlayFromStart)
                      (:Update
                        (bind _returnvalue_6 (Rendering|Material|CreateDynamicMaterialInstance (Variables|Character|GetMesh) 0 "/Game/Art/VFX/NS_EdgeBurnv1/MI_EnemyDissolve.MI_EnemyDissolve" "None" :!class /Script/Engine.PrimitiveComponent))
                        (Rendering|Material|SetScalarParameterValue _returnvalue_6 "Dissolve" (Math|Float|Lerp 5.0 0.0 _slowoff) :!class /Script/Engine.MaterialInstanceDynamic)
                        (Rendering|Material|SetScalarParameterValue _returnvalue_6 "DissolveWidth" (Math|Float|Lerp 5.0 0.0 _slowoff) :!class /Script/Engine.MaterialInstanceDynamic)
                        (Physics|SetSimulatePhysics _mesh true)
                        (Collision|SetCollisionProfileName _mesh "Ragdoll" true :!class /Script/Engine.PrimitiveComponent)
                        (Utilities|FlowControl|Delay 1.0)
                        (Actor|DestroyActor)))))))))))))

(event EventTick
  (params (DeltaSeconds :type Float%20%28single-precision%29))
  ;[0.3462 0.666 1] Event Tick
  (if (Variables|Default|GetIsOverlapping)
    (CallFunction|KnockBackTrace (Variables|Character|GetMesh) (Variables|Default|GetTrace%20Start) (Variables|Default|GetTrace%20End) 3e+01 "/Game/Art/SFX/InGame/ER_WoodBreaking.ER_WoodBreaking")
    (else
      ;;[1 0.3008 0.6326] Event Tick Line Trace Damage Logic
      (if (Variables|Default|GetLeftFistAttack)
        (Variables|Default|SetSocketStart "LeftHandStart")
        (Variables|Default|SetSocketEnd "LeftHandEnd")
        (CallFunction|AttackTrace (Variables|Character|GetMesh) (Variables|Default|GetSocketStart) (Variables|Default|GetSocketEnd) 2e+01 1e+03 self 5.0 "/Game/Art/SFX/InGame/ER_WoodBreaking.ER_WoodBreaking" :!label _label)
        (elif (Variables|Default|GetRightFistAttack)
          (Variables|Default|SetSocketStart "RightHandStart")
          (Variables|Default|SetSocketEnd "RightHandEnd")
          (goto _label))))))

(event EventAttack
  (params (AttackTarget :type Actor%20Object%20Reference)))

(event EventStoreAttackTokens
  (params (AttackTarget :type Actor%20Object%20Reference) (Amount :type Integer))
  (bind _reservedattacktokens (Variables|Default|GetReservedAttackTokens))
  (bind (_value _returnvalue) (Utilities|Map|Find _reservedattacktokens AttackTarget))
  ;[1 1 1] Experimental Code
  (Utilities|Map|Add (Variables|Default|GetReservedAttackTokens) AttackTarget (Math|Integer|SelectInt (+ Amount _value) Amount _returnvalue)))

(event EventTakeDamage)

(event EventGetCurrentHealth)

(event EventAttackEnd
  (params (AttackTarget :type Actor%20Object%20Reference))
  (bind _token_used_current (Variables|Default|GetToken%20Used%20Current))
  ;[1 1 1] Experimental Code
  (Class|BPIDamageable|ReturnToken(Message) AttackTarget _token_used_current)
  (CallFunction|StoreAttackTokens AttackTarget (* _token_used_current -1))
  (Default|CallOnAttackEnd))

(event EventReturnToken
  (params (Amount :type Integer)))

(event Custom|Clear%20Attack%20Stack%20Light
  ;[1 0.2424 0.4752] Clear Light Attack Stack
  (Utilities|Array|Clear (Variables|Default|GetActorsIgnore)))

(event Custom|LightSoundReset
  ;[1 0.8174 0.4385] Light Sound Reset
  (Variables|Default|SetBreakSound false))

(event Custom|ResetFirstTimer
  (Variables|Default|SetCanSwapLayerFirst false))

(event Custom|ResetSecondTimer
  (Variables|Default|SetCanSwapLayerSecond false))

(event Custom|Reset%20First%20Count
  (Variables|Default|SetFirstLayerCount 0))

(event Custom|ResetSecondCount
  (Variables|Default|SetSecondLayerCount 0))

(fn ConstructionScript
  (Variables|Default|SetAttackTokenCount 2))

(fn AttackStart
  (params (AttackTarget :type Actor%20Object%20Reference) (Tokens%20Needed :type Integer))
  (bind _success (Class|BPIDamageable|ReserveAttackToken(Message) AttackTarget Tokens%20Needed))
  (if _success
    (CallFunction|StoreAttackTokens AttackTarget Tokens%20Needed)
    (Variables|Default|SetToken%20Used%20Current Tokens%20Needed)
    (return true)
    (else
      (return false))))

(fn GetIdealRange
  (return 1.2e+02 2.5e+02 4.5e+02))

(fn ReserveAttackToken
  (params (Amount :type Integer)))

(fn SetMovementSpeed
  (params (Speed :type E_MovementSpeed%20Enum :default "NewEnumerator0"))
  ;[1 1 1] Movement Speed Function
  (bind _output_get (Variables|/Script/Engine.CharacterMovementComponent|SetMaxWalkSpeed (Variables|Character|GetCharacterMovement) (Utilities|Select :Index Speed :NewEnumerator0 0.0 :NewEnumerator1 2.5e+02 :NewEnumerator2 5e+02 :NewEnumerator4 0.0)))
  (return _output_get))