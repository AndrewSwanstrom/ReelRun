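; BP_SPBombv1 is a bomb actor that deals player heavy-attack damage to enemies.
; When its damage flag is on, Creation triggers a radial blast credited to the player and ignoring their character, and Dmg component overlaps hurt BaseEnemy actors.
; Custom events toggle the flag and set lifespan, which Creation also sets.
; The shockwave effect and damage-off timer are unwired.
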(event OnComponentBeginOverlap(dmg)
  (params (OverlappedComponent :type Primitive%20Component%20Object%20Reference) (OtherActor :type Actor%20Object%20Reference) (OtherComp :type Primitive%20Component%20Object%20Reference) (OtherBodyIndex :type Integer) (bFromSweep :type Boolean) (SweepResult :type Hit%20Result%20Structure%20%28by%20ref%29))
  (if (Variables|Default|Getbcandmg)
    (bind _asbase_enemy (Utilities|Casting|CastToBaseEnemy OtherActor))
    (Game|Damage|ApplyDamage _asbase_enemy 1e+02 0 self "/Game/Blueprints/Damaging/DT_PlayerHeavyAttack.DT_PlayerHeavyAttack_C")))

(event Custom|lifespan
  (params (InLifespan :type Float%20%28single-precision%29))
  (Actor|SetLifeSpan InLifespan))

(event Custom|creation
  (Actor|SetLifeSpan 5.0)
  (CallFunction|DmgEnemies))

(event Custom|can%20dmg
  (Variables|Default|Setbcandmg true))

(event Custom|no%20dmg
  (Variables|Default|Setbcandmg false))

(event Custom|dmg%20enemies
  (if (Variables|Default|Getbcandmg)
    (bind _returnvalue (Actor|GetActorOfClass "/Game/Blueprints/Characters/Base_Character.Base_Character_C"))
    (Game|Damage|ApplyRadialDamage 1e+02 (.location (Transformation|GetActorTransform)) 1e+03 "/Game/Blueprints/Damaging/DT_PlayerHeavyAttack.DT_PlayerHeavyAttack_C" (Utilities|Array|MakeArray _returnvalue) _returnvalue (Game|GetPlayerController 0) false "ECC_Camera")))

(fn ConstructionScript)