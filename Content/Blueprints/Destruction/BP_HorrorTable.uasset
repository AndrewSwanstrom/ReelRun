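; BP_HorrorTable is a destructible table prop built on a Chaos geometry collection.
; When the collection breaks, it applies a transient field around the destruction center, using radial falloff, radial vector and culling inputs.
; If the Box component is still valid, it destroys it, sets a CanTick flag and switches the debris to a custom collision channel.
; After a delay, it turns off the debris' physics and collision.
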(event OnChaosBreakEvent(gc_table)
  (params (BreakEvent :type Chaos%20Break%20Event%20Structure%20%28by%20ref%29))
  (bind _box (Variables|Default|GetBox))
  (CallFunction|TransientField (Variables|Default|GetFieldSystem) (Variables|Default|GetCullingField) (Variables|Default|GetRadialFalloff) (Variables|Default|GetRadialVector) (Variables|Default|GetDestructionCenter) (Variables|Default|GetSphere))
  (Utilities|IsValid _box
    (:Is%20Valid
      (Components|DestroyComponent _box)
      (Variables|Default|SetCanTick true)
      (Collision|SetCollisionObjectType (Variables|Default|Getgc_table) "ECC_GameTraceChannel2")
      (Utilities|FlowControl|Delay 15.0)
      (Physics|SetSimulatePhysics (Variables|Default|Getgc_table) false)
      (Collision|SetCollisionEnabled (Variables|Default|Getgc_table) "NoCollision"))))

(fn ConstructionScript)