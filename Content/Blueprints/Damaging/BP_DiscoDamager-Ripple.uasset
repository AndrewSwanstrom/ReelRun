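; A ripple variant of the disco damager actor that sinks downward after spawning, then removes itself.
; On BeginPlay it stores its starting location and plays a timeline that lerps only its Z position down by a fixed depth, destroying the actor when the timeline finishes.
; The construction script only calls the parent's, and this file adds no damage logic of its own.
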(event EventBeginPlay
  (bind _returnvalue (Transformation|GetActorLocation))
  (Variables|Default|SetInitialPosition (Transformation|GetActorLocation))
  (bind _alpha (Timeline|Timeline PlayFromStart)
    (:Update
      (Transformation|SetActorLocation (Math|Vector|MakeVector (.x _returnvalue) (.y _returnvalue) (Math|Float|Lerp (.z (Variables|Default|GetInitialPosition)) (- (.z (Variables|Default|GetInitialPosition)) 9.6e+02) _alpha)) false false))
    (:Finished
      (Actor|DestroyActor))))

(fn ConstructionScript
  (|CallParentFunction))