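; BP_SandbagShooterEnemy is an enemy that turns to face the player and fires projectiles on a cooldown.
; Tick sets yaw toward the player and, on a real-time timer, spawns a BP_Damager ahead, pushes it with an impulse and plays a Niagara muzzle flash.
; BeginPlay calls RunBehaviorTree with no tree asset shown, while aiming and firing run in Tick.
; AnyDamage lowers Health and destroys the actor below zero.
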(event Game|Damage|EventAnyDamage
  (params (Damage :type Float%20%28single-precision%29) (DamageType :type Damage%20Type%20Object%20Reference) (InstigatedBy :type Controller%20Object%20Reference) (DamageCauser :type Actor%20Object%20Reference))
  (bind _output_get (Variables|Default|SetHealth (- (Variables|Default|GetHealth) Damage)))
  (if (< _output_get 0.0)
    (Actor|DestroyActor)))

(event EventBeginPlay
  (AI|RunBehaviorTree (AI|GetAIController self)))

(event EventTick
  (params (DeltaSeconds :type Float%20%28single-precision%29))
  (bind _self self)
  (bind _returnvalue (Transformation|GetActorTransform _self))
  (Transformation|SetActorRotation (Math|Rotator|MakeRotator 0.0 0.0 (.yaw (Math|Rotator|FindLookatRotation (Transformation|GetActorLocation) (Transformation|GetActorLocation (Game|GetPlayerCharacter 0))))))
  (if (> (- (Utilities|Time|GetRealTimeSeconds) (Variables|Default|GetShootTimer)) (Variables|Default|GetShootCooldown))
    (Variables|Default|SetShootTimer (Utilities|Time|GetRealTimeSeconds))
    (bind _returnvalue_2 (Game|SpawnActorfromClass "/Game/Blueprints/Damaging/BP_Damager.BP_Damager_C" (Math|Transform|MakeTransform (+ (+ (* (Transformation|GetActorForwardVector _self) 1e+02) (.location _returnvalue)) "0.000000,0.000000,50.000000") (.rotation _returnvalue) (.scale _returnvalue)) "Undefined" "MultiplyWithRoot" 0 0))
    (Rendering|SetVisibility (Variables|Default|GetFlash) false false)
    (Niagara|SpawnSystemAttached "/Game/Art/VFX/NS_MuzzleFlash.NS_MuzzleFlash" (Variables|Default|GetSM_Gun_01a) "None" "0.000000,35.000000,10.000000" "0.000000,45.000000,0.000000" "KeepRelativeOffset" false)
    (Physics|AddImpulse (Variables|/Game/Blueprints/Damaging/BP_Damager.BP_Damager_C|GetCollider _returnvalue_2) (* (Transformation|GetActorForwardVector) 1e+03) "None" true)))

(fn ConstructionScript)