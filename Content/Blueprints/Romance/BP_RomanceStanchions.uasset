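; Rope stanchion barrier prop that builds a line of poles joined by hanging ropes along an editable spline.
; The construction script adds a pole mesh at each spline point, raised by a fixed height, and links neighbours with cable components whose length equals the gap.
; Event graph is empty; disconnected leftovers hold an earlier spline-mesh rope and sine-sagged light bulb placement.
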(event EventBeginPlay)

(event Collision|EventActorBeginOverlap
  (params (OtherActor :type Actor%20Object%20Reference)))

(event EventTick
  (params (DeltaSeconds :type Float%20%28single-precision%29)))

(fn ConstructionScript
  (bind _spline (Variables|Default|GetSpline))
  ;[1 0.5233 0.06354] Set up spline points and beams
  (for _index (range 0 (- (Spline|GetNumberOfSplinePoints (Variables|Default|GetSpline)) 2))
    (Variables|Default|SetSplineStartPos (+ (Spline|GetLocationatSplinePoint (Variables|Default|GetSpline) _index "Local") "0.000000,0.000000,125.000000"))
    (Variables|Default|SetSplineEndPos (+ (Spline|GetLocationatSplinePoint (Variables|Default|GetSpline) (+ _index 1) "Local") "0.000000,0.000000,125.000000"))
    (Variables|Default|SetSplineDistance (Math|Vector|Distance(Vector) (Variables|Default|GetSplineStartPos) (Variables|Default|GetSplineEndPos)))
    (Variables|Default|SetSplineUnitDirection (Math|Vector|GetUnitDirection(Vector) (Variables|Default|GetSplineStartPos) (Variables|Default|GetSplineEndPos)))
    (AddComponent|AddStaticMeshComponent false (Math|Conversions|ToTransform(Vector) (Variables|Default|GetSplineStartPos))) ; set up pole mesh
    (bind _returnvalue (AddComponent|AddCableComponent false (Math|Conversions|ToTransform(Vector) (Variables|Default|GetSplineStartPos))))
    (Variables|/Script/CableComponent.CableComponent|SetEndLocation _returnvalue (Variables|Default|GetSplineEndPos))
    (Variables|/Script/CableComponent.CableComponent|SetCableLength _returnvalue (Variables|Default|GetSplineDistance)))
  (AddComponent|AddStaticMeshComponent false (Math|Conversions|ToTransform(Vector) (+ (Spline|GetLocationatSplinePoint _spline (Spline|GetNumberOfSplinePoints _spline) "Local") "0.000000,0.000000,125.000000"))) ; set up pole mesh
)