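; Destructible train table prop built on a Chaos geometry collection, with a Box collider that ignores the player during a dash.
; On break, a radial velocity field culled by the Sphere component pushes the pieces and the Box is destroyed.
; After a delay, the debris stops simulating and loses collision.
; Tick polls BP_Betsy's Invulnerable flag to switch Box collision off and back on.
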(event OnChaosBreakEvent(GC_SM_MERGED_StaticMeshActor_101)
  (params (BreakEvent :type Chaos%20Break%20Event%20Structure%20%28by%20ref%29))
  (bind _box (Variables|Default|GetBox))
  (bind _gc_sm_merged_staticmeshactor_101 (Variables|Default|GetGC_SM_MERGED_StaticMeshActor_101))
  (bind _sphere (Variables|Default|GetSphere))
  ;[1 1 1] Chair Chaos Logic
  (Class|FieldSystemComponent|ApplyPhysicsField (Variables|Default|GetFieldSystem) true "Field_LinearVelocity" 0 (Field|SetCullingField (Variables|Default|GetCullingField) (Field|SetRadialFalloff (Variables|Default|GetRadialFalloff) 1.0 0.0 1.0 0.0 (Components|Sphere|GetScaledSphereRadius _sphere) (Transformation|GetWorldLocation _sphere) "Field_FallOff_None") (Field|SetRadialVector (Variables|Default|GetRadialVector) 1e+01 (Variables|Default|GetCenter%20Position)) "Field_Culling_Outside"))
  (Utilities|IsValid _box
    (:Is%20Valid
      (Components|DestroyComponent _box)
      (Utilities|FlowControl|Delay 15.0)
      (Physics|SetSimulatePhysics _gc_sm_merged_staticmeshactor_101 false)
      (Collision|SetCollisionEnabled _gc_sm_merged_staticmeshactor_101 "NoCollision"))))

(event EventTick
  (params (DeltaSeconds :type Float%20%28single-precision%29))
  (bind _box (Variables|Default|GetBox))
  ;[1 1 1] Disable Collision On Dash
  (bind _asbp_betsy (Utilities|Casting|CastToBP_Betsy (Game|Player|GetPlayerPawn 0)))
  (if (Variables|/Game/Blueprints/Characters/BP_Betsy.BP_Betsy_C|GetInvulnerable _asbp_betsy)
    (Utilities|IsValid _box
      (:Is%20Valid
        (Collision|SetCollisionEnabled _box "NoCollision")))
    (else
      (Utilities|IsValid _box
        (:Is%20Valid
          (Collision|SetCollisionEnabled _box "QueryAndPhysics"))))))

(event EventBeginPlay
  (Variables|Default|SetCurrentPos (Transformation|GetWorldTransform (Variables|Default|GetGC_SM_MERGED_StaticMeshActor_101))))

(fn ConstructionScript)