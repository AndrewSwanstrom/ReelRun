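; Buoyant actor that floats a boat and three pontoons on procedural Gerstner waves.
; Each tick, eight summed waves, calculated from Blueprint variables rather than the material parameter collection, offset each component from its BeginPlay location, with horizontal motion softened.
; The boat's tilt comes from the plane through the three pontoons, blended by a fixed per-tick rotator lerp.
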(event EventBeginPlay
  (Variables|Default|SetBoatOriginLocation (Transformation|GetWorldLocation (Variables|Default|GetBoat)))
  (Variables|Default|SetPontoon0OriginLocation (Transformation|GetWorldLocation (Variables|Default|GetPontoon)))
  (Variables|Default|SetPontoon1OriginLocation (Transformation|GetWorldLocation (Variables|Default|GetPontoon1)))
  (Variables|Default|SetPontoon2OriginLocation (Transformation|GetWorldLocation (Variables|Default|GetPontoon2))))

(event EventTick
  (params (DeltaSeconds :type Float%20%28single-precision%29))
  (bind _pontoon2 (Variables|Default|GetPontoon2))
  (bind _returnvalue (Transformation|GetWorldLocation _pontoon2))
  (CallFunction|FloatActoronGerstnerWave (Variables|Default|GetBoatOriginLocation) (Variables|Default|GetBoat) 6.0)
  (CallFunction|FloatActoronGerstnerWave (Variables|Default|GetPontoon0OriginLocation) (Variables|Default|GetPontoon) 2.0) ; pontoon 1 location
  (CallFunction|FloatActoronGerstnerWave (Variables|Default|GetPontoon1OriginLocation) (Variables|Default|GetPontoon1) 2.0) ; pontoon 2 location
  (CallFunction|FloatActoronGerstnerWave (Variables|Default|GetPontoon2OriginLocation) (Variables|Default|GetPontoon2) 2.0) ; pontoon 3 location
  (Variables|Default|SetTargetRot (Math|Rotator|MakeRotfromZX (Math|Vector|CrossProduct (- _returnvalue (Transformation|GetWorldLocation (Variables|Default|GetPontoon1))) (- _returnvalue (Transformation|GetWorldLocation (Variables|Default|GetPontoon)))) (Transformation|GetActorForwardVector)))
  (Variables|Default|SetCurrentRot (Math|Rotator|Lerp(Rotator) (Variables|Default|GetCurrentRot) (Variables|Default|GetTargetRot) 0.25 true))
  (Transformation|SetWorldRotation (Variables|Default|GetBoat) (Variables|Default|GetCurrentRot) false false))

(fn ConstructionScript)

(fn GerstnerWaveFunction
  (params (NumOfWaves :type Float%20%28double-precision%29) (Direction :type Linear%20Color%20Structure) (Amplitude :type Float%20%28double-precision%29) (Wavelength :type Float%20%28double-precision%29) (Speed :type Float%20%28double-precision%29) (Steepness :type Float%20%28double-precision%29) (ActorWorldLocation :type Vector))
  (bind _returnvalue (Utilities|Time|GetTimeSeconds))
  (bind _returnvalue_2 (Math|Trig|GetPI))
  (bind _returnvalue_3 (Math|Conversions|ToVector(LinearColor) Direction))
  (bind _returnvalue_4 (Math|Trig|GetPI))
  (bind (_x _y) (Math|Vector|BreakVector ActorWorldLocation))
  (bind (_x_2 _y_2) (Math|Vector|BreakVector _returnvalue_3))
  (bind _returnvalue_5 (Math|Vector|MakeVector _x _y 0.0))
  (bind _returnvalue_6 (* _returnvalue_2 2.0))
  (bind _returnvalue_7 (* _returnvalue_4 2.0))
  (bind _returnvalue_8 (Math|Vector|MakeVector _x_2 _y_2 0.0))
  (bind _returnvalue_9 (/ _returnvalue_6 Wavelength))
  (bind _returnvalue_10 (* NumOfWaves _returnvalue_7))
  (bind _returnvalue_11 (Math|Vector|Normalize _returnvalue_8))
  (bind _returnvalue_12 (* _returnvalue_9 Speed))
  (bind _returnvalue_13 (* _returnvalue_9 Amplitude))
  (bind _returnvalue_14 (Math|Vector|DotProduct _returnvalue_11 _returnvalue_5))
  (bind _returnvalue_15 (* _returnvalue_12 _returnvalue))
  (bind _returnvalue_16 (* _returnvalue_13 _returnvalue_10))
  (bind _returnvalue_17 (* _returnvalue_14 _returnvalue_9))
  (bind _returnvalue_18 (/ Steepness _returnvalue_16))
  (bind _returnvalue_19 (+ _returnvalue_17 _returnvalue_15))
  (bind _returnvalue_20 (* _returnvalue_18 Amplitude))
  (bind _returnvalue_21 (Math|Trig|Cos(Radians) _returnvalue_19))
  (bind _returnvalue_22 (* _returnvalue_20 _returnvalue_21))
  (return (Math|Vector|MakeVector (* _returnvalue_22 (.X (Math|Vector|BreakVector _returnvalue_3))) (* _returnvalue_22 (.Y (Math|Vector|BreakVector _returnvalue_3))) (* (Math|Trig|Sin(Radians) _returnvalue_19) (* Amplitude 2.0)))))

(fn CombinedGerstnerWaves
  (params (NumberOfWaves%20 :type Float%20%28double-precision%29) (PrimaryAmplitude :type Float%20%28double-precision%29) (PrimaryWavelength :type Float%20%28double-precision%29) (PrimarySpeed :type Float%20%28double-precision%29) (PrimarySteepness :type Float%20%28double-precision%29) (SecondaryAmplitude :type Float%20%28double-precision%29) (SecondaryWavelength :type Float%20%28double-precision%29) (SecondarySpeed :type Float%20%28double-precision%29) (SecondarySteepness :type Float%20%28double-precision%29) (TertiaryAmplitude :type Float%20%28double-precision%29) (TertiaryWavelength :type Float%20%28double-precision%29) (TertiarySpeed :type Float%20%28double-precision%29) (TertiarySteepness :type Float%20%28double-precision%29) (Dir1 :type Linear%20Color%20Structure) (Dir2 :type Linear%20Color%20Structure) (Dir3 :type Linear%20Color%20Structure) (Dir4 :type Linear%20Color%20Structure) (SecondaryDir1 :type Linear%20Color%20Structure) (SecondaryDir2 :type Linear%20Color%20Structure) (SecondaryDir3 :type Linear%20Color%20Structure) (SecondaryDir4 :type Linear%20Color%20Structure) (ActorWorldLocation :type Vector))
  (return (+ (+ (CallFunction|GerstnerWaveFunction NumberOfWaves%20 Dir1 PrimaryAmplitude PrimaryWavelength PrimarySpeed PrimarySteepness ActorWorldLocation) (CallFunction|GerstnerWaveFunction NumberOfWaves%20 Dir2 PrimaryAmplitude PrimaryWavelength PrimarySpeed PrimarySteepness ActorWorldLocation)) (+ (CallFunction|GerstnerWaveFunction NumberOfWaves%20 (Math|Conversions|ToLinearColor(Vector) (* (Math|Conversions|ToVector(LinearColor) Dir3) -1.0)) (* PrimaryAmplitude 0.5) (* PrimaryWavelength 0.5) (* PrimarySpeed 0.5) PrimarySteepness ActorWorldLocation) (+ (CallFunction|GerstnerWaveFunction NumberOfWaves%20 (Math|Conversions|ToLinearColor(Vector) (* (Math|Conversions|ToVector(LinearColor) Dir4) -1.0)) (* PrimaryAmplitude 0.5) (* PrimaryWavelength 0.5) (* PrimarySpeed 0.5) PrimarySteepness ActorWorldLocation) (+ (+ (CallFunction|GerstnerWaveFunction NumberOfWaves%20 SecondaryDir1 SecondaryAmplitude SecondaryWavelength SecondarySpeed SecondarySteepness ActorWorldLocation) (CallFunction|GerstnerWaveFunction NumberOfWaves%20 SecondaryDir2 SecondaryAmplitude SecondaryWavelength SecondarySpeed SecondarySteepness ActorWorldLocation)) (+ (CallFunction|GerstnerWaveFunction NumberOfWaves%20 SecondaryDir3 TertiaryAmplitude TertiaryWavelength TertiarySpeed TertiarySteepness ActorWorldLocation) (CallFunction|GerstnerWaveFunction NumberOfWaves%20 (Math|Conversions|ToLinearColor(Vector) (* (Math|Conversions|ToVector(LinearColor) SecondaryDir4) -1.0)) TertiaryAmplitude TertiaryWavelength TertiarySpeed TertiarySteepness ActorWorldLocation))))))))

(fn FloatActoronGerstnerWave
  (params (ActorOrigin :type Vector) (Component :type Static%20Mesh%20Component%20Object%20Reference) (WaveSofteningFactor :type Float%20%28double-precision%29))
  (bind _outputwavevector (CallFunction|CombinedGerstnerWaves (Variables|Default|GetNumberOfWaves) (Variables|Default|GetPrimaryAmplitude) (Variables|Default|GetPrimaryWavelength) (Variables|Default|GetPrimarySpeed) (Variables|Default|GetPrimarySteepness) (Variables|Default|GetSecondaryAmplitude) (Variables|Default|GetSecondaryWavelength) (Variables|Default|GetSecondarySpeed) (Variables|Default|GetSecondarySteepness) (Variables|Default|GetTertiaryAmplitude) (Variables|Default|GetTertiaryWavelength) (Variables|Default|GetTertiarySpeed) (Variables|Default|GetTertiarySteepness) (Variables|Default|GetLinearColorDirection1) (Variables|Default|GetLinearColorDirection2) (Variables|Default|GetLinearColorDirection3) (Variables|Default|GetLinearColorDirection4) (Variables|Default|GetLinearColorDirection5) (Variables|Default|GetLinearColorDirection6) (Variables|Default|GetLinearColorDirection7) (Variables|Default|GetLinearColorDirection8) (Transformation|GetWorldLocation Component)))
  (Transformation|SetWorldLocation Component (+ (Math|Vector|MakeVector (/ (.x _outputwavevector) WaveSofteningFactor) (/ (.y _outputwavevector) WaveSofteningFactor) (.z _outputwavevector)) ActorOrigin) false false))