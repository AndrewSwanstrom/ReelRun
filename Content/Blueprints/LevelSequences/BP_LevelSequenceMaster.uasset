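; Level manager that runs a level's enemy waves through Level Sequences, starting with an intro that starts the game timer.
; Sequencer events spawn or register enemies; destroying all of them plays the next sequence or dispatches level end.
; Sequences with a camera cut track count as cutscenes, hiding the HUD, disabling player input and allowing skip to the end.
; When cutscenes finish, enemies with stopping locations teleport near them.
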(event Custom|OnEnemyDestroyed_Event
  (params (DestroyedActor :type Actor%20Object%20Reference))
  (bind _currentwaveint (Variables|Default|GetCurrentWaveInt))
  (bind _wavesequencers (Variables|Default|GetWaveSequencers))
  (bind _enemiesinwave (Variables|Default|GetEnemiesInWave))
  (bind _output (Utilities|Array|Get(acopy) _wavesequencers _currentwaveint))
  ;[1 1 1] Count down per defeated enemy, end wave at 0 enemies and initialize the next wave
  (Utilities|Array|RemoveItem _enemiesinwave DestroyedActor)
  (if (<= (Utilities|Array|Length _enemiesinwave) 0)
    (Math|Integer|IncrementInt (Variables|Default|GetCurrentWaveInt)
      (:%20%20
        (Utilities|IsValid _output
          (:Is%20Valid
            (bind _outactor (Sequencer|Player|CreateLevelSequencePlayer _output))
            (Utilities|Array|Clear (Variables|Default|GetEnemiesInWave)) ; just to be safe
            (CallFunction|RunSequencer _outactor) ; At the end of wave, run the next wave's sequencer that handles enemy spawning and cutscenes
            (EventDispatchers|BindEventtoOnFinished (Variables|/Script/LevelSequence.LevelSequenceActor|GetSequencePlayer _outactor) (delegate Custom|SequenceFinished)))
          (:Is%20Not%20Valid
            ;[0.06902 0 1] NEXT LEVEL
            (Default|CallEndLevelDispatch) ; level bp checks for this
          ))))))

(event Custom|StartAct
  (for _array_element (Variables|Default|GetEnemiesInWave)
    (Game|AssignOnDestroyed _array_element (delegate Custom|OnEnemyDestroyed_Event))))

(event Custom|SequenceFinished
  ;[1 1 1] Start next wave
  (CallFunction|StartAct))

(event Custom|RunSequencer
  (params (CutsceneSequencePlayer :type Level%20Sequence%20Actor%20Object%20Reference))
  ;[1 1 1] Run Sequencer, dynamically determine whether or not this a cutscene or a standard sequence
  (Variables|Default|SetCutscene%20Sequence%20Player CutsceneSequencePlayer)
  (bind _returnvalue (Class|MovieSceneSequenceExtensions|FindTracksbyType (Class|LevelSequenceActor|GetSequence CutsceneSequencePlayer) "/Script/MovieSceneTracks.MovieSceneCameraCutTrack"))
  (Utilities|IsValid (Utilities|Array|Get(acopy) _returnvalue)
    (:Is%20Valid
      ;[1 1 1] For playing sequencers with a cutscene
      ;;[1 1 1] Hide Hud
      (bind _foundwidgets (Widget|GetAllWidgetsOfClass "/Game/Blueprints/UI/HUD/WBP_PlayerHUD.WBP_PlayerHUD_C" true))
      (Utilities|IsValid (Utilities|Array|Get(acopy) _foundwidgets)
        (:Is%20Valid
          (Default|HideShowHud (Utilities|Array|Get(acopy) _foundwidgets) "Collapsed"))
        (:Is%20Not%20Valid
          _))
      ;;[1 1 1] Skip Cutscene Widget
      (bind _returnvalue_2 (UserInterface|CreateWidget "/Game/Blueprints/UI/HUD/WBP_Cutscene.WBP_Cutscene_C"))
      (Variables|Default|SetCutsceneWidgetRef _returnvalue_2)
      (UserInterface|Viewport|AddtoViewport _returnvalue_2 0)
      (Input|DisableInput (Game|GetPlayerCharacter 0) (Game|GetPlayerController 0))
      (Sequencer|Player|Play (Variables|/Script/LevelSequence.LevelSequenceActor|GetSequencePlayer (Variables|Default|GetCutscene%20Sequence%20Player)) :!class /Script/MovieScene.MovieSceneSequencePlayer)
      (EventDispatchers|BindEventtoOnFinished (Variables|/Script/LevelSequence.LevelSequenceActor|GetSequencePlayer (Variables|Default|GetCutscene%20Sequence%20Player)) (delegate Custom|CutsceneFinished)))
    (:Is%20Not%20Valid
      ;[1 1 1] For playing sequencers without a cutscene
      (Sequencer|Player|Play (Variables|/Script/LevelSequence.LevelSequenceActor|GetSequencePlayer (Variables|Default|GetCutscene%20Sequence%20Player)) :!class /Script/MovieScene.MovieSceneSequencePlayer))))

(event Custom|OnIntroFinished
  ;[1 1 1] Do Intro Cutscene
  (Input|SetInputModeGameOnly (Game|GetPlayerController 0) false)
  (bind _asbp_game_instance (Utilities|Casting|CastToBP_GameInstance (Game|GetGameInstance)))
  (Default|StartTimer _asbp_game_instance)
  (CallFunction|StartAct))

(event Custom|CutsceneFinished
  ;[1 1 1] Remove widget and give player control back
  (Widget|RemovefromParent (Variables|Default|GetCutsceneWidgetRef))
  (Input|EnableInput (Game|GetPlayerCharacter 0) (Game|GetPlayerController 0))
  ;[1 1 1] Show Hud
  (bind _foundwidgets (Widget|GetAllWidgetsOfClass "/Game/Blueprints/UI/HUD/WBP_PlayerHUD.WBP_PlayerHUD_C" true))
  (Default|HideShowHud (Utilities|Array|Get(acopy) _foundwidgets) "Visible")
  ;[1 1 1] If enemies have a stopping point, TP them at end of sequence
  (for _array_element (Variables|Default|GetEnemiesInWave)
    (bind _asbase_enemy (Utilities|Casting|CastToBaseEnemy _array_element))
    (Utilities|IsValid (Variables|/Game/Blueprints/Enemies/Base_Enemy/BaseEnemy.BaseEnemy_C|GetStoppingLocation _asbase_enemy)
      (:Is%20Valid
        (Transformation|SetActorTransform _asbase_enemy (Math|Transform|MakeTransform (.RandomLocation (AI|Navigation|GetRandomReachablePointinRadius (.location (Transformation|GetActorTransform (Variables|/Game/Blueprints/Enemies/Base_Enemy/BaseEnemy.BaseEnemy_C|GetStoppingLocation _asbase_enemy))) 5e+01 0 0)) (.rotation (Transformation|GetActorTransform (Variables|/Game/Blueprints/Enemies/Base_Enemy/BaseEnemy.BaseEnemy_C|GetStoppingLocation _asbase_enemy))) (.scale (Transformation|GetActorTransform (Variables|/Game/Blueprints/Enemies/Base_Enemy/BaseEnemy.BaseEnemy_C|GetStoppingLocation _asbase_enemy)))))))))

(event Custom|Start
  ;[1 1 1] Do Intro Cutscene
  (bind _outactor (Sequencer|Player|CreateLevelSequencePlayer (Utilities|Array|Get(acopy) (Variables|Default|GetWaveSequencers))))
  (CallFunction|RunSequencer _outactor)
  (EventDispatchers|BindEventtoOnFinished (Variables|/Script/LevelSequence.LevelSequenceActor|GetSequencePlayer _outactor) (delegate Custom|OnIntroFinished))
  ;[1 1 1] Fade Out
  (bind _returnvalue (UserInterface|CreateWidget "/Game/Blueprints/UI/BPW_BlackFadeOut.BPW_BlackFadeOut_C"))
  (UserInterface|Viewport|AddtoViewport _returnvalue 0))

(event Custom|BeginSequencer
  ;[0 1 0] Begin
  (Input|EnableInput (Game|GetPlayerController 0)) ; allow this bp to read input for skipping
  (CallFunction|Start))

(event Input|EnhancedActionEvents|EnhancedInputActionIA_SkipCutscene
  (params (ActionValue :type Boolean) (ElapsedSeconds :type Float%20%28double-precision%29) (TriggeredSeconds :type Float%20%28double-precision%29) (InputAction :type Input%20Action%20Object%20Reference :default "/Game/Blueprints/Input/Actions/IA_SkipCutscene.IA_SkipCutscene"))
  (bind _cutscene_sequence_player (Variables|Default|GetCutscene%20Sequence%20Player))
  (bind _cutscene_sequence_player_2 (Variables|Default|GetCutscene%20Sequence%20Player))
  (bind _sequenceplayer (Variables|/Script/LevelSequence.LevelSequenceActor|GetSequencePlayer _cutscene_sequence_player_2))
  ;[1 0.2364 0.2185] Skip Cutscene
  (:Started
    (Utilities|IsValid _cutscene_sequence_player
      (:Is%20Valid
        (bind _returnvalue (Class|MovieSceneSequenceExtensions|FindTracksbyType (Class|LevelSequenceActor|GetSequence _cutscene_sequence_player) "/Script/MovieSceneTracks.MovieSceneCameraCutTrack"))
        (if (and (Audio|Components|Audio|IsPlaying _sequenceplayer) (Utilities|IsValid (Utilities|Array|Get(acopy) _returnvalue)))
          (Components|Timeline|SetPlaybackPosition _sequenceplayer (Utilities|Struct|MakeMovieSceneSequencePlaybackParams (Utilities|Struct|MakeFrameTime (Utilities|Struct|MakeFrameNumber (.value (.frame (Media|MediaPlayer|GetDuration _sequenceplayer)))) 0.0) 0.0 "" "(Hours=0,Minutes=0,Seconds=0,Frames=0,bDropFrameFormat=False)" "Frame" "Play")))))))

(event Custom|SpawnAll
  (params (SpawnerParent :type Actor%20Object%20Reference))
  (for _array_element (Actor|GetAttachedActors SpawnerParent true false)
    (bind _asbp_enemy_spawnpoint (Utilities|Casting|CastToBP_EnemySpawnpoint _array_element))
    (bind _spawnedactor (Default|Spawn _asbp_enemy_spawnpoint false))
    (Utilities|Array|Add (Variables|Default|GetEnemiesInWave) _spawnedactor)))

(event Custom|SpawnSingle
  (params (EnemySpawnClass :type BP%20Enemy%20Spawnpoint%20Object%20Reference))
  (bind _spawnedactor (Default|Spawn EnemySpawnClass false))
  (Utilities|Array|Add (Variables|Default|GetEnemiesInWave) _spawnedactor)
  (Utilities|IsValid (Variables|/Game/Blueprints/Enemies/Base_Enemy/BaseEnemy.BaseEnemy_C|GetStoppingLocation _spawnedactor)
    (:Is%20Valid
      (Utilities|FlowControl|Delay 0.2)
      (Utilities|IsValid (Variables|/Script/AIModule.AIController|GetBlackboard (AI|GetAIController _spawnedactor))
        (:Is%20Valid
          (AI|Components|Blackboard|SetValueasEnum (Variables|/Script/AIModule.AIController|GetBlackboard (AI|GetAIController _spawnedactor)) (Variables|Default|GetKey%20Name) (Utilities|Enum|LiteralenumLightEnemy "NewEnumerator5")))))))

(event Custom|TeleportPlayer
  (params (TeleportPoint :type Target%20Point%20Object%20Reference))
  (Transformation|SetActorTransform (Game|GetPlayerCharacter 0) (Transformation|GetActorTransform TeleportPoint) false true))

(event Custom|WalkPlayer)

(event Custom|ReturnPlayerCamera)

(event Custom|TurnPlayerCamera)

(event Custom|UpdateGlobalTimeDilation
  (Utilities|Time|SetGlobalTimeDilation (Variables|Default|GetGlobalTimeDilationTrack)))

(event Custom|InitiatePlacedEnemies
  (params (InWorldEnemy :type Base%20Enemy%20Object%20Reference))
  (Utilities|Array|Add (Variables|Default|GetEnemiesInWave) InWorldEnemy)
  (Utilities|IsValid (Variables|/Game/Blueprints/Enemies/Base_Enemy/BaseEnemy.BaseEnemy_C|GetStoppingLocation InWorldEnemy)
    (:Is%20Valid
      (AI|Components|Blackboard|SetValueasEnum (Variables|/Script/AIModule.AIController|GetBlackboard (AI|GetAIController InWorldEnemy)) (Variables|Default|GetKey%20Name) (Utilities|Enum|LiteralenumLightEnemy "NewEnumerator5")))))

(event Custom|WarpEnemyToPosition
  (params (EnemyToWarp :type Base%20Enemy%20Object%20Reference)))

(fn ConstructionScript)