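; Animation notify state that locks Betsy's movement for the span of an animation window.
; On begin it casts the mesh owner to BP_Betsy and sets CanMove to false.
; On end it sets CanMove back to true, so the notify's placement on the animation timeline defines how long movement is disabled.
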(fn ReceivedNotifyBegin
  (params (MeshComp :type Skeletal%20Mesh%20Component%20Object%20Reference) (Animation :type Anim%20Sequence%20Base%20Object%20Reference) (TotalDuration :type Float%20%28single-precision%29) (EventReference :type Anim%20Notify%20Event%20Reference%20Structure%20%28by%20ref%29))
  (bind _asbp_betsy (Utilities|Casting|CastToBP_Betsy (Components|GetOwner MeshComp)))
  (Utilities|IsValid _asbp_betsy
    (:Is%20Valid
      (Variables|/Game/Blueprints/Characters/BP_Betsy.BP_Betsy_C|SetCanMove _asbp_betsy false)
      (return false))))

(fn ReceivedNotifyEnd
  (params (MeshComp :type Skeletal%20Mesh%20Component%20Object%20Reference) (Animation :type Anim%20Sequence%20Base%20Object%20Reference) (EventReference :type Anim%20Notify%20Event%20Reference%20Structure%20%28by%20ref%29))
  (bind _asbp_betsy (Utilities|Casting|CastToBP_Betsy (Components|GetOwner MeshComp)))
  (Utilities|IsValid _asbp_betsy
    (:Is%20Valid
      (Variables|/Game/Blueprints/Characters/BP_Betsy.BP_Betsy_C|SetCanMove _asbp_betsy true)
      (return false))))