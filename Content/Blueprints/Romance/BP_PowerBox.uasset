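; BP_PowerBox is a punchable power box that temporarily powers a blue or orange spotlight.
; Any damage while Vulnerable plays a pitch-varied punch sound, swaps the mesh, sets HasPower and lights its point light.
; ControlBlue chooses the spotlight class, and GetActorOfClass finds a single instance to light.
; After a fixed delay it switches both lights off, spawns a Niagara effect, restores the mesh and becomes hittable again.
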(event EventBeginPlay)

(event Game|Damage|EventAnyDamage
  (params (Damage :type Float%20%28single-precision%29) (DamageType :type Damage%20Type%20Object%20Reference) (InstigatedBy :type Controller%20Object%20Reference) (DamageCauser :type Actor%20Object%20Reference))
  (bind _collider (Variables|Default|Getcollider))
  (bind _collider_2 (Variables|Default|Getcollider))
  (bind _returnvalue (Transformation|GetWorldTransform _collider))
  (bind _returnvalue_2 (Transformation|GetWorldTransform _collider_2))
  (if (Variables|Default|GetVulnerable)
    (Audio|SpawnSoundatLocation "/Game/JohnVizaria/Sounds/CombatSounds/PunchSounds/punch_2.punch_2" (.location _returnvalue) (.rotation _returnvalue) 1.0 (Math|Random|RandomFloatinRange 0.8 1.2) 0.0 "/Game/Art/SFX/Attenuations/SA_Footstep.SA_Footstep" 0)
    (Variables|Default|SetVulnerable false)
    (Components|StaticMesh|SetStaticMesh (Variables|Default|GetPowerBox) "/Game/Art/Environment/Romance/Act1/SM_PowerBox_02.SM_PowerBox_02")
    (if (Variables|Default|GetbControlBlue?)
      (Rendering|SetVisibility (Variables|Default|GetPointLight) true true)
      (Development|PrintString "PowerBox Punched On" true true "(R=0.239583,G=0.211235,B=0.185927,A=1.000000)")
      (Variables|Default|SetbHasPower true)
      (bind _returnvalue_3 (Actor|GetActorOfClass "/Game/Blueprints/Romance/PoweredSpotlightBlue.PoweredSpotlightBlue_C"))
      (Rendering|SetVisibility (Variables|/Game/Blueprints/Romance/PoweredSpotlightBlue.PoweredSpotlightBlue_C|GetSpotLight _returnvalue_3) true false)
      (Utilities|FlowControl|Delay 5.0)
      (Rendering|SetVisibility (Variables|Default|GetPointLight) false true)
      (Development|PrintString "PowerBox Off" true true "(R=0.526042,G=0.463799,B=0.408232,A=1.000000)")
      (Variables|Default|SetbHasPower false)
      (Rendering|SetVisibility (Variables|/Game/Blueprints/Romance/PoweredSpotlightBlue.PoweredSpotlightBlue_C|GetSpotLight _returnvalue_3) false false)
      (else
        (Rendering|SetVisibility (Variables|Default|GetPointLight) true true)
        (Development|PrintString "PowerBox Punched On" true true "(R=0.239583,G=0.211235,B=0.185927,A=1.000000)")
        (Variables|Default|SetbHasPower true)
        (bind _returnvalue_4 (Actor|GetActorOfClass "/Game/Blueprints/Romance/BP_PoweredSpotlightOrange.BP_PoweredSpotlightOrange_C"))
        (Rendering|SetVisibility (Variables|/Game/Blueprints/Romance/BP_PoweredSpotlightOrange.BP_PoweredSpotlightOrange_C|GetSpotLight _returnvalue_4) true false)
        (Utilities|FlowControl|Delay 5.0)
        (Rendering|SetVisibility (Variables|Default|GetPointLight) false true)
        (Development|PrintString "PowerBox Off" true true "(R=0.526042,G=0.463799,B=0.408232,A=1.000000)")
        (Variables|Default|SetbHasPower false)
        (Rendering|SetVisibility (Variables|/Game/Blueprints/Romance/BP_PoweredSpotlightOrange.BP_PoweredSpotlightOrange_C|GetSpotLight _returnvalue_4) false false)))
    (Variables|Default|SetVulnerable true)
    (Niagara|SpawnSystematLocation "/Game/Art/VFX/NS_Dash.NS_Dash" (.location _returnvalue_2) (.rotation _returnvalue_2) "2.000000,2.000000,2.000000")
    (Components|StaticMesh|SetStaticMesh (Variables|Default|GetPowerBox) "/Game/Art/Environment/Romance/Act1/SM_PowerBox_01.SM_PowerBox_01")))

(fn ConstructionScript)