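; Campfire plume actor for the horror game that shows a Niagara plume while enemies from its campsite remain.
; StartPlume activates the effect after a short delay, then runs one multi-sphere trace around itself to collect hit actors and bind their OnDestroyed events.
; Each destruction removes that actor from the list, and the plume deactivates when the list empties.
; Debug prints remain, and the actor's self-destroy is unconnected.
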(event Custom|OnDestroyed_Event
  (params (DestroyedActor :type Actor%20Object%20Reference))
  (bind _enemiesfromcampfire (Variables|Default|GetEnemiesFromCampfire))
  (bind _returnvalue (Utilities|Array|Length _enemiesfromcampfire))
  (Utilities|Array|RemoveItem _enemiesfromcampfire DestroyedActor)
  (Development|PrintString (Utilities|String|ToString(Integer) _returnvalue))
  (if (<= _returnvalue 0)
    (Components|Activation|Deactivate (Variables|NiagaraActor|GetNiagaraComponent))))

(event Custom|StartPlume
  (bind _self self)
  (bind _returnvalue (Transformation|GetActorLocation _self))
  (Utilities|FlowControl|Delay 0.5)
  (Components|Activation|Activate (Variables|NiagaraActor|GetNiagaraComponent) false)
  (bind _outhits (Collision|MultiSphereTraceByChannel _returnvalue _returnvalue 1e+03 "TraceTypeQuery3" false 0 "None")) ; Single trace to capture all enemies from this campsite and put onto array and bind destroyed event to them
  (for _array_element _outhits
    (Development|PrintString (Utilities|GetDisplayName (.HitActor (Collision|BreakHitResult _array_element))))
    (Utilities|Array|Add (Variables|Default|GetEnemiesFromCampfire) (.HitActor (Collision|BreakHitResult _array_element)))
    (Game|AssignOnDestroyed (.HitActor (Collision|BreakHitResult _array_element)) (delegate Custom|OnDestroyed_Event))))

(event EventTick
  (params (DeltaSeconds :type Float%20%28single-precision%29)))

(fn ConstructionScript)