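; Destructible barstool prop built on a Chaos fractured mesh with a separate Box collider.
; When the mesh breaks, it fires a transient radial field at the destruction center, destroys the Box and switches the pieces to a custom collision channel.
; Until that break, Tick polls the BP_Betsy player and disables Box collision while the player is invulnerable.
; CanTick works inversely to its name, stopping the polling once true.
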(event OnChaosBreakEvent(fracturedBarstool)
  (params (BreakEvent :type Chaos%20Break%20Event%20Structure%20%28by%20ref%29))
  (bind _box (Variables|Default|GetBox))
  ;[1 1 1] velocity field
  (CallFunction|TransientField (Variables|Default|GetFieldSystem) (Variables|Default|GetCullingField) (Variables|Default|GetRadialFalloff) (Variables|Default|GetRadialVector) (Variables|Default|GetDestructionCenter) (Variables|Default|GetSphere))
  (Utilities|IsValid _box
    (:Is%20Valid
      (Components|DestroyComponent _box)
      (Variables|Default|SetCanTick true)
      (Collision|SetCollisionObjectType (Variables|Default|GetfracturedBarstool) "ECC_GameTraceChannel2"))))

(event EventTick
  (params (DeltaSeconds :type Float%20%28single-precision%29))
  (bind _box (Variables|Default|GetBox))
  (if (not (Variables|Default|GetCanTick))
    (bind _asbp_betsy (Utilities|Casting|CastToBP_Betsy (Game|Player|GetPlayerPawn 0)))
    (if (Variables|/Game/Blueprints/Characters/BP_Betsy.BP_Betsy_C|GetInvulnerable _asbp_betsy)
      (Utilities|IsValid (Variables|Default|GetBox)
        (:Is%20Valid
          (Collision|SetCollisionEnabled _box "NoCollision")))
      (else
        (Utilities|IsValid (Variables|Default|GetBox)
          (:Is%20Valid
            (Collision|SetCollisionEnabled _box "QueryAndPhysics")))))))

(fn ConstructionScript)