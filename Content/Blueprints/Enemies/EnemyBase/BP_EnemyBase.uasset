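; Base melee enemy character that takes damage, destroys itself at zero health, and punches targets with a montage-driven attack.
; While a left or right fist flag is set, Tick sphere-traces between that hand's sockets, damaging each actor once until the ignore list is cleared.
; The attack broadcasts its end when the montage completes or is interrupted.
; Helper functions supply ideal attack and defense ranges and map movement states to walk speeds.
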(event Custom|AttackAnim
  (Animation|Montage|PlayMontage (Variables|Character|GetMesh) "/Game/Art/Characters/Enemies/Light/Animations/Montage/Anim_LightEnemy_Attack_Montage.Anim_LightEnemy_Attack_Montage"
    (:OnCompleted
      _)
    (:OnInterrupted
      _))
  (Default|CallOnAttackEnd))

(event Custom|ClearAttackStack
  ;[1 1 1] Clear Stacks From Line Trace
  (Utilities|Array|Clear (Variables|Default|GetActors%20to%20Ignore)))

(event Game|Damage|EventAnyDamage
  (params (Damage :type Float%20%28single-precision%29) (DamageType :type Damage%20Type%20Object%20Reference) (InstigatedBy :type Controller%20Object%20Reference) (DamageCauser :type Actor%20Object%20Reference))
  ;[1 1 1] Damage Enemy
  (bind _output_get (Variables|Default|SetHealth (- (Variables|Default|GetHealth) Damage)))
  (if (<= _output_get 0.0)
    (Actor|DestroyActor)))

(event EventTick
  (params (DeltaSeconds :type Float%20%28single-precision%29))
  (bind _mesh (Variables|Character|GetMesh))
  ;[1 1 1] Event Tick Line Trace Damage Logic
  (Variables|Default|SetDelta%20Seconds DeltaSeconds)
  (if (Variables|Default|GetLeftFistAttack)
    (Variables|Default|SetSocketStart "LeftHandStart")
    (Variables|Default|SetSocketEnd "LeftHandEnd")
    (bind _outhits (Collision|MultiSphereTraceForObjects (Transformation|GetSocketLocation _mesh (Variables|Default|GetSocketStart)) (Transformation|GetSocketLocation _mesh (Variables|Default|GetSocketEnd)) 2e+01 (Utilities|Array|MakeArray "ObjectTypeQuery7") false 0 "None" :!label _label))
    (for _array_element _outhits
      (if (not (Utilities|Array|ContainsItem (Variables|Default|GetActors%20to%20Ignore) (.HitActor (Collision|BreakHitResult _array_element))))
        (Game|Damage|ApplyDamage (.HitActor (Collision|BreakHitResult _array_element)) 5.0 0 0)
        (Utilities|Array|Add (Variables|Default|GetActors%20to%20Ignore) (.HitActor (Collision|BreakHitResult _array_element)))))
    (elif (Variables|Default|GetRightFistAttack)
      (Variables|Default|SetSocketStart "RightHandStart")
      (Variables|Default|SetSocketEnd "RightHandEnd")
      (goto _label))))

(event EventBeginPlay
  ;[1 1 1] Random Wander
)

(fn ConstructionScript)

(fn GetIdealRange
  (return 1e+02 3.5e+02))

(fn SetMovementSpeed
  (params (Speed :type E_MovementSpeed%20Enum :default "NewEnumerator0"))
  (bind _output_get (Variables|/Script/Engine.CharacterMovementComponent|SetMaxWalkSpeed (Variables|Character|GetCharacterMovement) (Utilities|Select :Index Speed :NewEnumerator0 0.0 :NewEnumerator1 1e+02 :NewEnumerator2 5e+02)))
  (return _output_get))