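; BP_ClickIt is a clickable actor that slides back and forth along the world Y axis on alternate clicks.
; BeginPlay enables click and mouse-over events on the first player controller.
; Each click drives a FlipFlop that restarts one of two timelines, one for positive Y, one for negative.
; Each update lerps from the current location toward a small offset, so movement accumulates per tick rather than interpolating between fixed endpoints.
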(event EventBeginPlay
  (bind _returnvalue (Game|GetPlayerController 0))
  (Variables|/Script/Engine.PlayerController|SetbEnableClickEvents _returnvalue true)
  (Variables|/Script/Engine.PlayerController|SetbEnableMouseOverEvents _returnvalue true))

(event MouseInput|EventActorOnClicked
  (params (ButtonPressed :type Key%20Structure :default "None"))
  (bind _returnvalue (Transformation|GetActorLocation))
  (bind _returnvalue_2 (Transformation|GetActorLocation))
  (bind _returnvalue_3 (Transformation|GetActorLocation))
  (bind _returnvalue_4 (Transformation|GetActorLocation))
  (bind (_x _y _z) (Math|Vector|BreakVector _returnvalue))
  (bind _y_2 (Math|Vector|BreakVector _returnvalue_2))
  (bind _y_3 (Math|Vector|BreakVector _returnvalue_3))
  (bind (_x_2 _y_4 _z_2) (Math|Vector|BreakVector _returnvalue_4))
  (Utilities|FlowControl|FlipFlop
    (:A
      (bind _move_actor_timeline (Timeline|Move%20Actor PlayFromStart)
        (:Update
          (Transformation|SetActorLocation (Math|Vector|MakeVector _x_2 (Math|Float|Lerp _y_3 (+ _y_3 2.0) _move_actor_timeline) _z_2) false false))))
    (:B
      (bind _move_actor_timeline_2 (Timeline|Timeline PlayFromStart)
        (:Update
          (Transformation|SetActorLocation (Math|Vector|MakeVector _x (Math|Float|Lerp _y_2 (+ _y_2 -2.0) _move_actor_timeline_2) _z) false false))))))

(fn ConstructionScript)