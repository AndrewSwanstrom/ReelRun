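; BP_LevelProgressionEnemy is a damageable enemy whose death moves the game on to another level.
; AnyDamage plays a pitch-randomized hit sound and damage montage, optionally spawns a damage number actor, and adds a Niagara effect when the causer's display name matches BP_Syd0.
; It then subtracts health; at zero it disables further damage, shows a black fade widget and opens the next level after a short delay.
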(event Game|Damage|EventAnyDamage
  (params (Damage :type Float%20%28single-precision%29) (DamageType :type Damage%20Type%20Object%20Reference) (InstigatedBy :type Controller%20Object%20Reference) (DamageCauser :type Actor%20Object%20Reference))
  (bind _self self)
  ;[1 1 1] Receive Damage
  (if (Variables|Default|GetBCanBeMDmgd)
    (Audio|PlaySoundatLocation "/Game/Art/SFX/RandomHitCue.RandomHitCue" (Transformation|GetActorLocation) "0, 0, 0" 1.0 (Math|Random|RandomFloatinRange 0.5 1.3) 0.0 0 0 0 0)
    ;;[1 1 1] show dmg numbers?
    (if (Variables|Default|GetShowDmgNums?)
      (Game|SpawnActorfromClass "/Game/Art/VFX/Blood_And_Nums/DamageNumbers/BP_DmgNum.BP_DmgNum_C" (Transformation|GetActorTransform _self) "Undefined" "MultiplyWithRoot" _self Damage "(R=0.000000,G=0.000000,B=0.000000,A=0.000000)" 0))
    ;;[1 1 1] is dmg causer syd
    (if (== (Utilities|String|StringToName (Utilities|GetDisplayName DamageCauser)) "BP_Syd0")
      (AddComponent|AddNiagaraComponent false))
    (Animation|Montage|PlayMontage (Variables|Character|GetMesh) "/Game/Art/Characters/Enemies/Light/Animations/Montage/Anim_LightEnemyDamage_Montage.Anim_LightEnemyDamage_Montage"
      (:then
        (Utilities|FlowControl|Sequence
          (:then_1
            (bind _output_get (Variables|Default|SetHealth (- (Variables|Default|GetHealth) Damage)))
            (if (<= _output_get 0.0)
              (Variables|Default|SetBCanBeMDmgd false)
              (bind _returnvalue (UserInterface|CreateWidget "/Game/Blueprints/UI/BPW_BlackFadeIn.BPW_BlackFadeIn_C"))
              (UserInterface|Viewport|AddtoPlayerScreen _returnvalue)
              (Utilities|FlowControl|Delay 1.0)
              (Widget|RemovefromParent _returnvalue)
              (Game|OpenLevel(byObjectReference) (Variables|Default|GetLevel2Open))))))
      (:OnCompleted
        (Development|PrintString "Light: OW!")))))

(event Collision|EventActorBeginOverlap
  (params (OtherActor :type Actor%20Object%20Reference))
  (|CallParentFunction OtherActor) ; This node is disabled and will not be called.\nDrag off pins to build functionality.
)

(event EventTick
  (params (DeltaSeconds :type Float%20%28single-precision%29))
  (|CallParentFunction DeltaSeconds) ; This node is disabled and will not be called.\nDrag off pins to build functionality.
)

(event EventBeginPlay
  (|CallParentFunction) ; This node is disabled and will not be called.\nDrag off pins to build functionality.
)

(fn ConstructionScript
  (|CallParentFunction))