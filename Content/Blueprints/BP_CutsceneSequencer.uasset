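; Cutscene controller actor that plays a given level sequence and lets the player skip it.
; PlayCutscene adds the WBP_Cutscene widget, disables input on the player character and starts the sequence.
; The actor enables its own input, so IA_Jump during playback moves the sequence to its duration frame to skip it.
; The sequence's OnFinished event removes the widget and restores character input.
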(event Custom|CutsceneFinished
  ;[1 1 1] Play Cutscene
  ;;[1 1 1] Remove widget and give player control back
  (Widget|RemovefromParent (Variables|Default|GetCutsceneWidgetRef))
  (Input|EnableInput (Game|GetPlayerCharacter 0) (Game|GetPlayerController 0)))

(event Custom|PlayCutscene
  (params (CutsceneSequencePlayer :type Level%20Sequence%20Actor%20Object%20Reference))
  (bind _sequenceplayer (Variables|/Script/LevelSequence.LevelSequenceActor|GetSequencePlayer CutsceneSequencePlayer))
  ;[1 1 1] Play Cutscene
  ;;[1 1 1] Skip Cutscene Widget
  (bind _returnvalue (UserInterface|CreateWidget "/Game/Blueprints/UI/HUD/WBP_Cutscene.WBP_Cutscene_C"))
  (Variables|Default|SetCutsceneWidgetRef _returnvalue)
  (UserInterface|Viewport|AddtoViewport _returnvalue 0)
  (Input|DisableInput (Game|GetPlayerCharacter 0) (Game|GetPlayerController 0))
  (Sequencer|Player|Play _sequenceplayer :!class /Script/MovieScene.MovieSceneSequencePlayer)
  (EventDispatchers|BindEventtoOnFinished _sequenceplayer (delegate Custom|CutsceneFinished)))

(event Input|EnhancedActionEvents|EnhancedInputActionIA_Jump
  (params (ActionValue :type Boolean) (ElapsedSeconds :type Float%20%28double-precision%29) (TriggeredSeconds :type Float%20%28double-precision%29) (InputAction :type Input%20Action%20Object%20Reference :default "/Game/Blueprints/Input/Actions/IA_Jump.IA_Jump"))
  ;[1 1 1] Play Cutscene
  ;;[1 0.2364 0.2185] Skip Cutscene
  (:Started
    (Utilities|IsValid (stale Custom|PlayCutscene CutsceneSequencePlayer)
      (:Is%20Valid
        (if (Audio|Components|Audio|IsPlaying (Variables|/Script/LevelSequence.LevelSequenceActor|GetSequencePlayer (stale Custom|PlayCutscene CutsceneSequencePlayer)))
          (Components|Timeline|SetPlaybackPosition (Variables|/Script/LevelSequence.LevelSequenceActor|GetSequencePlayer (stale Custom|PlayCutscene CutsceneSequencePlayer)) (Utilities|Struct|MakeMovieSceneSequencePlaybackParams (Utilities|Struct|MakeFrameTime (Utilities|Struct|MakeFrameNumber (.value (.frame (Media|MediaPlayer|GetDuration (Variables|/Script/LevelSequence.LevelSequenceActor|GetSequencePlayer (stale Custom|PlayCutscene CutsceneSequencePlayer)))))) 0.0) 0.0 "" "(Hours=0,Minutes=0,Seconds=0,Frames=0,bDropFrameFormat=False)" "Frame" "Play")))))))

(event EventBeginPlay
  ;[1 1 1] allow this to read input
  (Input|EnableInput (Game|GetPlayerController 0)))

(fn ConstructionScript)