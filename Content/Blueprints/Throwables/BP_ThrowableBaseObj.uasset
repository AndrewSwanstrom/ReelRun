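; Base actor for throwable bottles that the player can highlight in range and throw to damage enemies or break destructibles.
; A timeline moves the spinning mesh along an arc, sphere-tracing between its Top and Bottom sockets each update.
; Hits branch by object type: pawns and bosses take damage and AI blackboard changes, geometry collections receive strain, and impacts spawn break effects.
; Overlap events toggle the outline and interact prompts.
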(event Custom|ThrowableDamage
  (params (ChildMesh :type Static%20Mesh%20Component%20Object%20Reference))
  ;[1 1 1] Trace when Thrown
  (if (Variables|Default|GetBottleThrown)
    (bind _outhits (Collision|MultiSphereTraceForObjects (Transformation|GetSocketLocation ChildMesh "Top") (Transformation|GetSocketLocation ChildMesh "Bottom") 5.0 (Utilities|Array|MakeArray "ObjectTypeQuery3" "ObjectTypeQuery6" "ObjectTypeQuery1" "ObjectTypeQuery2" "ObjectTypeQuery12") false (Utilities|Array|MakeArray (Game|Player|GetPlayerPawn 0)) "None"))
    (for _array_element _outhits
      (Utilities|IsValid (.hitactor _array_element)
        (:Is%20Valid
          (switch Utilities|FlowControl|Switch|SwitchonECollisionChannel (Collision|GetCollisionObjectType (.hitcomponent _array_element))
            (:ECC_WorldStatic
              _)
            (:ECC_WorldDynamic
              _)
            (:ECC_Pawn
              (Game|Damage|ApplyDamage (.hitactor _array_element) 5.0 0 0 :!label _label)
              (Utilities|IsValid (AI|GetAIController (.hitactor _array_element))
                (:Is%20Valid
                  (AI|Components|Blackboard|SetValueasEnum (Variables|/Script/AIModule.AIController|GetBlackboard (AI|GetAIController (.hitactor _array_element))) (Variables|Default|GetKey) (Utilities|Enum|LiteralenumLightEnemy "NewEnumerator7")))))
            (:ECC_Destructible
              (bind _asbase_character (Utilities|Casting|CastToBase_Character (Game|GetPlayerCharacter 0)))
              (Variables|/Game/Blueprints/Characters/Base_Character.Base_Character_C|SetCenterSpotTest _asbase_character (.impactpoint _array_element))
              (bind _asgeometry_collection_component (Utilities|Casting|CastToGeometryCollectionComponent (.hitcomponent _array_element)))
              (Class|GeometryCollectionComponent|ApplyInternalStrain _asgeometry_collection_component (.hititem _array_element) (.impactpoint _array_element) 1e+02 0 1.0 1e+06))
            (:ECC_GameTraceChannel8
              (goto _label))))
        (:Is%20Not%20Valid
          _))
      (Audio|PlaySound2D "/Game/Art/SFX/InGame/R_Bottlebreak.R_Bottlebreak" 1.0 1.0 0.0 0 0)
      (Niagara|SpawnSystematLocation "/Game/Art/VFX/NS_BottleDebris.NS_BottleDebris" (.impactpoint _array_element))
      (Actor|DestroyActor))))

(event Custom|End%20Collider%20Overlap
  (params (Actor%20Overlapping :type Actor%20Object%20Reference) (Interact%20Icon :type Widget%20Component%20Object%20Reference) (Item%20Mesh :type Mesh%20Component%20Object%20Reference))
  ;[1 1 1] begin / end collider overlap
  (Variables|Default|SetInRange false)
  (bind _asbase_character (Utilities|Casting|CastToBase_Character Actor%20Overlapping))
  (Rendering|SetVisibility Interact%20Icon false false)
  (Rendering|Material|SetOverlayMaterial Item%20Mesh 0 :!class /Script/Engine.MeshComponent)
  (Widget|SetVisibility (Variables|/Game/Blueprints/UI/HUD/WBP_PlayerHUD.WBP_PlayerHUD_C|Getinteract_hand (Variables|/Game/Blueprints/Characters/Base_Character.Base_Character_C|GetHudRef _asbase_character)) "Hidden"))

(event Custom|Begin%20Collider%20Overlap
  (params (Actor%20Overlapping :type Actor%20Object%20Reference) (Interact%20Icon :type Widget%20Component%20Object%20Reference) (Item%20Mesh :type Mesh%20Component%20Object%20Reference))
  ;[1 1 1] begin / end collider overlap
  (Variables|Default|SetInRange true)
  (bind _asbase_character (Utilities|Casting|CastToBase_Character Actor%20Overlapping))
  (if (not (Variables|/Game/Blueprints/Characters/Base_Character.Base_Character_C|GetbHasItem _asbase_character))
    (Rendering|SetVisibility Interact%20Icon true false)
    (Rendering|Material|SetOverlayMaterial Item%20Mesh "/Game/Materials/OutlineMat/Mi_OutlineMat_Inst.Mi_OutlineMat_Inst" :!class /Script/Engine.MeshComponent)
    (Widget|SetVisibility (Variables|/Game/Blueprints/UI/HUD/WBP_PlayerHUD.WBP_PlayerHUD_C|Getinteract_hand (Variables|/Game/Blueprints/Characters/Base_Character.Base_Character_C|GetHudRef _asbase_character)) "Visible")))

(event Custom|DoBottleThrowArc
  (bind _itemmesh (Variables|Default|GetItemMesh))
  ;[1 1 1] Runs throwing arc
  (Variables|Default|SetBottleThrown true)
  (Rendering|SetVisibility (Variables|Default|GetNiagara) true false)
  (Physics|SetSimulatePhysics _itemmesh true)
  (Class|PrimitiveComponent|SetPhysicsAngularVelocityinRadians _itemmesh (* (Math|Random|RandomUnitVector) 1e+01) false "None") ; random angular velocity
  (Variables|Default|SetDoHitCheck true)
  (bind (_direction _arcapex _alpha) (Timeline|Timeline PlayFromStart)
    (:Update
      (CallFunction|ThrowableDamage (Variables|Default|GetItemMesh)) ; only trace during timeline
      (Utilities|IsValid self
        (:Is%20Valid
          (Transformation|SetWorldLocation (Variables|Default|GetItemMesh) (+ (Variables|Default|GetThrowArcLerpStart) (* (Variables|Default|GetBotleArcInitAngle) _alpha (Variables|Default|GetMaxThrowDisance)) (Math|Vector|MakeVector 0.0 0.0 _arcapex)) false false))))
    (:Finished
      (Variables|Default|SetBottleThrown false)
      (Actor|DestroyActor))))

(fn ConstructionScript)