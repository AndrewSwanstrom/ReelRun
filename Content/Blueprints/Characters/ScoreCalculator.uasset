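; ScoreCalculator computes a player performance score from combo, death, finisher and timer values.
; ComboCalc, DeathCalc and FinisherCalc each divide an actual value by an intended one, and FinalCalc returns the weighted sum with Timer, favouring combo most.
; Tick overwrites Timer with the frame delta rather than accumulating it, and TimerCalc is an empty stub noted for per-level target times.
; AddCombo only assigns ActualCombo without incrementing it.
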(event EventBeginPlay)

(event EventTick
  (params (DeltaSeconds :type Float%20%28single-precision%29))
  (Variables|Default|SetTimer DeltaSeconds))

(fn ComboCalc
  (Variables|Default|SetFinalCombo (/ (Variables|Default|GetActualCombo) (Variables|Default|GetIntendedCombo))))

(fn DeathCalc
  (Variables|Default|SetFinalDeath (/ (Variables|Default|GetActualDeath) (Variables|Default|GetIntendedDeath))))

(fn FinisherCalc
  (Variables|Default|SetFinalFinisher (/ (Variables|Default|GetActualFinisher) (Variables|Default|GetIntendedFinisher))))

(fn TimerCalc
  ;[1 1 1] me note: possible bool saying what level that sets needed time based on that
)

(fn FinalCalc
  (Variables|Default|SetFinalCombo (* (Variables|Default|GetFinalCombo) 0.4))
  (Variables|Default|SetFinalDeath (* (Variables|Default|GetFinalDeath) 0.3))
  (Variables|Default|SetFinalFinisher (* (Variables|Default|GetFinalFinisher) 0.2))
  (Variables|Default|SetTimer (* (Variables|Default|GetTimer) 0.1))
  (bind _output_get (Variables|Default|SetFinalScore (+ (Variables|Default|GetFinalCombo) (Variables|Default|GetFinalDeath) (Variables|Default|GetFinalFinisher) (Variables|Default|GetTimer))))
  (return _output_get))

(fn AddCombo
  (params (ActualCombo :type Float%20%28double-precision%29))
  (Variables|Default|SetActualCombo ActualCombo))