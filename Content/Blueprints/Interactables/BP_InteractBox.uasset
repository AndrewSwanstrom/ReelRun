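; BP_InteractBox is an interactable trigger volume that shows an icon and responds to the interact input while the player is inside.
; Box overlaps set IsIn and, when Enabled, toggle the icon and call IsInside for special behavior; end overlap clears these for any actor, not only the player.
; IA_Interact calls InteractAction when inside and enabled.
; Helpers unhide the actor (WakeUP) and return LoadNext (ReturnLoad).
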(event OnComponentBeginOverlap(Box)
  (params (OverlappedComponent :type Primitive%20Component%20Object%20Reference) (OtherActor :type Actor%20Object%20Reference) (OtherComp :type Primitive%20Component%20Object%20Reference) (OtherBodyIndex :type Integer) (bFromSweep :type Boolean) (SweepResult :type Hit%20Result%20Structure%20%28by%20ref%29))
  (if (== (Game|GetPlayerCharacter 0) OtherActor)
    (Variables|Default|SetisIn true)
    (if (Variables|Default|GetEnabled)
      (Rendering|SetVisibility (Variables|Default|GetInteract%20Icon) true false)
      ;[1 1 1] For interactables that have special behavior when inside
      (CallFunction|IsInside true))))

(event OnComponentEndOverlap(Box)
  (params (OverlappedComponent :type Primitive%20Component%20Object%20Reference) (OtherActor :type Actor%20Object%20Reference) (OtherComp :type Primitive%20Component%20Object%20Reference) (OtherBodyIndex :type Integer))
  (if (== OtherActor (Game|GetPlayerCharacter 0))
    _
    (else
      _))
  (Variables|Default|SetisIn false)
  (if (Variables|Default|GetEnabled)
    (Rendering|SetVisibility (Variables|Default|GetInteract%20Icon) false false)
    ;[1 1 1] For interactables that have special behavior when inside
    (CallFunction|IsInside false)))

(event Input|EnhancedActionEvents|EnhancedInputActionIA_Interact
  (params (ActionValue :type Boolean) (ElapsedSeconds :type Float%20%28double-precision%29) (TriggeredSeconds :type Float%20%28double-precision%29) (InputAction :type Input%20Action%20Object%20Reference :default "/Game/Blueprints/Input/Actions/IA_Interact.IA_Interact"))
  (:Started
    (if (and (Variables|Default|GetisIn) (Variables|Default|GetEnabled))
      (CallFunction|InteractAction))))

(event EventBeginPlay
  (Input|EnableInput (Game|GetPlayerController 0)))

(fn ConstructionScript)

(fn WakeUP
  (Rendering|SetActorHiddenInGame false))

(fn ReturnLoad
  (return (Variables|Default|GetloadNext)))