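; BP_DiscoDamager-CircleAttack is a short-lived actor in the Damaging set, named as the circle attack variant of the disco damager.
; On BeginPlay it stores its start location and plays a timeline that lerps its height down 250 units.
; It destroys itself when the timeline finishes.
; The construction script only calls the parent, and the file itself contains no damage logic.
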(event EventBeginPlay
  (bind _returnvalue (Transformation|GetActorLocation))
  (Variables|Default|SetInitialPosition (Transformation|GetActorLocation))
  (bind _alpha (Timeline|Timeline_0 PlayFromStart)
    (:Update
      (Transformation|SetActorLocation (Math|Vector|MakeVector (.x _returnvalue) (.y _returnvalue) (Math|Float|Lerp (.z (Variables|Default|GetInitialPosition)) (- (.z (Variables|Default|GetInitialPosition)) 2.5e+02) _alpha)) false false))
    (:Finished
      (Actor|DestroyActor))))

(fn ConstructionScript
  (|CallParentFunction))