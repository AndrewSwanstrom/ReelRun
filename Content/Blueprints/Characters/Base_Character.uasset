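; Base player character Blueprint providing shared events for movement, camera pitch, pausing, melee combos and throwables, using Enhanced Input.
; Light and heavy attacks share a counter and buffered inputs to chain montages, set knockback and run timeline-driven thrusts.
; A capsule trace along input or facing direction soft-locks thrusts and throws onto targets.
; Also includes nearby throwable pickup, a debug area kill and unfinished save/load.
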(event EventBeginPlay
  (bind _asbp_main_hud (Utilities|Casting|CastToBP_MainHUD (HUD|GetHUD (Game|GetPlayerController 0))))
  (Variables|Default|SetPauseMenu (Variables|/Game/Blueprints/UI/BP_MainHUD.BP_MainHUD_C|GetPauseScreenRef _asbp_main_hud))
  (Variables|Default|SetHudRef (Variables|/Game/Blueprints/UI/BP_MainHUD.BP_MainHUD_C|GetMainHUDRef _asbp_main_hud))
  (|Mapping))

(event Collision|EventActorBeginOverlap
  (params (OtherActor :type Actor%20Object%20Reference)))

(event EventTick
  (params (DeltaSeconds :type Float%20%28single-precision%29)))

(event Custom|Locomotion
  (params (ActionValue :type Float%20%28double-precision%29) (Pivot :type Scene%20Component%20Object%20Reference))
  ;[0.4532 1 0.3538] Movement Parent Functions
  (Pawn|Input|AddMovementInput (Math|Vector|GetForwardVector (Math|Rotator|MakeRotator 0.0 0.0 (.Yaw (Math|Rotator|BreakRotator (Transformation|GetWorldRotation Pivot))))) ActionValue false))

(event Custom|Strafe
  (params (ActionValue :type Float%20%28double-precision%29) (Pivot :type Scene%20Component%20Object%20Reference))
  ;[0.4532 1 0.3538] Movement Parent Functions
  (Pawn|Input|AddMovementInput (Math|Vector|GetRightVector (Math|Rotator|MakeRotator 0.0 0.0 (.Yaw (Math|Rotator|BreakRotator (Transformation|GetWorldRotation Pivot))))) ActionValue false))

(event Custom|BoomArmPitch
  (params (ActionValue :type Float%20%28double-precision%29) (UpperClamp :type Float%20%28double-precision%29))
  ;[0.3886 1 0.9101] Camera Controls
  (Variables|Default|SetBoomArmPitchRotation (Math|Float|Clamp(Float) (+ ActionValue (Variables|Default|GetBoomArmPitchRotation)) 0.0 UpperClamp)))

(event Custom|YawDirection&Lerp
  (params (ActionValue :type Float%20%28double-precision%29))
  ;[0.3886 1 0.9101] Camera Controls
  (if (> (Variables|Default|GetSqueezeAlpha) 0.0)
    (Variables|Default|SetYawDirection 0.0)
    (Variables|Default|SetYawLerp (+ ActionValue (Variables|Default|GetYawLerp)))))

(event Custom|Tick_InputVector
  (params (CameraYawPivot :type Static%20Mesh%20Component%20Object%20Reference) (SpringArm :type Spring%20Arm%20Component%20Object%20Reference))
  ;[0.1435 1 0.414] InputVector Tick
  (Variables|Default|SetInputVector (Math|Vector|RotateVector (Math|Vector|Normalize (Math|Vector|MakeVector (Variables|Default|GetXMovementValue) (Variables|Default|GetYMovementValue) 0.0)) (Math|Rotator|MakeRotator 0.0 0.0 (+ (.yaw (Variables|/Script/Engine.SceneComponent|GetRelativeRotation CameraYawPivot)) (.yaw (Class|SpringArmComponent|GetTargetRotation SpringArm)))))))

(event Custom|PlayerHealth
  (params (MaxHealth :type Float%20%28double-precision%29))
  ;[0.345 1 0.2628] Initialize Player Health
  (Variables|Default|SetHealth MaxHealth))

(event Custom|ResetCombo
  ;[1 0.2292 0.2292] Combo Reset
  (Variables|Default|SetAttackCount 0)
  (Utilities|FlowControl|Sequence
    (:then_0
      (Variables|Default|SetSaveAttack false))
    (:then_1
      (Variables|Default|SetIsAttacking false))
    (:then_2
      (Variables|Default|SetHeavyIsAttacking false))
    (:then_3
      (Variables|Default|SetHeavySaveAttack false))))

(event Custom|ComboSaveHeavy
  ;[0.7669 0.7622 1] Base Combo Mechanic
  ;;[1 0.5036 0.3015] Check if Heavy Attack should Combo or is Disconnected
  (if (Variables|Default|GetHeavySaveAttack)
    (Variables|Default|SetHeavySaveAttack false)
    ;;[1 0.9958 0.5284] Connect Correct Combo Animations
    (switch int (Variables|Default|GetAttackCount)
      (:0
        (Variables|Default|SetAttackCount 3)
        (Animation|PlayAnimMontage (stale Custom|HeavyAttackStart HeavyAttack1) 1.0 "None")
        (Variables|Default|SetKnockBackForce 2e+02)
        ;;[1 0.4268 0.6092] Set Thrust Power if Necessary
        (Variables|Default|SetAttackThrustPower (stale Custom|HeavyAttackStart AttackThrust1)))
      (:1
        (Variables|Default|SetAttackCount 4 :!label _label)
        (Animation|PlayAnimMontage (stale Custom|HeavyAttackStart HeavyAttack2) 1.0 "None")
        (Variables|Default|SetKnockBackForce 2.5e+02)
        (Variables|Default|SetAttackThrustPower (stale Custom|HeavyAttackStart AttackThrust1))
        (Variables|Default|SetIsAttacking false))
      (:2
        (Variables|Default|SetAttackCount 0 :!label _label_2)
        (Animation|PlayAnimMontage (stale Custom|HeavyAttackStart HeavyAttack3) 1.2 "None")
        (Variables|Default|SetKnockBackForce 4e+02)
        (Variables|Default|SetAttackThrustPower (stale Custom|HeavyAttackStart AttackThrust1)))
      (:3
        (goto _label))
      (:4
        (goto _label_2)))
    (bind _outhitactor (Utilities|DoTargetTrace 1e+02 5e+02 0.0)
      (:TargetHit
        ;;[0.6417 1 0.5249] Thrust Impulse Timeline
        (bind _alpha (Timeline|Timeline_0 PlayFromStart)
          (:Update
            (Utilities|IsValid _outhitactor
              (:Is%20Valid
                (Transformation|SetActorRotation (Math|Rotator|Lerp(Rotator) (Transformation|GetActorRotation) (Math|Rotator|MakeRotator 0.0 0.0 (.yaw (Math|Conversions|RotationFromXVector (Math|Rotator|GetRotationXVector (Math|Rotator|FindLookatRotation (Transformation|GetActorLocation) (Transformation|GetActorLocation _outhitactor)))))) 0.25 true))
                (Physics|AddImpulse (Variables|Character|GetCharacterMovement) (* (* (* (Transformation|GetActorRotation) (Variables|Default|GetAttackThrustPower)) _alpha) (/ 6e+01 (/ 1.0 (Utilities|Time|GetWorldDeltaSeconds)))) true))))))
      (:NoHit
        (bind _alpha_2 (Timeline|Timeline PlayFromStart)
          (:Update
            (Transformation|SetActorRotation (Math|Rotator|Lerp(Rotator) (Transformation|GetActorRotation) (Math|Rotator|MakeRotator 0.0 0.0 (.yaw (Math|Conversions|RotationFromXVector (Utilities|SelectVectoronInput)))) 0.25 true))
            (Physics|AddImpulse (Variables|Character|GetCharacterMovement) (* (* (* (Transformation|GetActorRotation) (Variables|Default|GetAttackThrustPower)) _alpha_2) (/ 6e+01 (/ 1.0 (Utilities|Time|GetWorldDeltaSeconds)))) true)))))))

(event Custom|Pause%20the%20Game
  (bind _returnvalue (Game|GetPlayerController 0))
  (bind _pausemenu (Variables|Default|GetPauseMenu))
  (bind _hudref (Variables|Default|GetHudRef))
  ;[0.2854 0.2935 1] Pause Menu
  (if (not (Variables|Default|GetIsPaused))
    (Variables|Default|SetIsPaused true)
    (Widget|SetVisibility _pausemenu "Visible")
    (Widget|SetVisibility _hudref "Hidden")
    (Input|SetInputModeGameandUI _returnvalue (Variables|Default|GetPauseMenu) "DoNotLock" true false)
    (Variables|/Script/Engine.PlayerController|SetbShowMouseCursor _returnvalue true)
    (Game|SetGamePaused true)
    (else
      (Variables|Default|SetIsPaused false)
      (Widget|SetVisibility _pausemenu "Hidden")
      (Widget|SetVisibility _hudref "Visible")
      (Game|SetGamePaused false)
      (Input|SetInputModeGameOnly _returnvalue false)
      (Variables|/Script/Engine.PlayerController|SetbShowMouseCursor _returnvalue false))))

(event Custom|Interactable
  (params (ThrowDistance :type Float%20%28double-precision%29) (TraceRadius :type Float%20%28double-precision%29) (HalfHeight :type Float%20%28double-precision%29) (HeightVector :type Vector) (ObjectHeightVector :type Vector) (ParentSkeleton :type Skeletal%20Mesh%20Component%20Object%20Reference) (CustomSocket :type Name) (CustomLocation :type Vector) (CustomScale :type Vector))
  (bind _returnvalue (Transformation|GetActorLocation))
  ;[0.9059 0.4464 1] Custom Interactable Code
  (if (not (Variables|Default|GetIsAttacking))
    (Utilities|IsValid (Variables|Default|GetInteractableObject)
      (:Is%20Valid
        ;;[1 1 1] Throw Throwable if already equipped
        (Transformation|DetachFromActor (Variables|Default|GetInteractableObject) "KeepWorld" "KeepWorld" "KeepWorld")
        (bind _asbp_throwable_base_obj (Utilities|Casting|CastToBP_ThrowableBaseObj (Variables|Default|GetInteractableObject)))
        (Variables|Default|SetIgnoreInteractable (Utilities|Array|MakeArray _asbp_throwable_base_obj))
        (Variables|Default|SetInteractableObject 0)
        (bind _output_get (Variables|/Game/Blueprints/Throwables/BP_ThrowableBaseObj.BP_ThrowableBaseObj_C|SetMaxThrowDisance _asbp_throwable_base_obj ThrowDistance))
        (bind _outhitactor (Utilities|DoTargetTrace TraceRadius _output_get HalfHeight) ; Capsule trace by selected vector
          (:TargetHit
            (Variables|/Game/Blueprints/Throwables/BP_ThrowableBaseObj.BP_ThrowableBaseObj_C|SetBotleArcInitAngle _asbp_throwable_base_obj (Math|Vector|GetUnitDirection(Vector) (Transformation|GetActorLocation) (Transformation|GetActorLocation _outhitactor))) ; If target hit, soft lock on to the enemy
          )
          (:NoHit
            (Variables|/Game/Blueprints/Throwables/BP_ThrowableBaseObj.BP_ThrowableBaseObj_C|SetBotleArcInitAngle _asbp_throwable_base_obj (Utilities|SelectVectoronInput)) ; if no target hit, throw in player's Select Vector
          ))
        (Variables|/Game/Blueprints/Throwables/BP_ThrowableBaseObj.BP_ThrowableBaseObj_C|SetThrowArcLerpStart _asbp_throwable_base_obj (Transformation|GetActorLocation))
        (Default|DoBottleThrowArc _asbp_throwable_base_obj) ; Run timeline curve event inside throwable
      )
      (:Is%20Not%20Valid
        ;;[1 1 1] Equip Throwable if one isn't equipped
        (bind (_outactors _returnvalue_2) (Collision|SphereOverlapActors _returnvalue 2.5e+02 (Utilities|Array|MakeArray "ObjectTypeQuery2") "/Game/Blueprints/Throwables/BP_ThrowableBaseObj.BP_ThrowableBaseObj_C" (Variables|Default|GetIgnoreInteractable))) ; sphere overlap, filter to check all throwables in radius
        (if _returnvalue_2
          (bind _outhit (Collision|LineTraceByChannel (+ HeightVector _returnvalue) (+ (Transformation|GetActorLocation (.ReturnValue (Actor|FindNearestActor _returnvalue _outactors))) ObjectHeightVector) "TraceTypeQuery1" false 0 "None")) ; (WIP) trace to check if bottle is in front of player
          (if (== (.hitactor _outhit) (.ReturnValue (Actor|FindNearestActor _returnvalue _outactors)))
            (bind _output_get_2 (Variables|Default|SetInteractableObject (.hitactor _outhit)))
            (Transformation|AttachComponentToComponent _output_get_2 ParentSkeleton CustomSocket "SnapToTarget" "SnapToTarget" "SnapToTarget" true) ; Attach throwable to character's equip socket
            (Class|Actor|AddActorLocalTransform _output_get_2 (Math|Transform|MakeTransform CustomLocation "0, 0, 0" CustomScale) false false) ; Set position of equip manually...
          ))))))

(event Custom|LightAttackStart
  (params (LightAttack1 :type Anim%20Montage%20Object%20Reference) (LightAttack2 :type Anim%20Montage%20Object%20Reference) (LightAttack3 :type Anim%20Montage%20Object%20Reference) (AttackThrust1 :type Float%20%28double-precision%29) (AttackThrust2 :type Float%20%28double-precision%29))
  ;[0.7669 0.7622 1] Base Combo Mechanic
  ;;[1 0.4682 0.3783] Check if Light Attack Should combo or is disconnected
  (if (Variables|Default|GetIsAttacking)
    (Variables|Default|SetSaveAttack true)
    (else
      (Variables|Default|SetIsAttacking true)
      ;;[0.9547 1 0.5198] Connect Correct Combo Animations
      (switch int (Variables|Default|GetAttackCount)
        (:0
          (Variables|Default|SetAttackCount 1)
          (Animation|PlayAnimMontage LightAttack1 1.0 "None")
          (Variables|Default|SetKnockBackForce 1.5e+02)
          ;;[1 0.4268 0.6092] Set Thrust Power if Necessary
          (Variables|Default|SetAttackThrustPower AttackThrust1))
        (:1
          (Variables|Default|SetAttackCount 2 :!label _label)
          (Animation|PlayAnimMontage LightAttack2 0.5 "None")
          (Variables|Default|SetKnockBackForce 2.5e+02)
          (Variables|Default|SetAttackThrustPower AttackThrust1)
          (Variables|Default|SetHeavyIsAttacking false))
        (:2
          (Variables|Default|SetAttackCount 0 :!label _label_2)
          (Animation|PlayAnimMontage LightAttack3 1.0 "None")
          (Variables|Default|SetKnockBackForce 3e+02)
          (Variables|Default|SetAttackThrustPower AttackThrust2))
        (:3
          (goto _label))
        (:4
          (goto _label_2)))
      (bind _outhitactor (Utilities|DoTargetTrace 1e+02 5e+02 0.0)
        (:TargetHit
          ;;[0.6417 1 0.5249] Thrust Impulse Timeline
          (bind _alpha (Timeline|Timeline_0 PlayFromStart)
            (:Update
              (Utilities|IsValid _outhitactor
                (:Is%20Valid
                  (Transformation|SetActorRotation (Math|Rotator|Lerp(Rotator) (Transformation|GetActorRotation) (Math|Rotator|MakeRotator 0.0 0.0 (.yaw (Math|Conversions|RotationFromXVector (Math|Rotator|GetRotationXVector (Math|Rotator|FindLookatRotation (Transformation|GetActorLocation) (Transformation|GetActorLocation _outhitactor)))))) 0.25 true))
                  (Physics|AddImpulse (Variables|Character|GetCharacterMovement) (* (* (* (Transformation|GetActorRotation) (Variables|Default|GetAttackThrustPower)) _alpha) (/ 6e+01 (/ 1.0 (Utilities|Time|GetWorldDeltaSeconds)))) true))))))
        (:NoHit
          (bind _alpha_2 (Timeline|Timeline PlayFromStart)
            (:Update
              (Transformation|SetActorRotation (Math|Rotator|Lerp(Rotator) (Transformation|GetActorRotation) (Math|Rotator|MakeRotator 0.0 0.0 (.yaw (Math|Conversions|RotationFromXVector (Utilities|SelectVectoronInput)))) 0.25 true))
              (Physics|AddImpulse (Variables|Character|GetCharacterMovement) (* (* (* (Transformation|GetActorRotation) (Variables|Default|GetAttackThrustPower)) _alpha_2) (/ 6e+01 (/ 1.0 (Utilities|Time|GetWorldDeltaSeconds)))) true))))))))

(event Custom|ComboSaveLight
  ;[0.7669 0.7622 1] Base Combo Mechanic
  ;;[1 0.4682 0.3783] Check if Light Attack Should combo or is disconnected
  (if (Variables|Default|GetSaveAttack)
    (Variables|Default|SetSaveAttack false)
    ;;[0.9547 1 0.5198] Connect Correct Combo Animations
    (switch int (Variables|Default|GetAttackCount)
      (:0
        (Variables|Default|SetAttackCount 1)
        (Animation|PlayAnimMontage (stale Custom|LightAttackStart LightAttack1) 1.0 "None")
        (Variables|Default|SetKnockBackForce 1.5e+02)
        ;;[1 0.4268 0.6092] Set Thrust Power if Necessary
        (Variables|Default|SetAttackThrustPower (stale Custom|LightAttackStart AttackThrust1)))
      (:1
        (Variables|Default|SetAttackCount 2 :!label _label)
        (Animation|PlayAnimMontage (stale Custom|LightAttackStart LightAttack2) 0.5 "None")
        (Variables|Default|SetKnockBackForce 2.5e+02)
        (Variables|Default|SetAttackThrustPower (stale Custom|LightAttackStart AttackThrust1))
        (Variables|Default|SetHeavyIsAttacking false))
      (:2
        (Variables|Default|SetAttackCount 0 :!label _label_2)
        (Animation|PlayAnimMontage (stale Custom|LightAttackStart LightAttack3) 1.0 "None")
        (Variables|Default|SetKnockBackForce 3e+02)
        (Variables|Default|SetAttackThrustPower (stale Custom|LightAttackStart AttackThrust2)))
      (:3
        (goto _label))
      (:4
        (goto _label_2)))
    (bind _outhitactor (Utilities|DoTargetTrace 1e+02 5e+02 0.0)
      (:TargetHit
        ;;[0.6417 1 0.5249] Thrust Impulse Timeline
        (bind _alpha (Timeline|Timeline_0 PlayFromStart)
          (:Update
            (Utilities|IsValid _outhitactor
              (:Is%20Valid
                (Transformation|SetActorRotation (Math|Rotator|Lerp(Rotator) (Transformation|GetActorRotation) (Math|Rotator|MakeRotator 0.0 0.0 (.yaw (Math|Conversions|RotationFromXVector (Math|Rotator|GetRotationXVector (Math|Rotator|FindLookatRotation (Transformation|GetActorLocation) (Transformation|GetActorLocation _outhitactor)))))) 0.25 true))
                (Physics|AddImpulse (Variables|Character|GetCharacterMovement) (* (* (* (Transformation|GetActorRotation) (Variables|Default|GetAttackThrustPower)) _alpha) (/ 6e+01 (/ 1.0 (Utilities|Time|GetWorldDeltaSeconds)))) true))))))
      (:NoHit
        (bind _alpha_2 (Timeline|Timeline PlayFromStart)
          (:Update
            (Transformation|SetActorRotation (Math|Rotator|Lerp(Rotator) (Transformation|GetActorRotation) (Math|Rotator|MakeRotator 0.0 0.0 (.yaw (Math|Conversions|RotationFromXVector (Utilities|SelectVectoronInput)))) 0.25 true))
            (Physics|AddImpulse (Variables|Character|GetCharacterMovement) (* (* (* (Transformation|GetActorRotation) (Variables|Default|GetAttackThrustPower)) _alpha_2) (/ 6e+01 (/ 1.0 (Utilities|Time|GetWorldDeltaSeconds)))) true)))))))

(event Custom|Load%20Data%20Base
  ;[1 1 1] Load Data, Work in Progress
  (bind _asbp_game_instance (Utilities|Casting|CastToBP_GameInstance (Game|GetGameInstance)))
  (bind _asbp_save_game (Default|LoadData _asbp_game_instance))
  (Utilities|IsValid _asbp_save_game
    (:Is%20Valid
      (Utilities|FlowControl|Sequence))))

(event Custom|Save%20Data%20Base
  (params (ScoreCalc :type Score%20Calculator%20Object%20Reference))
  ;[1 1 1] Save Data, Work in Progress
  (bind _asbp_game_instance (Utilities|Casting|CastToBP_GameInstance (Game|GetGameInstance)))
  (bind _returnvalue (SaveGame|CreateSaveGameObject "/Game/Blueprints/BP_SaveGame.BP_SaveGame_C"))
  (Variables|/Game/Blueprints/BP_SaveGame.BP_SaveGame_C|SetSaveLevel _returnvalue 0)
  (bind _final_score (Default|FinalCalc ScoreCalc))
  (Variables|/Game/Blueprints/BP_SaveGame.BP_SaveGame_C|SetSaveScore _returnvalue _final_score)
  (Default|SaveData _asbp_game_instance "FileName" true _returnvalue))

(event Custom|HeavyAttackStart
  (params (HeavyAttack1 :type Anim%20Montage%20Object%20Reference) (HeavyAttack2 :type Anim%20Montage%20Object%20Reference) (HeavyAttack3 :type Anim%20Montage%20Object%20Reference) (AttackThrust1 :type Float%20%28double-precision%29))
  ;[0.7669 0.7622 1] Base Combo Mechanic
  ;;[1 0.5036 0.3015] Check if Heavy Attack should Combo or is Disconnected
  (if (Variables|Default|GetHeavyIsAttacking)
    (Variables|Default|SetHeavySaveAttack true)
    (else
      (Variables|Default|SetHeavyIsAttacking true)
      ;;[1 0.9958 0.5284] Connect Correct Combo Animations
      (switch int (Variables|Default|GetAttackCount)
        (:0
          (Variables|Default|SetAttackCount 3)
          (Animation|PlayAnimMontage HeavyAttack1 1.0 "None")
          (Variables|Default|SetKnockBackForce 2e+02)
          ;;[1 0.4268 0.6092] Set Thrust Power if Necessary
          (Variables|Default|SetAttackThrustPower AttackThrust1))
        (:1
          (Variables|Default|SetAttackCount 4 :!label _label)
          (Animation|PlayAnimMontage HeavyAttack2 1.0 "None")
          (Variables|Default|SetKnockBackForce 2.5e+02)
          (Variables|Default|SetAttackThrustPower AttackThrust1)
          (Variables|Default|SetIsAttacking false))
        (:2
          (Variables|Default|SetAttackCount 0 :!label _label_2)
          (Animation|PlayAnimMontage HeavyAttack3 1.2 "None")
          (Variables|Default|SetKnockBackForce 4e+02)
          (Variables|Default|SetAttackThrustPower AttackThrust1))
        (:3
          (goto _label))
        (:4
          (goto _label_2)))
      (bind _outhitactor (Utilities|DoTargetTrace 1e+02 5e+02 0.0)
        (:TargetHit
          ;;[0.6417 1 0.5249] Thrust Impulse Timeline
          (bind _alpha (Timeline|Timeline_0 PlayFromStart)
            (:Update
              (Utilities|IsValid _outhitactor
                (:Is%20Valid
                  (Transformation|SetActorRotation (Math|Rotator|Lerp(Rotator) (Transformation|GetActorRotation) (Math|Rotator|MakeRotator 0.0 0.0 (.yaw (Math|Conversions|RotationFromXVector (Math|Rotator|GetRotationXVector (Math|Rotator|FindLookatRotation (Transformation|GetActorLocation) (Transformation|GetActorLocation _outhitactor)))))) 0.25 true))
                  (Physics|AddImpulse (Variables|Character|GetCharacterMovement) (* (* (* (Transformation|GetActorRotation) (Variables|Default|GetAttackThrustPower)) _alpha) (/ 6e+01 (/ 1.0 (Utilities|Time|GetWorldDeltaSeconds)))) true))))))
        (:NoHit
          (bind _alpha_2 (Timeline|Timeline PlayFromStart)
            (:Update
              (Transformation|SetActorRotation (Math|Rotator|Lerp(Rotator) (Transformation|GetActorRotation) (Math|Rotator|MakeRotator 0.0 0.0 (.yaw (Math|Conversions|RotationFromXVector (Utilities|SelectVectoronInput)))) 0.25 true))
              (Physics|AddImpulse (Variables|Character|GetCharacterMovement) (* (* (* (Transformation|GetActorRotation) (Variables|Default|GetAttackThrustPower)) _alpha_2) (/ 6e+01 (/ 1.0 (Utilities|Time|GetWorldDeltaSeconds)))) true))))))))

(event Input|KeyboardEvents|DebugKeyX
  (params (Key :type Key%20Structure :default "None") (ActionValue :type Input%20Action%20Value%20Structure))
  (bind _returnvalue (Transformation|GetActorLocation))
  ;[0 0 0] Debug Nuke
  (:Pressed
    (bind _outhits (Collision|MultiSphereTraceForObjects _returnvalue _returnvalue 2.5e+02 (Utilities|Array|MakeArray "ObjectTypeQuery3" "ObjectTypeQuery6") false 0 "None"))
    (for _array_element _outhits
      (Game|Damage|ApplyDamage (.hitactor _array_element) 9999.0 0 0 "/Game/Blueprints/Damaging/DT_PlayerHeavyAttack.DT_PlayerHeavyAttack_C"))))

(fn ConstructionScript)