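; BP_CharSelect is an interactable that sends the player back to character selection.
; On InteractAction it destroys every actor directly attached to player character 0, then the character itself.
; It then calls InteractOpenCharSelect to request the character select, whose handling lives outside this Blueprint.
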(event EventBeginPlay
  (|CallParentFunction) ; This node is disabled and will not be called.\nDrag off pins to build functionality.
)

(event Collision|EventActorBeginOverlap
  (params (OtherActor :type Actor%20Object%20Reference)))

(event EventTick
  (params (DeltaSeconds :type Float%20%28single-precision%29)))

(event EventInteractAction
  ;[1 1 1] interact; destroy entire character and call character select
  (for _array_element (Actor|GetAttachedActors (Game|GetPlayerCharacter 0) true false)
    (Actor|DestroyActor _array_element))
  (Actor|DestroyActor (Game|GetPlayerCharacter 0))
  (Default|CallInteractOpenCharSelect))

(fn ConstructionScript
  (|CallParentFunction))