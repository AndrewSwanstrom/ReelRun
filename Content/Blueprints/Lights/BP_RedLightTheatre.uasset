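; BP_RedLightTheatre is a wall light that stages a one-time lighting event when a player or other Base_Character enters its trigger box.
; The first overlap sets the spotlight to a high intensity and plays an electrical flicker sound at the wall light mesh.
; After a short delay the spotlight drops to a very low intensity as the sound stops, and a DoOnce keeps it from repeating.
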(event OnComponentBeginOverlap(Box)
  (params (OverlappedComponent :type Primitive%20Component%20Object%20Reference) (OtherActor :type Actor%20Object%20Reference) (OtherComp :type Primitive%20Component%20Object%20Reference) (OtherBodyIndex :type Integer) (bFromSweep :type Boolean) (SweepResult :type Hit%20Result%20Structure%20%28by%20ref%29))
  (Utilities|Casting|CastToBase_Character OtherActor)
  (Utilities|FlowControl|DoOnce false
    (:Completed
      (Rendering|Components|Light|SetIntensity (Variables|Default|GetSpotLight) 1e+03)
      (bind _returnvalue (Audio|SpawnSoundatLocation "/Game/Art/SFX/Horror/232446__mmaruska__lights-flicker-on-and-some-electrical-noises.232446__mmaruska__lights-flicker-on-and-some-electrical-noises" (Transformation|GetWorldLocation (Variables|Default|GetSM_WallLight_01)) "0, 0, 0" 1.0 1.0 1.0 0 0))
      (Audio|Components|Audio|StopDelayed _returnvalue 3.0)
      (Utilities|FlowControl|Delay 3.0)
      (Rendering|Components|Light|SetIntensity (Variables|Default|GetSpotLight) 3.0))))

(fn ConstructionScript)