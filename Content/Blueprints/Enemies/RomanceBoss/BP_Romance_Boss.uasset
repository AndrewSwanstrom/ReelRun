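; BP_Romance_Boss is an enemy boss character, still mostly a skeleton.
; BeginPlay records the starting Health as MaxHealth, and SetMovementSpeed maps idle, walking and sprinting states to the character's max walk speed.
; AttackStart and GetIdealRange are placeholders that return false and zero radii, so the file defines no attack or range behavior of its own.
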(event EventBeginPlay
  (Variables|Default|SetMaxHealth (Variables|Default|GetHealth)))

(event Collision|EventActorBeginOverlap
  (params (OtherActor :type Actor%20Object%20Reference)))

(event EventTick
  (params (DeltaSeconds :type Float%20%28single-precision%29)))

(fn ConstructionScript)

(fn AttackStart
  (params (AttackTarget :type Actor%20Object%20Reference) (Tokens%20Needed :type Integer))
  (return false))

(fn GetIdealRange
  (return 0.0 0.0 0.0))

(fn SetMovementSpeed
  (params (Speed :type E_MovementSpeed%20Enum :default "NewEnumerator0"))
  (bind _output_get (Variables|/Script/Engine.CharacterMovementComponent|SetMaxWalkSpeed (Variables|Character|GetCharacterMovement) (Utilities|Select :Index Speed :NewEnumerator0 0.0 :NewEnumerator1 1e+02 :NewEnumerator2 6e+02)))
  (return _output_get))