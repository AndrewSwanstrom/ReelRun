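; BP_SnackThrowable is a throwable snack pickup with a mesh that can be set through SetSnackMesh.
; Its sphere overlaps pass the interact icon and mesh to shared begin and end overlap handlers.
; Each tick it runs ThrowableDamage once thrown.
; Before that, it clears the mesh's overlay material if the player holds an item, and otherwise rotates the interact icon.
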(event OnComponentBeginOverlap(Sphere)
  (params (OverlappedComponent :type Primitive%20Component%20Object%20Reference) (OtherActor :type Actor%20Object%20Reference) (OtherComp :type Primitive%20Component%20Object%20Reference) (OtherBodyIndex :type Integer) (bFromSweep :type Boolean) (SweepResult :type Hit%20Result%20Structure%20%28by%20ref%29))
  (CallFunction|BeginColliderOverlap OtherActor (Variables|Default|GetInteractIconParent) (Variables|Default|GetItemMesh)))

(event OnComponentEndOverlap(Sphere)
  (params (OverlappedComponent :type Primitive%20Component%20Object%20Reference) (OtherActor :type Actor%20Object%20Reference) (OtherComp :type Primitive%20Component%20Object%20Reference) (OtherBodyIndex :type Integer))
  (CallFunction|EndColliderOverlap OtherActor (Variables|Default|GetInteractIconParent) (Variables|Default|GetItemMesh)))

(event Custom|SetSnackMesh
  (params (StaticMesh :type Static%20Mesh%20Object%20Reference))
  (Components|StaticMesh|SetStaticMesh (Variables|Default|GetItemMesh) StaticMesh))

(event EventTick
  (params (DeltaSeconds :type Float%20%28single-precision%29))
  (if (Variables|Default|GetBottleThrown)
    (CallFunction|ThrowableDamage (Variables|Default|GetItemMesh))
    (else
      (bind _asbase_character (Utilities|Casting|CastToBase_Character (Game|GetPlayerCharacter 0)))
      (if (Variables|/Game/Blueprints/Characters/Base_Character.Base_Character_C|GetbHasItem _asbase_character)
        (Rendering|Material|SetOverlayMaterial (Variables|Default|GetItemMesh) 0 :!class /Script/Engine.MeshComponent)
        (else
          (CallFunction|RotateInteractIcon (Variables|Default|GetInteractIconParent)))))))

(fn ConstructionScript
  (|CallParentFunction))