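; Cutscene manager actor that plays level sequences and provides event helpers for spawning enemies and teleporting the player.
; RunSequencer scans the sequence's tracks for a camera cut track to detect a cutscene, which hides the HUD, shows a cutscene widget and disables player input until finished.
; IA_SkipCutscene jumps the playing sequence to its end.
; SpawnAll triggers enemy spawn points attached to a given actor; WalkPlayer and TurnPlayerCamera are empty.
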(event Custom|RunSequencer
  (params (CutsceneSequencePlayer :type Level%20Sequence%20Actor%20Object%20Reference))
  (Development|PrintString "note: skip will work for normal sequence right now" true true "(R=1.000000,G=0.031241,B=0.000000,A=1.000000)")
  ;[1 1 1] Run Sequencer, dynamically determine whether or not this a cutscene or a standard sequence
  (Variables|Default|SetCutscene%20Sequence%20Player CutsceneSequencePlayer)
  (bind _returnvalue (Class|MovieSceneSequenceExtensions|GetTracks (Class|LevelSequenceActor|GetSequence CutsceneSequencePlayer)))
  (bind _array_element (Utilities|Array|ForEachLoopwithBreak _returnvalue :!label _label)
    (:LoopBody
      (if (== (Utilities|GetClass _array_element) "/Script/MovieSceneTracks.MovieSceneCameraCutTrack")
        ;[1 1 1] For playing sequencers with a cutscene
        ;;[1 1 1] Hide Hud
        (bind _foundwidgets (Widget|GetAllWidgetsOfClass "/Game/Blueprints/UI/HUD/WBP_PlayerHUD.WBP_PlayerHUD_C" true))
        (Default|HideShowHud (Utilities|Array|Get(acopy) _foundwidgets) "Collapsed")
        ;;[1 1 1] Skip Cutscene Widget
        (bind _returnvalue_2 (UserInterface|CreateWidget "/Game/Blueprints/UI/HUD/WBP_Cutscene.WBP_Cutscene_C"))
        (Variables|Default|SetCutsceneWidgetRef _returnvalue_2)
        (UserInterface|Viewport|AddtoViewport _returnvalue_2 0)
        (Input|DisableInput (Game|GetPlayerCharacter 0) (Game|GetPlayerController 0))
        (Sequencer|Player|Play (Variables|/Script/LevelSequence.LevelSequenceActor|GetSequencePlayer (Variables|Default|GetCutscene%20Sequence%20Player)) :!class /Script/MovieScene.MovieSceneSequencePlayer)
        (EventDispatchers|BindEventtoOnFinished (Variables|/Script/LevelSequence.LevelSequenceActor|GetSequencePlayer (Variables|Default|GetCutscene%20Sequence%20Player)) (delegate Custom|CutsceneFinished))
        (goto _label Break)
        (else
          ;[1 1 1] For playing sequencers without a cutscene
          (Sequencer|Player|Play (Variables|/Script/LevelSequence.LevelSequenceActor|GetSequencePlayer (Variables|Default|GetCutscene%20Sequence%20Player)) :!class /Script/MovieScene.MovieSceneSequencePlayer))))))

(event Custom|CutsceneFinished
  ;[1 1 1] Remove widget and give player control back
  (Widget|RemovefromParent (Variables|Default|GetCutsceneWidgetRef))
  (Input|EnableInput (Game|GetPlayerCharacter 0) (Game|GetPlayerController 0))
  ;[1 1 1] Show Hud
  (bind _foundwidgets (Widget|GetAllWidgetsOfClass "/Game/Blueprints/UI/HUD/WBP_PlayerHUD.WBP_PlayerHUD_C" true))
  (Default|HideShowHud (Utilities|Array|Get(acopy) _foundwidgets) "Visible"))

(event Input|EnhancedActionEvents|EnhancedInputActionIA_SkipCutscene
  (params (ActionValue :type Boolean) (ElapsedSeconds :type Float%20%28double-precision%29) (TriggeredSeconds :type Float%20%28double-precision%29) (InputAction :type Input%20Action%20Object%20Reference :default "/Game/Blueprints/Input/Actions/IA_SkipCutscene.IA_SkipCutscene"))
  (bind _cutscene_sequence_player (Variables|Default|GetCutscene%20Sequence%20Player))
  (bind _sequenceplayer (Variables|/Script/LevelSequence.LevelSequenceActor|GetSequencePlayer _cutscene_sequence_player))
  ;[1 0.2364 0.2185] Skip Cutscene
  (:Started
    (Utilities|IsValid (Variables|Default|GetCutscene%20Sequence%20Player)
      (:Is%20Valid
        (if (Audio|Components|Audio|IsPlaying _sequenceplayer)
          (Components|Timeline|SetPlaybackPosition _sequenceplayer (Utilities|Struct|MakeMovieSceneSequencePlaybackParams (Utilities|Struct|MakeFrameTime (Utilities|Struct|MakeFrameNumber (.value (.frame (Media|MediaPlayer|GetDuration _sequenceplayer)))) 0.0) 0.0 "" "(Hours=0,Minutes=0,Seconds=0,Frames=0,bDropFrameFormat=False)" "Frame" "Play")))))))

(event EventBeginPlay
  ;[1 1 1] allow this to read input
  (Input|EnableInput (Game|GetPlayerController 0)))

(event Custom|SpawnAll
  (params (Sequencer :type Level%20Sequence%20Actor%20Object%20Reference))
  (Utilities|IsValid Sequencer
    (:Is%20Valid
      (Variables|Default|SetOut%20Actors (Actor|GetAttachedActors Sequencer true false))
      (for _array_element (Variables|Default|GetOut%20Actors)
        (bind _asbp_enemy_spawnpoint (Utilities|Casting|CastToBP_EnemySpawnpoint _array_element))
        (Default|SpawnEnemy _asbp_enemy_spawnpoint)))
    (:Is%20Not%20Valid
      (Development|PrintString "Sequencer Unset" true true "(R=1.000000,G=0.000000,B=0.046022,A=1.000000)"))))

(event Custom|Spawn
  (params (EnemySpawnClass :type BP%20Enemy%20Spawnpoint%20Object%20Reference))
  (Default|SpawnEnemy EnemySpawnClass))

(event Custom|TeleportPlayer
  (params (TeleportPoint :type Target%20Point%20Object%20Reference))
  (Transformation|SetActorTransform (Game|GetPlayerCharacter 0) (Transformation|GetActorTransform TeleportPoint) false true))

(event Custom|WalkPlayer)

(event Custom|TurnPlayerCamera)

(fn ConstructionScript)