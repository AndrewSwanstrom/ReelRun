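; Spline-placed string of hanging lights for the horror content, which plays a quiet glass clinking sound on BeginPlay.
; The construction script adds a pole at each spline point and evenly spaced bulb meshes between them, offset along a sine curve scaled by Gravity.
; Two elongated point lights per segment, angled toward the sag, approximate the strand's glow.
; LightsOn toggles light visibility and bulb material color; cable and spline-mesh ropes are disconnected experiments.
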(event EventBeginPlay
  (Audio|PlaySoundatLocation "/Game/Art/SFX/Horror/498516__16hpanskazavadovsky_igor__3-clinking-deep-regular-glass.498516__16hpanskazavadovsky_igor__3-clinking-deep-regular-glass" (Transformation|GetWorldLocation (Variables|Default|GetDefaultSceneRoot)) "0, 0, 0" 0.25 2.0 0.0 "/Game/Art/SFX/Attenuations/WoodBreakAtten.WoodBreakAtten" 0 0 0))

(event Collision|EventActorBeginOverlap
  (params (OtherActor :type Actor%20Object%20Reference)))

(event EventTick
  (params (DeltaSeconds :type Float%20%28single-precision%29)))

(fn ConstructionScript
  (bind _spline (Variables|Default|GetSpline))
  ;[0.7985 0.4302 1] Set up spline points and beams
  (for _index (range 0 (- (Spline|GetNumberOfSplinePoints (Variables|Default|GetSpline)) 2))
    (Variables|Default|SetSplineStartPos (Spline|GetLocationatSplinePoint (Variables|Default|GetSpline) _index "Local"))
    (Variables|Default|SetSplineEndPos (Spline|GetLocationatSplinePoint (Variables|Default|GetSpline) (+ _index 1) "Local"))
    (Variables|Default|SetSplineDistance (Math|Vector|Distance(Vector) (Variables|Default|GetSplineStartPos) (Variables|Default|GetSplineEndPos)))
    (Variables|Default|SetSplineUnitDirection (Math|Vector|GetUnitDirection(Vector) (Variables|Default|GetSplineStartPos) (Variables|Default|GetSplineEndPos)))
    (AddComponent|AddStaticMeshComponent false (Math|Conversions|ToTransform(Vector) (Variables|Default|GetSplineStartPos))) ; set up pole mesh
    ;[1 1 0.1802] Place long Point Lights
    (bind _returnvalue (AddComponent|AddPointLightComponent false (Math|Transform|MakeTransform (- (+ (Variables|Default|GetSplineStartPos) (* (Variables|Default|GetSplineUnitDirection) (/ (Variables|Default|GetSplineDistance) 4.0))) (Math|Vector|MakeVector 0.0 0.0 3e+01)) (Math|Rotator|Delta(Rotator) (Math|Rotator|FindLookatRotation (Variables|Default|GetSplineStartPos) (+ (+ (Variables|Default|GetSplineStartPos) (* (Variables|Default|GetSplineUnitDirection) (/ (Variables|Default|GetSplineDistance) 2.0))) (Math|Vector|MakeVector 0.0 0.0 (Variables|Default|GetGravity)))) "90.000000,0.000000,0.000000") "1.000000,1.000000,1.000000")))
    (Class|PointLightComponent|SetSourceRadius _returnvalue 3e+01)
    (Class|PointLightComponent|SetSourceLength _returnvalue (/ (Variables|Default|GetSplineDistance) 2.0))
    (Rendering|Components|Light|SetLightColor _returnvalue (Variables|Light|GetLightColorVector) true)
    (Rendering|Components|Light|SetIntensity _returnvalue (Variables|Light|GetIntensity))
    (Class|LightComponent|SetTemperature _returnvalue (Variables|Light|GetTemperature))
    (Rendering|Lighting|SetAttenuationRadius _returnvalue (Variables|Light|GetAttenuationRadius))
    (Rendering|Components|Light|SetCastShadows _returnvalue (Variables|Light|GetCastShadows))
    (bind _returnvalue_2 (AddComponent|AddPointLightComponent false (Math|Transform|MakeTransform (- (+ (Variables|Default|GetSplineEndPos) (* (Variables|Default|GetSplineUnitDirection) (/ (Variables|Default|GetSplineDistance) 4.0) -1.0)) (Math|Vector|MakeVector 0.0 0.0 3e+01)) (Math|Rotator|Delta(Rotator) (Math|Rotator|FindLookatRotation (Variables|Default|GetSplineEndPos) (+ (+ (Variables|Default|GetSplineStartPos) (* (Variables|Default|GetSplineUnitDirection) (/ (Variables|Default|GetSplineDistance) 2.0))) (Math|Vector|MakeVector 0.0 0.0 (Variables|Default|GetGravity)))) "90.000000,0.000000,0.000000") "1.000000,1.000000,1.000000")))
    (Class|PointLightComponent|SetSourceRadius _returnvalue_2 3e+01)
    (Class|PointLightComponent|SetSourceLength _returnvalue_2 (/ (Variables|Default|GetSplineDistance) 2.0))
    (Rendering|Components|Light|SetLightColor _returnvalue_2 (Variables|Light|GetLightColorVector) true)
    (Rendering|Components|Light|SetIntensity _returnvalue_2 (Variables|Light|GetIntensity))
    (Class|LightComponent|SetTemperature _returnvalue_2 (Variables|Light|GetTemperature))
    (Rendering|Lighting|SetAttenuationRadius _returnvalue_2 (Variables|Light|GetAttenuationRadius))
    (Rendering|Components|Light|SetCastShadows _returnvalue_2 (Variables|Light|GetCastShadows))
    (Rendering|SetVisibility _returnvalue_2 (Variables|Default|GetLightsOn) false) ; lights on/off
    ;[1 0.6405 0.2177] Place light bulbs
    (for _index_2 (range 0 (Math|Float|Truncate (/ (Variables|Default|GetSplineDistance) (Variables|Default|GetDistanceBetweenLights))))
      (bind _returnvalue_3 (AddComponent|AddStaticMeshComponent false (Math|Conversions|ToTransform(Vector) (+ (+ (* (Variables|Default|GetSplineUnitDirection) (* _index_2 (Variables|Default|GetDistanceBetweenLights))) (Variables|Default|GetSplineStartPos)) (Math|Vector|MakeVector 0.0 0.0 (* (Math|Trig|Sin(Degrees) (* (/ (* _index_2 (Variables|Default|GetDistanceBetweenLights)) (/ (Variables|Default|GetSplineDistance) (Variables|Default|GetDistanceBetweenLights))) (Variables|Default|Getdebugsine))) (Variables|Default|GetGravity))))))) ; set up light bulb mesh
      (Rendering|Material|SetVectorParameterValueonMaterials _returnvalue_3 "ColorVector" (Math|Vector|SelectVector (Math|Conversions|ToVector(LinearColor) (Variables|Default|GetMaterialColorVector)) "0, 0, 0" (Variables|Default|GetLightsOn)))
      (Rendering|SetCastShadow _returnvalue_3 false)))
  (AddComponent|AddStaticMeshComponent false (Math|Conversions|ToTransform(Vector) (Spline|GetLocationatSplinePoint _spline (Spline|GetNumberOfSplinePoints _spline) "Local"))) ; place last pole
)