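; Base locked door that the player opens with the interact input while inside its box trigger, once KeyObtained is true.
; Overlap toggles the interact icon, which Tick rotates toward the player camera.
; Interacting destroys the trigger, plays OpenSequence and optionally passes per-instance mission text to Base_Character.
; Sequencer event endpoints activate the slam and slash effects, switching the slam off after a short delay.
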(event OnComponentBeginOverlap(Box)
  (params (OverlappedComponent :type Primitive%20Component%20Object%20Reference) (OtherActor :type Actor%20Object%20Reference) (OtherComp :type Primitive%20Component%20Object%20Reference) (OtherBodyIndex :type Integer) (bFromSweep :type Boolean) (SweepResult :type Hit%20Result%20Structure%20%28by%20ref%29))
  (Variables|Default|SetisIn true)
  (if (Variables|Default|GetKeyObtained)
    (Rendering|SetVisibility (Variables|Default|GetInteract%20Icon) true false)))

(event OnComponentEndOverlap(Box)
  (params (OverlappedComponent :type Primitive%20Component%20Object%20Reference) (OtherActor :type Actor%20Object%20Reference) (OtherComp :type Primitive%20Component%20Object%20Reference) (OtherBodyIndex :type Integer))
  (Variables|Default|SetisIn false)
  (if (Variables|Default|GetKeyObtained)
    (Rendering|SetVisibility (Variables|Default|GetInteract%20Icon) false false)))

(event Input|EnhancedActionEvents|EnhancedInputActionIA_Interact
  (params (ActionValue :type Boolean) (ElapsedSeconds :type Float%20%28double-precision%29) (TriggeredSeconds :type Float%20%28double-precision%29) (InputAction :type Input%20Action%20Object%20Reference :default "/Game/Blueprints/Input/Actions/IA_Interact.IA_Interact"))
  ;[1 1 1] interact; opens door w/ animation
  (:Started
    (if (and (Variables|Default|GetisIn) (Variables|Default|GetKeyObtained))
      (Components|DestroyComponent (Variables|Default|GetBox))
      (Variables|Default|SetisIn false)
      (Class|ActorSequenceComponent|PlaySequence (Variables|Default|GetOpenSequence)) ; Play OpenSequence animation
      ;[1 1 1] Update mission text after unlocked (if any text was set in BP details panel)
      (if (Utilities|Enum|NotEqual(Enum) (Variables|Default|GetDoorUnlockMissionText) "")
        (bind _asbase_character (Utilities|Casting|CastToBase_Character (Game|GetPlayerCharacter 0)))
        (Default|UpdateMissionText _asbase_character (Variables|Default|GetDoorUnlockMissionText)) ; update mission text when key taken
      ))))

(event EventTick
  (params (DeltaSeconds :type Float%20%28single-precision%29))
  ;[1 1 1] we can replace these with a UI so we dont have to event Tick
  (if (Variables|Default|GetisIn)
    (Transformation|SetWorldRotation (Variables|Default|GetInteract%20Icon) (Math|Rotator|FindLookatRotation (Transformation|GetWorldLocation (Variables|Default|GetInteract%20Icon)) (Transformation|GetWorldLocation (Variables|/Script/Engine.PlayerCameraManager|GetTransformComponent (Game|GetPlayerCameraManager 0)))) false false)))

(event EventBeginPlay
  (Input|EnableInput (Game|GetPlayerController 0)))

(event Custom|NiagaraSlam1_Event
  (params (NiagaraSlam1 :type Niagara%20Component%20Object%20Reference) (bReset :type Boolean))
  (Components|Activation|Activate NiagaraSlam1 bReset)
  (Utilities|FlowControl|Delay 1.0)
  (Components|Activation|Deactivate NiagaraSlam1))

(event Custom|SwingSlash_Event
  (params (SwingSlash :type Niagara%20Component%20Object%20Reference) (bReset :type Boolean))
  (Components|Activation|Activate SwingSlash bReset))

(fn ConstructionScript)