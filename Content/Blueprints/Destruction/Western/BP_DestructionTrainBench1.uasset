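; BP_DestructionTrainBench1 is a Chaos-destructible train bench for the Western destruction set, built from two geometry collections.
; A break event on either collection fires a transient radial velocity field at the destruction center.
; The first break also removes the invisible collision box and changes the first collection's collision channel.
; After a delay, it disables physics and collision on both pieces as an optimization, then randomly destroys the actor half the time.
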(event OnChaosBreakEvent(GC_SM_MERGED_StaticMeshActor_102)
  (params (BreakEvent :type Chaos%20Break%20Event%20Structure%20%28by%20ref%29))
  (bind _box (Variables|Default|GetBox))
  ;[1 1 1] On Chaos Break Event
  ;;[0.2371 0.3006 1] Add Velocity Field
  (CallFunction|TransientField (Variables|Default|GetFieldSystem) (Variables|Default|GetCullingField) (Variables|Default|GetRadialFalloff) (Variables|Default|GetRadialVector) (Variables|Default|GetDestructionCenter) (Variables|Default|GetSphere))
  ;;[1 0.12 0.2097] Destroy Invisible Collision Box when chaos break happens
  (Utilities|IsValid _box
    (:Is%20Valid
      (Components|DestroyComponent _box)
      ;;[0.214 1 0.2762] Disable Event Tick, change collisoin type
      (Variables|Default|SetCanTick true)
      (Collision|SetCollisionObjectType (Variables|Default|GetGC_SM_MERGED_StaticMeshActor_101) "ECC_GameTraceChannel2")
      ;;[0.237 1 0.9402] Chaos Destructible Optimization
      (Utilities|FlowControl|Delay 1e+01)
      (Physics|SetSimulatePhysics (Variables|Default|GetGC_SM_MERGED_StaticMeshActor_101) false)
      (Collision|SetCollisionEnabled (Variables|Default|GetGC_SM_MERGED_StaticMeshActor_101) "NoCollision")
      (Collision|SetCollisionObjectType (Variables|Default|GetGC_SM_MERGED_StaticMeshActor_101) "ECC_GameTraceChannel2")
      (Physics|SetSimulatePhysics (Variables|Default|GetGC_SM_MERGED_StaticMeshActor_102) false)
      (Collision|SetCollisionEnabled (Variables|Default|GetGC_SM_MERGED_StaticMeshActor_102) "NoCollision")
      (if (== (Math|Random|RandomIntegerinRange 0 1) 0)
        (Actor|DestroyActor)))))

(event OnChaosBreakEvent(GC_SM_MERGED_StaticMeshActor_101)
  (params (BreakEvent :type Chaos%20Break%20Event%20Structure%20%28by%20ref%29))
  (bind _box (Variables|Default|GetBox))
  ;[1 1 1] On Chaos Break Event
  ;;[0.2371 0.3006 1] Add Velocity Field
  (CallFunction|TransientField (Variables|Default|GetFieldSystem) (Variables|Default|GetCullingField) (Variables|Default|GetRadialFalloff) (Variables|Default|GetRadialVector) (Variables|Default|GetDestructionCenter) (Variables|Default|GetSphere))
  ;;[1 0.12 0.2097] Destroy Invisible Collision Box when chaos break happens
  (Utilities|IsValid _box
    (:Is%20Valid
      (Components|DestroyComponent _box)
      ;;[0.214 1 0.2762] Disable Event Tick, change collisoin type
      (Variables|Default|SetCanTick true)
      (Collision|SetCollisionObjectType (Variables|Default|GetGC_SM_MERGED_StaticMeshActor_101) "ECC_GameTraceChannel2")
      ;;[0.237 1 0.9402] Chaos Destructible Optimization
      (Utilities|FlowControl|Delay 1e+01)
      (Physics|SetSimulatePhysics (Variables|Default|GetGC_SM_MERGED_StaticMeshActor_101) false)
      (Collision|SetCollisionEnabled (Variables|Default|GetGC_SM_MERGED_StaticMeshActor_101) "NoCollision")
      (Collision|SetCollisionObjectType (Variables|Default|GetGC_SM_MERGED_StaticMeshActor_101) "ECC_GameTraceChannel2")
      (Physics|SetSimulatePhysics (Variables|Default|GetGC_SM_MERGED_StaticMeshActor_102) false)
      (Collision|SetCollisionEnabled (Variables|Default|GetGC_SM_MERGED_StaticMeshActor_102) "NoCollision")
      (if (== (Math|Random|RandomIntegerinRange 0 1) 0)
        (Actor|DestroyActor)))))

(event EventTick
  (params (DeltaSeconds :type Float%20%28single-precision%29)))

(fn ConstructionScript)