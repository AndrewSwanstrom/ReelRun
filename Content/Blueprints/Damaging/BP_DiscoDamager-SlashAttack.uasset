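; BP_DiscoDamager-SlashAttack is a slash attack actor that travels in a straight line and removes itself when done.
; On BeginPlay it stores its start location, then a timeline lerps it 2500 units along its forward vector without sweeping, and destroys it on finish.
; The graph holds only this movement, with no damage logic, and the construction script just calls the parent.
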(event EventBeginPlay
  (Variables|Default|SetInitialPosition (Transformation|GetActorLocation))
  (bind _alpha (Timeline|Timeline_0 PlayFromStart)
    (:Update
      (Transformation|SetActorLocation (Math|Vector|Lerp(Vector) (Variables|Default|GetInitialPosition) (+ (Variables|Default|GetInitialPosition) (* (Transformation|GetActorForwardVector) 2.5e+03)) _alpha) false false))
    (:Finished
      (Actor|DestroyActor))))

(fn ConstructionScript
  (|CallParentFunction))