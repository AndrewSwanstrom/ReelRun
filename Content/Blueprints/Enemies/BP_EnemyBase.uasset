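; Base enemy Blueprint that provides AI activation and health-based death.
; ActivateAI starts the BT_BasicEnemy behavior tree on its AI controller; BeginPlay is empty, so activation depends on that event being called.
; AnyDamage subtracts from Health and destroys the actor only once it drops below zero.
; An unconnected AIMoveTo chain toward the BP_Betsy player pawn never runs.
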(event Custom|ActivateAI
  ;[1 1 1] Random Wander
  (AI|RunBehaviorTree (AI|GetAIController self) "/Game/Blueprints/Enemies/BehavioralTree/BT_BasicEnemy.BT_BasicEnemy"))

(event Game|Damage|EventAnyDamage
  (params (Damage :type Float%20%28single-precision%29) (DamageType :type Damage%20Type%20Object%20Reference) (InstigatedBy :type Controller%20Object%20Reference) (DamageCauser :type Actor%20Object%20Reference))
  ;[1 1 1] Damage Enemy
  (bind _output_get (Variables|Default|SetHealth (- (Variables|Default|GetHealth) Damage)))
  (if (< _output_get 0.0)
    (Actor|DestroyActor)))

(event EventBeginPlay)

(fn ConstructionScript)