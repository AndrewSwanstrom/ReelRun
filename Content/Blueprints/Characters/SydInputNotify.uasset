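; SydInputNotify is an animation notify state that locks player input on the BP_Syd character during part of an animation.
; On begin, it casts the mesh owner to BP_Syd and disables its input for player controller 0.
; On end, it re-enables that input, and its comments tie the window to the start and end of a trace.
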(fn ReceivedNotifyBegin
  (params (MeshComp :type Skeletal%20Mesh%20Component%20Object%20Reference) (Animation :type Anim%20Sequence%20Base%20Object%20Reference) (TotalDuration :type Float%20%28single-precision%29) (EventReference :type Anim%20Notify%20Event%20Reference%20Structure%20%28by%20ref%29))
  ;[1 1 1] Disable Movement on Trace Start
  (bind _asbp_syd (Utilities|Casting|CastToBP_Syd (Components|GetOwner MeshComp)))
  (Utilities|IsValid _asbp_syd
    (:Is%20Valid
      (Input|DisableInput _asbp_syd (Game|GetPlayerController _asbp_syd))
      (return false))))

(fn ReceivedNotifyEnd
  (params (MeshComp :type Skeletal%20Mesh%20Component%20Object%20Reference) (Animation :type Anim%20Sequence%20Base%20Object%20Reference) (EventReference :type Anim%20Notify%20Event%20Reference%20Structure%20%28by%20ref%29))
  ;[1 1 1] Enable Player Move on Trace End
  (bind _asbp_syd (Utilities|Casting|CastToBP_Syd (Components|GetOwner MeshComp)))
  (Utilities|IsValid _asbp_syd
    (:Is%20Valid
      (Input|EnableInput _asbp_syd (Game|GetPlayerController _asbp_syd))
      (return true))))