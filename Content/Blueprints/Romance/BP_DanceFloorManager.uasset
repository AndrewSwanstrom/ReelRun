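; Dance floor manager that builds a grid of tiles and plays telegraphed circle attacks on it.
; The construction script fills GridBounds with TileSize-scaled mesh components stored in TileArray.
; The warning event picks a random center tile and sine-flashes WarningColor within the radius; the separately triggered attack grows a TileColor circle from that tile.
; Timelines drive both through distance-based material parameters; overlapping characters are only counted and printed, not damaged.
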(event Custom|FilledCircleAttackWarningFlash
  (params (Speed :type Float%20%28double-precision%29) (Radius :type Float%20%28double-precision%29))
  (Variables|Default|SetSelectedTile (.OutItem (Utilities|Array|Random (Variables|Default|GetTileArray))))
  (Components|Timeline|SetPlayRate (Variables|Default|GetFilledCircleWarningFlashTimeline) (/ 1.0 Speed))
  ;[1 1 1] Warning Flash Filled Circle
  (Timeline|FilledCircleWarningFlashTimeline PlayFromStart
    (:Update
      (for _array_element (Variables|Default|GetTileArray)
        (Variables|Default|SetArray%20Element _array_element)
        (Rendering|Material|SetVectorParameterValueonMaterials (Variables|Default|GetArray%20Element) "WarningColor" (Math|Vector|MakeVector (* (Math|Conversions|ToFloat(Integer) (Math|Float|Ceil (Math|Float|MapRangeClamped (Math|Vector|Distance(Vector) (Variables|/Script/Engine.SceneComponent|GetRelativeLocation _array_element) (Variables|/Script/Engine.SceneComponent|GetRelativeLocation (Variables|Default|GetSelectedTile))) Radius 0.0 0.0 1.0))) (Math|Trig|Sin(Radians) (* (Utilities|Time|GetTimeSeconds) (* (Utilities|Time|GetWorldDeltaSeconds) 2e+03)))) 0.0 0.0))))
    (:Finished
      (for _array_element_2 (Variables|Default|GetTileArray)
        (Rendering|Material|SetVectorParameterValueonMaterials _array_element_2 "WarningColor" (Math|Vector|MakeVector 0.0 0.0 0.0))))))

(event Custom|FilledCircleAttack
  (params (Speed :type Float%20%28double-precision%29) (Radius :type Float%20%28double-precision%29))
  (Components|Timeline|SetPlayRate (Variables|Default|GetFilledCircleTimeline) (/ 1.0 Speed))
  ;[1 1 1] Light up in filled circle
  (bind _alpha (Timeline|FilledCircleTimeline PlayFromStart)
    (:Update
      (Variables|Default|SetCurrentRadius (* Radius _alpha))
      (for _array_element (Variables|Default|GetTileArray)
        (Variables|Default|SetArray%20Element _array_element)
        (Rendering|Material|SetVectorParameterValueonMaterials (Variables|Default|GetArray%20Element) "TileColor" (Math|Vector|MakeVector (Math|Conversions|ToFloat(Integer) (Math|Float|Ceil (Math|Float|MapRangeClamped (Math|Vector|Distance(Vector) (Variables|/Script/Engine.SceneComponent|GetRelativeLocation _array_element) (Variables|/Script/Engine.SceneComponent|GetRelativeLocation (Variables|Default|GetSelectedTile))) (Variables|Default|GetCurrentRadius) 0.0 0.0 1.0))) 0.0 0.0))
        (Development|PrintString (Utilities|String|ToString(Integer) (Utilities|Array|Length (Collision|GetOverlappingActors (Variables|Default|GetArray%20Element) "/Game/Blueprints/Characters/Base_Character.Base_Character_C" :!class /Script/Engine.PrimitiveComponent))))))
    (:Finished
      (for _array_element_2 (Variables|Default|GetTileArray)
        (Rendering|Material|SetVectorParameterValueonMaterials _array_element_2 "TileColor" (Math|Vector|MakeVector 0.0 0.0 0.0))))))

(event EventBeginPlay)

(event EventTick
  (params (DeltaSeconds :type Float%20%28single-precision%29)))

(fn ConstructionScript
  (bind _gridbounds (Variables|Default|GetGridBounds))
  (bind _tilesize (Variables|Default|GetTileSize))
  (bind _tilesize_2 (Variables|Default|GetTileSize))
  (bind _tilesize_3 (Variables|Default|GetTileSize))
  (bind _boxextent (Collision|GetComponentBounds _gridbounds))
  (bind _returnvalue (/ _tilesize_2 2.0))
  (bind _returnvalue_2 (/ _tilesize_3 2.0))
  (bind _returnvalue_3 (/ (.y _boxextent) _returnvalue))
  (bind _returnvalue_4 (/ (.x _boxextent) _returnvalue_2))
  (bind _returnvalue_5 (Math|Float|Floor _returnvalue_3))
  (bind _returnvalue_6 (Math|Float|Floor _returnvalue_4))
  ;[1 1 1] Place Rows
  (for _index (range 1 _returnvalue_6) ; Place each row
    ;[1 1 1] Place Columns
    (for _index_2 (range 1 _returnvalue_5) ; Place each column
      (bind _returnvalue_7 (AddComponent|AddStaticMeshComponent false (Math|Transform|MakeTransform (+ (Transformation|GetActorLocation) (Math|Vector|MakeVector (- (* (- _index 1) (Variables|Default|GetTileSize)) (* (Variables|Default|GetTileSize) (/ (- _returnvalue_6 1) 2))) (- (* (- _index_2 1) (Variables|Default|GetTileSize)) (* (Variables|Default|GetTileSize) (/ (- _returnvalue_5 1) 2))) 0.0)) "0, 0, 0" (Math|Vector|MakeVector _tilesize _tilesize 2e+01))))
      (Utilities|Array|Add (Variables|Default|GetTileArray) _returnvalue_7))))