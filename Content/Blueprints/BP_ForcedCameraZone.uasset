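; BP_ForcedCameraZone is a trigger zone that forces a playable character's camera yaw while they overlap it.
; On begin overlap it switches on the class name for Betsy, Syd or Alley and calls CameraForcedLerpStart with that character's yaw pivot and camera, targeting yaw opposite the zone's forward vector.
; The per-class branches exist because those components are not in Base_Character.
; End overlap calls CameraForcedLerpEnd on any Base_Character.
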(event Collision|EventActorBeginOverlap
  (params (OtherActor :type Actor%20Object%20Reference))
  (bind _returnvalue (Transformation|GetActorForwardVector))
  (bind _self self)
  (bind _returnvalue_2 (Math|Vector|NegateVector _returnvalue))
  (bind _returnvalue_3 (Math|Conversions|RotationFromXVector _returnvalue_2))
  ;[0.1781 0.1207 0] this is gross, one day lets put camera Yaw Pivot and Camera in Base Character
  (switch string (Utilities|GetClassDisplayName (Utilities|GetClass OtherActor))
    (:BP_Betsy_C
      (bind _asbp_betsy (Utilities|Casting|CastToBP_Betsy OtherActor))
      (Default|CameraForcedLerpStart _asbp_betsy (Variables|/Game/Blueprints/Characters/BP_Betsy.BP_Betsy_C|GetCameraYawPivot _asbp_betsy) (.yaw _returnvalue_3) _self (Variables|/Game/Blueprints/Characters/BP_Betsy.BP_Betsy_C|GetCamera_0 _asbp_betsy)))
    (:BP_Syd_C
      (bind _asbp_syd (Utilities|Casting|CastToBP_Syd OtherActor))
      (Default|CameraForcedLerpStart _asbp_syd (Variables|/Game/Blueprints/Characters/BP_Syd.BP_Syd_C|GetCameraYawPivot1 _asbp_syd) (.yaw _returnvalue_3) _self (Variables|/Game/Blueprints/Characters/BP_Syd.BP_Syd_C|GetCamera1 _asbp_syd)))
    (:BP_Alley_C
      (bind _asbp_alley (Utilities|Casting|CastToBP_Alley OtherActor))
      (Default|CameraForcedLerpStart _asbp_alley (Variables|/Game/Blueprints/Characters/BP_Alley.BP_Alley_C|GetCameraYawPivot1 _asbp_alley) (.yaw _returnvalue_3) _self (Variables|/Game/Blueprints/Characters/BP_Alley.BP_Alley_C|GetCamera1 _asbp_alley)))))

(event Collision|EventActorEndOverlap
  (params (OtherActor :type Actor%20Object%20Reference))
  ;[0.1781 0.1207 0] this is gross, one day lets put camera Yaw Pivot and Camera in Base Character
  (bind _asbase_character (Utilities|Casting|CastToBase_Character OtherActor))
  (Default|CameraForcedLerpEnd _asbase_character))

(fn ConstructionScript)