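; AlleyFootTraceNotify is an animation notify state that marks the attack trace window in BP_Alley's animations.
; On begin it casts the mesh owner to BP_Alley and sets FistActive true, and on end it sets it back to false.
; Despite the Foot name, it toggles the FistActive flag and performs no trace itself.
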(fn ReceivedNotifyBegin
  (params (MeshComp :type Skeletal%20Mesh%20Component%20Object%20Reference) (Animation :type Anim%20Sequence%20Base%20Object%20Reference) (TotalDuration :type Float%20%28single-precision%29) (EventReference :type Anim%20Notify%20Event%20Reference%20Structure%20%28by%20ref%29))
  ;[1 1 1] Start Attack Trace
  (bind _asbp_alley (Utilities|Casting|CastToBP_Alley (Components|GetOwner MeshComp)))
  (Utilities|IsValid _asbp_alley
    (:Is%20Valid
      (Variables|/Game/Blueprints/Characters/Base_Character.Base_Character_C|SetFistActive _asbp_alley true)
      (return true))))

(fn ReceivedNotifyEnd
  (params (MeshComp :type Skeletal%20Mesh%20Component%20Object%20Reference) (Animation :type Anim%20Sequence%20Base%20Object%20Reference) (EventReference :type Anim%20Notify%20Event%20Reference%20Structure%20%28by%20ref%29))
  ;[1 1 1] Stop Attack Trace
  (bind _asbp_alley (Utilities|Casting|CastToBP_Alley (Components|GetOwner MeshComp)))
  (Utilities|IsValid _asbp_alley
    (:Is%20Valid
      (Variables|/Game/Blueprints/Characters/BP_Betsy.BP_Betsy_C|SetFistActive _asbp_alley false)
      (return true))))