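; Base player character Blueprint that tracks nearby interactable objects and plays a dash effect.
; InteractCollider overlaps store the latest IInteractable actor in a single Interactable slot and call its CanInteractMessage.
; Any interactable leaving the collider calls StopInteractMessage on the stored one and clears the slot.
; Left Shift only spawns the NS_Dash Niagara effect on the mesh; dash movement and interact input are absent here.
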(event OnComponentBeginOverlap(InteractCollider)
  (params (OverlappedComponent :type Primitive%20Component%20Object%20Reference) (OtherActor :type Actor%20Object%20Reference) (OtherComp :type Primitive%20Component%20Object%20Reference) (OtherBodyIndex :type Integer) (bFromSweep :type Boolean) (SweepResult :type Hit%20Result%20Structure%20%28by%20ref%29))
  (if (Utilities|DoesObjectImplementInterface OtherActor "/Game/Blueprints/Interactions/IInteractable.IInteractable_C")
    (bind _output_get (Variables|Default|SetInteractable OtherActor))
    (Class|IInteractable|CanInteract(Message) _output_get)))

(event OnComponentEndOverlap(InteractCollider)
  (params (OverlappedComponent :type Primitive%20Component%20Object%20Reference) (OtherActor :type Actor%20Object%20Reference) (OtherComp :type Primitive%20Component%20Object%20Reference) (OtherBodyIndex :type Integer))
  (if (Utilities|DoesObjectImplementInterface OtherActor "/Game/Blueprints/Interactions/IInteractable.IInteractable_C")
    (Utilities|IsValid (Variables|Default|GetInteractable)
      (:Is%20Valid
        (Class|IInteractable|StopInteract(Message) (Variables|Default|GetInteractable))
        (Variables|Default|SetInteractable 0)))))

(event EventBeginPlay)

(event Collision|EventActorBeginOverlap
  (params (OtherActor :type Actor%20Object%20Reference)))

(event EventTick
  (params (DeltaSeconds :type Float%20%28single-precision%29)))

(event Input|KeyboardEvents|LeftShift
  (params (Key :type Key%20Structure :default "None"))
  (:Pressed
    (Niagara|SpawnSystemAttached "/Game/Art/VFX/NS_Dash.NS_Dash" (Variables|Character|GetMesh) "None" "0, 0, 0" "0, 0, 0" "KeepRelativeOffset" false)))

(fn ConstructionScript)