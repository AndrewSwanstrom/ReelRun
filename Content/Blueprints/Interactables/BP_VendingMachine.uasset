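; BP_VendingMachine is an interactable that dispenses a throwable snack when the interact action fires while InRange is set.
; Its box overlaps call shared begin/end handlers with the interact icon and overlay mesh.
; Interacting plays a door sequence, spawns a BP_SnackThrowable at the spawn point and assigns it a random snack mesh.
; It counts spawns, but the limit check and snack cleanup are disconnected, so dispensing is uncapped.
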(event OnComponentBeginOverlap(Box1)
  (params (OverlappedComponent :type Primitive%20Component%20Object%20Reference) (OtherActor :type Actor%20Object%20Reference) (OtherComp :type Primitive%20Component%20Object%20Reference) (OtherBodyIndex :type Integer) (bFromSweep :type Boolean) (SweepResult :type Hit%20Result%20Structure%20%28by%20ref%29))
  (CallFunction|BeginColliderOverlap OtherActor (Variables|Default|GetInteractIcon) (Variables|Default|GetOverlayMesh)))

(event OnComponentEndOverlap(Box1)
  (params (OverlappedComponent :type Primitive%20Component%20Object%20Reference) (OtherActor :type Actor%20Object%20Reference) (OtherComp :type Primitive%20Component%20Object%20Reference) (OtherBodyIndex :type Integer))
  (CallFunction|EndColliderOverlap OtherActor (Variables|Default|GetInteractIcon) (Variables|Default|GetOverlayMesh)))

(event EventInteractAction
  (bind _spawnpoint (Variables|Default|GetSpawnPoint))
  (bind _returnvalue (Transformation|GetWorldTransform _spawnpoint))
  (if (Variables|Default|GetbInRange)
    (if true
      (Class|ActorSequenceComponent|PlaySequence (Variables|Default|GetDoorSequence))
      (bind _returnvalue_2 (Game|SpawnActorfromClass "/Game/Blueprints/Throwables/BP_SnackThrowable.BP_SnackThrowable_C" (Math|Transform|MakeTransform (.location _returnvalue) (.rotation _returnvalue) "1.000000,1.000000,1.000000") "Undefined" "MultiplyWithRoot" 0 0))
      (bind _output_get (Variables|Default|SetSpawnedSnack _returnvalue_2))
      (Default|SetSnackMesh _output_get (.OutItem (Utilities|Array|Random (Variables|Default|GetArrayOfSnacks))))
      (bind _result (Math|Integer|IncrementInt (Variables|Default|GetSpawnedCount))
        (:%20%20
          (Variables|Default|SetSpawnedCount _result))))))

(event EventBeginPlay
  (Variables|Default|SetSpawnedCount 0))

(fn ConstructionScript
  (|CallParentFunction))