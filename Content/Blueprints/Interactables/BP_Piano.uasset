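; Interactable piano that plays a randomly pitched key on Interact while overlapped, showing an icon and outline in range.
; When the game mode's default pawn is BP_Syd, interacting smashes it with a burst of key and wood-break sounds, moves the trigger far below and strains the Geometry Collection.
; The Chaos break event applies a culled radial velocity field, then freezes the debris and disables its collision after a delay.
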(event OnChaosBreakEvent(gc_piano)
  (params (BreakEvent :type Chaos%20Break%20Event%20Structure%20%28by%20ref%29))
  (bind _box (Variables|Default|GetBox))
  (CallFunction|TransientField (Variables|Default|GetFieldSystem) (Variables|Default|GetCullingField) (Variables|Default|GetRadialFalloff) (Variables|Default|GetRadialVector) (+ (Transformation|GetWorldLocation (Variables|Default|Getgc_piano)) "0.000000,0.000000,150.000000") (Variables|Default|GetSphere))
  (Utilities|IsValid _box
    (:Is%20Valid
      (Components|DestroyComponent _box)
      (Variables|Default|SetCanTick true)
      (Collision|SetCollisionObjectType (Variables|Default|Getgc_piano) "ECC_GameTraceChannel2")
      (Utilities|FlowControl|Delay 15.0)
      (Physics|SetSimulatePhysics (Variables|Default|Getgc_piano) false)
      (Collision|SetCollisionEnabled (Variables|Default|Getgc_piano) "NoCollision"))))

(event OnComponentBeginOverlap(Box1)
  (params (OverlappedComponent :type Primitive%20Component%20Object%20Reference) (OtherActor :type Actor%20Object%20Reference) (OtherComp :type Primitive%20Component%20Object%20Reference) (OtherBodyIndex :type Integer) (bFromSweep :type Boolean) (SweepResult :type Hit%20Result%20Structure%20%28by%20ref%29))
  (Variables|Default|SetbInRange true)
  (Rendering|SetVisibility (Variables|Default|GetInteractIcon) true false)
  (Rendering|Material|SetOverlayMaterial (Variables|Default|GetStaticMesh) "/Game/Materials/OutlineMat/Mi_OutlineMat_Inst.Mi_OutlineMat_Inst" :!class /Script/Engine.MeshComponent)
  (Input|EnableInput (Game|GetPlayerController 0)))

(event OnComponentEndOverlap(Box1)
  (params (OverlappedComponent :type Primitive%20Component%20Object%20Reference) (OtherActor :type Actor%20Object%20Reference) (OtherComp :type Primitive%20Component%20Object%20Reference) (OtherBodyIndex :type Integer))
  (Variables|Default|SetbInRange false)
  (Rendering|SetVisibility (Variables|Default|GetInteractIcon) false false)
  (Rendering|Material|SetOverlayMaterial (Variables|Default|GetStaticMesh) 0 :!class /Script/Engine.MeshComponent)
  (Input|DisableInput (Game|GetPlayerController 0) 0))

(event Custom|Transient_Field
  (params (Field%20System :type Field%20System%20Component%20Object%20Reference) (Culling%20Field :type Culling%20Field%20Object%20Reference) (Radial%20Fall%20Off :type Radial%20Falloff%20Object%20Reference) (Radial%20Vector :type Radial%20Vector%20Object%20Reference) (Center%20Position :type Vector) (Sphere :type Sphere%20Component%20Object%20Reference))
  (Class|FieldSystemComponent|ApplyPhysicsField Field%20System true "Field_LinearVelocity" 0 (Field|SetCullingField Culling%20Field (Field|SetRadialFalloff Radial%20Fall%20Off 1.0 0.0 1.0 0.0 (Components|Sphere|GetScaledSphereRadius Sphere) (Transformation|GetWorldLocation Sphere) "Field_FallOff_None") (Field|SetRadialVector Radial%20Vector 15.0 Center%20Position) "Field_Culling_Outside")))

(event Custom|oh%20no%20our%20piano%20its%20broken
  (Physics|SetSimulatePhysics (Variables|Default|Getgc_piano) true)
  (for _index (range 0 10)
    (Audio|PlaySoundatLocation "/Game/Art/SFX/InGame/SW_PianoKey.SW_PianoKey" "0, 0, 0" "0, 0, 0" 2.0 (Math|Random|RandomFloatinRange 0.1 1.5) 0.0 0 0 0 0))
  (Audio|PlaySoundatLocation "/Game/Art/SFX/InGame/ER_WoodBreaking.ER_WoodBreaking" "0, 0, 0" "0, 0, 0" 0.75 (Math|Random|RandomFloatinRange 0.1 1.5) 0.0 0 0 0 0)
  (Transformation|SetWorldLocation (Variables|Default|GetBox1) "0.000000,0.000000,-99999.000000" false false)
  (Class|GeometryCollectionComponent|ApplyInternalStrain (Variables|Default|Getgc_piano) 0 (Transformation|GetWorldLocation (Variables|Default|Getgc_piano)) 1e+02 0 1.0 1e+07))

(event Input|EnhancedActionEvents|EnhancedInputActionIA_Interact
  (params (ActionValue :type Boolean) (ElapsedSeconds :type Float%20%28double-precision%29) (TriggeredSeconds :type Float%20%28double-precision%29) (InputAction :type Input%20Action%20Object%20Reference :default "/Game/Blueprints/Input/Actions/IA_Interact.IA_Interact"))
  (if (Variables|Default|GetbInRange)
    (Audio|PlaySoundatLocation "/Game/Art/SFX/InGame/SW_PianoKey.SW_PianoKey" "0, 0, 0" "0, 0, 0" 1.0 (Math|Random|RandomFloatinRange 0.1 1.5) 0.0 0 0 0 0)
    (if (== (Variables|/Script/Engine.GameModeBase|GetDefaultPawnClass (Game|GetGameMode)) "/Game/Blueprints/Characters/BP_Syd.BP_Syd_C")
      (CallFunction|OhNoOurPianoItsBroken))))

(fn ConstructionScript)