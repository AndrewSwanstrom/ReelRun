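; BP_SandbagShooterEnemy is an enemy that turns to face the player and periodically fires BP_Damager projectiles.
; Each Tick it snaps its yaw toward player character 0, keeping pitch and roll level.
; A real-time cooldown check on Tick gates firing, so low frame rates can limit the fire rate.
; Each shot spawns a damager ahead of and slightly above the enemy, then launches its collider with a forward velocity-change impulse.
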(event EventTick
  (params (DeltaSeconds :type Float%20%28single-precision%29))
  (bind _self self)
  (bind _returnvalue (Transformation|GetActorTransform _self))
  (Transformation|SetActorRotation (Math|Rotator|MakeRotator 0.0 0.0 (.yaw (Math|Rotator|FindLookatRotation (Transformation|GetActorLocation) (Transformation|GetActorLocation (Game|GetPlayerCharacter 0))))))
  (if (> (- (Utilities|Time|GetRealTimeSeconds) (Variables|Default|GetShootTimer)) (Variables|Default|GetShootCooldown))
    (Variables|Default|SetShootTimer (Utilities|Time|GetRealTimeSeconds))
    (bind _returnvalue_2 (Game|SpawnActorfromClass "/Game/Blueprints/Damaging/BP_Damager.BP_Damager_C" (Math|Transform|MakeTransform (+ (+ (* (Transformation|GetActorForwardVector _self) 3e+02) (.location _returnvalue)) "0.000000,0.000000,50.000000") (.rotation _returnvalue) (.scale _returnvalue)) "Undefined" "MultiplyWithRoot" 0 0))
    (Physics|AddImpulse (Variables|/Game/Blueprints/Damaging/BP_Damager.BP_Damager_C|GetCollider _returnvalue_2) (* (Transformation|GetActorForwardVector) 1e+03) "None" true)))

(fn ConstructionScript)