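; Enemy spawn point actor that spawns its configured enemy class at its own transform, adjusting for collision but always spawning.
; The Spawn function returns the new actor and optionally attaches it to the spawn point's parent, the current wave, for the level Blueprint.
; The optional attach keeps the romance content working with the old sequencer.
; The older SpawnEnemy event always attaches and is marked as superseded by Spawn.
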(event Custom|SpawnEnemy
  ;[1 1 1] old, consider using Spawn function instead
  (bind _returnvalue (Game|SpawnActorfromClass (Variables|Default|GetSpawnActorClass) (Transformation|GetActorTransform) "AdjustIfPossibleButAlwaysSpawn" "MultiplyWithRoot" 0 0))
  (Transformation|AttachActorToActor _returnvalue (Actor|GetAttachParentActor self) "None" "KeepWorld" "KeepWorld" "KeepWorld" false))

(fn ConstructionScript)

(fn Spawn
  (params (SpawnPreAttached :type Boolean))
  (bind _returnvalue (Game|SpawnActorfromClass (Variables|Default|GetSpawnActorClass) (Transformation|GetActorTransform) "AdjustIfPossibleButAlwaysSpawn" "MultiplyWithRoot" 0 0))
  (if SpawnPreAttached ; romance uses old sequencer, this allows romance to still work
    (Transformation|AttachActorToActor _returnvalue (Actor|GetAttachParentActor self) "None" "KeepWorld" "KeepWorld" "KeepWorld" false))
  (return _returnvalue))