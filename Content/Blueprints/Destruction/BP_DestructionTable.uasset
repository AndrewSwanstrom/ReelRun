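; Destructible table prop built from five Chaos geometry collection pieces, each paired with a box collision component.
; When a piece breaks, it switches to a different collision object type and destroys its box.
; Every tick, the remaining boxes lose collision while the BP_Betsy player pawn is invulnerable and regain it otherwise.
; Delayed destruction of the broken pieces is present but unconnected.
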(event OnChaosBreakEvent(GC_SM_MERGED_StaticMeshActor_118)
  (params (BreakEvent :type Chaos%20Break%20Event%20Structure%20%28by%20ref%29))
  (bind _box4 (Variables|Default|GetBox4))
  (Collision|SetCollisionObjectType (Variables|Default|GetGC_SM_MERGED_StaticMeshActor_118) "ECC_GameTraceChannel2")
  (Utilities|IsValid _box4
    (:Is%20Valid
      (Components|DestroyComponent _box4))))

(event OnChaosBreakEvent(GC_SM_MERGED_StaticMeshActor_116)
  (params (BreakEvent :type Chaos%20Break%20Event%20Structure%20%28by%20ref%29))
  (Collision|SetCollisionObjectType (Variables|Default|GetGC_SM_MERGED_StaticMeshActor_116) "ECC_GameTraceChannel2")
  (Utilities|IsValid (Variables|Default|GetBox1)
    (:Is%20Valid
      (Components|DestroyComponent (Variables|Default|GetBox1)))))

(event OnChaosBreakEvent(GC_SM_Table11)
  (params (BreakEvent :type Chaos%20Break%20Event%20Structure%20%28by%20ref%29))
  (bind _box (Variables|Default|GetBox))
  (Collision|SetCollisionObjectType (Variables|Default|GetGC_SM_Table11) "ECC_GameTraceChannel2")
  (Utilities|IsValid _box
    (:Is%20Valid
      (Components|DestroyComponent _box))))

(event OnChaosBreakEvent(GC_SM_MERGED_StaticMeshActor_117)
  (params (BreakEvent :type Chaos%20Break%20Event%20Structure%20%28by%20ref%29))
  (Collision|SetCollisionObjectType (Variables|Default|GetGC_SM_MERGED_StaticMeshActor_117) "ECC_GameTraceChannel2")
  (Utilities|IsValid (Variables|Default|GetBox2)
    (:Is%20Valid
      (Components|DestroyComponent (Variables|Default|GetBox2)))))

(event OnChaosBreakEvent(GC_SM_MERGED_StaticMeshActor_115)
  (params (BreakEvent :type Chaos%20Break%20Event%20Structure%20%28by%20ref%29))
  (Collision|SetCollisionObjectType (Variables|Default|GetGC_SM_MERGED_StaticMeshActor_115) "ECC_GameTraceChannel2")
  (Utilities|IsValid (Variables|Default|GetBox3)
    (:Is%20Valid
      (Components|DestroyComponent (Variables|Default|GetBox3)))))

(event EventTick
  (params (DeltaSeconds :type Float%20%28single-precision%29))
  (bind _asbp_betsy (Utilities|Casting|CastToBP_Betsy (Game|Player|GetPlayerPawn 0)))
  (if (Variables|/Game/Blueprints/Characters/BP_Betsy.BP_Betsy_C|GetInvulnerable _asbp_betsy)
    (for _array_element (Variables|Default|GetBoxCollisions)
      (Utilities|IsValid _array_element
        (:Is%20Valid
          (Collision|SetCollisionEnabled _array_element "NoCollision"))))
    (else
      (for _array_element_2 (Variables|Default|GetBoxCollisions)
        (Utilities|IsValid _array_element_2
          (:Is%20Valid
            (Collision|SetCollisionEnabled _array_element_2 "QueryAndPhysics")))))))

(event EventBeginPlay
  (Utilities|Array|Add (Variables|Default|GetBoxCollisions) (Variables|Default|GetBox))
  (Utilities|Array|Add (Variables|Default|GetBoxCollisions) (Variables|Default|GetBox1))
  (Utilities|Array|Add (Variables|Default|GetBoxCollisions) (Variables|Default|GetBox2))
  (Utilities|Array|Add (Variables|Default|GetBoxCollisions) (Variables|Default|GetBox3))
  (Utilities|Array|Add (Variables|Default|GetBoxCollisions) (Variables|Default|GetBox4)))

(fn ConstructionScript)