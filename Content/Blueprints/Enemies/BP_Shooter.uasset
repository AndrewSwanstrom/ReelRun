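; BP_Shooter is a gun-carrying AI enemy that runs a behavior tree, fights the player and destroys itself and its gun when health runs out.
; After sequencer-triggered ActivateAI and a delay, Tick sets the blackboard behavior by player distance, shooting only at mid range.
; Before activation it shoots regardless of range.
; Shots require line of sight and cooldown, launching an impulse-driven BP_Damager with montage and muzzle flash.
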(event Custom|ActivateAI
  ;[1 1 1] triggered by sequencer in level blueprint if there is one
  (AI|Components|Blackboard|SetValueasEnum (AI|GetBlackboard 0) (Utilities|Name|MakeLiteralName "ebehavior") (Utilities|Enum|LiteralenumEnum_ShooterEnemy "NewEnumerator2"))
  ;[1 1 1] bad temporary solution
  (Utilities|FlowControl|Delay 4.0)
  (Variables|Default|Setsequencestarted true))

(event Custom|ShootAnim
  (Animation|PlayAnimMontage "/Game/Art/Characters/Enemies/Shooter/Animations/Sequence/Anim_ShooterEnemy_Attack_Montage.Anim_ShooterEnemy_Attack_Montage" 1.0 "None")
  (Utilities|FlowControl|Delay 0.5))

(event Game|Damage|EventAnyDamage
  (params (Damage :type Float%20%28single-precision%29) (DamageType :type Damage%20Type%20Object%20Reference) (InstigatedBy :type Controller%20Object%20Reference) (DamageCauser :type Actor%20Object%20Reference))
  ;[1 1 1] Damage Enemy
  (bind _output_get (Variables|Default|SetHealth (- (Variables|Default|GetHealth) Damage)))
  (if (<= _output_get 0.0)
    (Actor|DestroyActor)
    (Actor|DestroyActor (Variables|Default|GetGunBP_Ref))))

(event EventTick
  (params (DeltaSeconds :type Float%20%28single-precision%29))
  (if (Variables|Default|Getsequencestarted)
    (bind _asbp_betsy (Utilities|Casting|CastToBP_Betsy (Game|Player|GetPlayerPawn 0)))
    (if (< (Math|Vector|Distance(Vector) (Transformation|GetActorLocation _asbp_betsy) (Transformation|GetActorLocation)) 5e+02)
      (AI|Components|Blackboard|SetValueasEnum (AI|GetBlackboard 0) (Utilities|Name|MakeLiteralName "ebehavior") (Utilities|Enum|LiteralenumEnum_ShooterEnemy "NewEnumerator1"))
      (elif (> (Math|Vector|Distance(Vector) (Transformation|GetActorLocation _asbp_betsy) (Transformation|GetActorLocation)) 1.5e+03)
        (AI|Components|Blackboard|SetValueasEnum (AI|GetBlackboard 0) (Utilities|Name|MakeLiteralName "ebehavior") (Utilities|Enum|LiteralenumEnum_ShooterEnemy "NewEnumerator2"))
        (else
          (AI|Components|Blackboard|SetValueasEnum (AI|GetBlackboard 0) (Utilities|Name|MakeLiteralName "ebehavior") (Utilities|Enum|LiteralenumEnum_ShooterEnemy "NewEnumerator0"))
          (CallFunction|ShootatPlayer))))
    (else
      (CallFunction|ShootatPlayer))))

(event EventBeginPlay
  (AI|RunBehaviorTree (AI|GetAIController self) "/Game/Blueprints/Enemies/BehavioralTree/BT_ShooterEnemy.BT_ShooterEnemy")
  ;[1 1 1] AI startup
  (bind _returnvalue (Game|SpawnActorfromClass (Variables|Default|GetHandGunRef) (Transformation|GetSocketTransform (Variables|Character|GetMesh) "Gun" "RTS_World") "Undefined" "MultiplyWithRoot" 0 0))
  (bind _output_get (Variables|Default|SetGunBP_Ref _returnvalue))
  (Transformation|AttachComponentToComponent _output_get (Variables|Character|GetMesh) "Gun" "SnapToTarget" "SnapToTarget" "SnapToTarget" true)
  (Variables|Default|SetShootTimer (Math|Random|RandomFloatinRange 0.0 4.0))
  (AI|Components|Blackboard|SetValueasEnum (AI|GetBlackboard 0) (Utilities|Name|MakeLiteralName "ebehavior") (Utilities|Enum|LiteralenumEnum_ShooterEnemy "NewEnumerator3")))

(fn ConstructionScript)

(fn ShootatPlayer
  (bind _self self)
  (bind _returnvalue (Transformation|GetActorTransform _self))
  (Transformation|SetActorRotation (Math|Rotator|MakeRotator 0.0 0.0 (.yaw (Math|Rotator|FindLookatRotation (Transformation|GetActorLocation) (Transformation|GetActorLocation (Game|GetPlayerCharacter 0))))))
  (bind _outhit (Collision|LineTraceByChannel (+ (Transformation|GetActorLocation) "0.000000,0.000000,100.000000") (Transformation|GetActorLocation (Game|GetPlayerCharacter 0)) "TraceTypeQuery1" false 0 "None" true "(R=1.000000,G=0.000000,B=0.000000,A=1.000000)" "(R=0.000000,G=1.000000,B=0.000000,A=1.000000)" 1.0))
  (if (== (Game|GetPlayerCharacter 0) (.hitactor _outhit)) ; only shoot if the line trace sees player
    (if (> (- (Utilities|Time|GetRealTimeSeconds) (Variables|Default|GetShootTimer)) (Variables|Default|GetShootCooldown))
      (CallFunction|ShootAnim)
      (Variables|Default|SetShootTimer (Utilities|Time|GetRealTimeSeconds))
      (bind _returnvalue_2 (Game|SpawnActorfromClass "/Game/Blueprints/Damaging/BP_Damager.BP_Damager_C" (Math|Transform|MakeTransform (+ (+ (* (Transformation|GetActorForwardVector _self) 1e+02) (.location _returnvalue)) "0.000000,0.000000,50.000000") (.rotation _returnvalue) (.scale _returnvalue)) "Undefined" "MultiplyWithRoot" 0 0))
      (Rendering|SetVisibility (Variables|Default|GetFlash) false false)
      (Niagara|SpawnSystemAttached "/Game/Art/VFX/NS_MuzzleFlash.NS_MuzzleFlash" 0 "None" "0.000000,35.000000,10.000000" "0.000000,45.000000,0.000000" "KeepRelativeOffset" false)
      (bind _asbp_betsy (Utilities|Casting|CastToBP_Betsy (Game|Player|GetPlayerPawn 0)))
      (Physics|AddImpulse (Variables|/Game/Blueprints/Damaging/BP_Damager.BP_Damager_C|GetCollider _returnvalue_2) (* (Math|Vector|GetUnitDirection(Vector) (+ (Transformation|GetActorLocation self) "0.000000,0.000000,50.000000") (Transformation|GetActorLocation _asbp_betsy)) 1e+03) "None" true))))