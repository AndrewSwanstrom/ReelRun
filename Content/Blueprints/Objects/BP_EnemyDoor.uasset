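; BP_EnemyDoor is a door that opens automatically for BaseEnemy actors overlapping its Box trigger.
; A counter tracks enemies inside, so the OpenClose level sequence plays forward on entry and reverses at a slower rate once the last enemy leaves.
; Each change first sets playback to the current frame, so the door reverses from wherever it is rather than jumping.
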(event OnComponentBeginOverlap(Box)
  (params (OverlappedComponent :type Primitive%20Component%20Object%20Reference) (OtherActor :type Actor%20Object%20Reference) (OtherComp :type Primitive%20Component%20Object%20Reference) (OtherBodyIndex :type Integer) (bFromSweep :type Boolean) (SweepResult :type Hit%20Result%20Structure%20%28by%20ref%29))
  (bind _openclose (Variables|Default|GetOpenClose))
  (bind _sequenceplayer (Variables|/Script/ActorSequence.ActorSequenceComponent|GetSequencePlayer _openclose))
  (Utilities|Casting|CastToBaseEnemy OtherActor)
  (Variables|Default|Setinsidecount (+ (Variables|Default|Getinsidecount) 1))
  (Components|Timeline|SetPlaybackPosition _sequenceplayer (Utilities|Struct|MakeMovieSceneSequencePlaybackParams (Utilities|Struct|MakeFrameTime (Utilities|Struct|MakeFrameNumber (.value (.frame (Sequencer|Player|GetCurrentTime _sequenceplayer)))) 0.0) 0.0 "" "(Hours=0,Minutes=0,Seconds=0,Frames=0,bDropFrameFormat=False)" "Frame" "Play"))
  (Components|Timeline|SetPlayRate _sequenceplayer 1.0)
  (Sequencer|Player|Play _sequenceplayer :!class /Script/MovieScene.MovieSceneSequencePlayer))

(event OnComponentEndOverlap(Box)
  (params (OverlappedComponent :type Primitive%20Component%20Object%20Reference) (OtherActor :type Actor%20Object%20Reference) (OtherComp :type Primitive%20Component%20Object%20Reference) (OtherBodyIndex :type Integer))
  (bind _openclose (Variables|Default|GetOpenClose))
  (bind _sequenceplayer (Variables|/Script/ActorSequence.ActorSequenceComponent|GetSequencePlayer _openclose))
  (Utilities|Casting|CastToBaseEnemy OtherActor)
  (Variables|Default|Setinsidecount (+ (Variables|Default|Getinsidecount) -1))
  (if (<= (Variables|Default|Getinsidecount) 0)
    (Variables|Default|Setinsidecount 0)
    (Components|Timeline|SetPlaybackPosition _sequenceplayer (Utilities|Struct|MakeMovieSceneSequencePlaybackParams (Utilities|Struct|MakeFrameTime (Utilities|Struct|MakeFrameNumber (.value (.frame (Sequencer|Player|GetCurrentTime _sequenceplayer)))) 0.0) 0.0 "" "(Hours=0,Minutes=0,Seconds=0,Frames=0,bDropFrameFormat=False)" "Frame" "Play"))
    (Components|Timeline|SetPlayRate _sequenceplayer 0.2)
    (Class|MovieSceneSequencePlayer|PlayReverse _sequenceplayer)))

(fn ConstructionScript)