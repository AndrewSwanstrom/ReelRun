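; BP_EnemyDoorsbad is an actor, named as an enemy door, that tracks how many enemies overlap it.
; On BeginPlay it binds its own actor begin and end overlap events, which raise and lower Insidecount.
; Only actors whose class is exactly BaseEnemy count, so child classes are ignored.
; The graph holds no door movement or other use of the count.
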(event Custom|OnActorBeginOverlap_Event
  (params (OverlappedActor :type Actor%20Object%20Reference) (OtherActor :type Actor%20Object%20Reference))
  (if (== (Utilities|GetClass OtherActor) "/Game/Blueprints/Enemies/Base_Enemy/BaseEnemy.BaseEnemy_C")
    (Variables|Default|Setinsidecount (+ (Variables|Default|Getinsidecount) 1))))

(event Custom|OnActorEndOverlap_Event
  (params (OverlappedActor :type Actor%20Object%20Reference) (OtherActor :type Actor%20Object%20Reference))
  (if (== (Utilities|GetClass OtherActor) "/Game/Blueprints/Enemies/Base_Enemy/BaseEnemy.BaseEnemy_C")
    (Variables|Default|Setinsidecount (+ (Variables|Default|Getinsidecount) -1))))

(event EventBeginPlay
  (EventDispatchers|BindEventtoOnActorBeginOverlap (delegate Custom|OnActorBeginOverlap_Event))
  (EventDispatchers|BindEventtoOnActorEndOverlap (delegate Custom|OnActorEndOverlap_Event)))

(fn ConstructionScript)