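; Candle cluster prop with a configurable number of visible candles, set up entirely in the construction script.
; When SpawnLight is true, CandleCount (1 to 4) reveals candles cumulatively: tall, small, medium, then a second small.
; Each candle mesh toggles with its paired material billboard; despite the flag's name, no light component is touched.
; With SpawnLight false or another count, visibility keeps its component defaults; the event graph is unused.
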(event EventBeginPlay)

(event Collision|EventActorBeginOverlap
  (params (OtherActor :type Actor%20Object%20Reference)))

(event EventTick
  (params (DeltaSeconds :type Float%20%28single-precision%29)))

(fn ConstructionScript
  (bind _sm_lightfixtures_01a_tall_candle_low (Variables|Default|GetSM_LightFixtures_01a_Tall_Candle_low))
  (if (Variables|Default|GetSpawn%20Light?)
    (switch int (Variables|Default|GetCandle%20Count)
      (:1
        (Rendering|SetVisibility _sm_lightfixtures_01a_tall_candle_low true false)
        (Rendering|SetVisibility (Variables|Default|GetSM_LightFixtures_01a_Small_Candle_low) false false)
        (Rendering|SetVisibility (Variables|Default|GetSM_LightFixtures_01a_Medium_Candle_low) false false)
        (Rendering|SetVisibility (Variables|Default|GetSM_LightFixtures_01a_Small_Candle_low1) false false))
      (:2
        (Rendering|SetVisibility _sm_lightfixtures_01a_tall_candle_low true false)
        (Rendering|SetVisibility (Variables|Default|GetSM_LightFixtures_01a_Small_Candle_low) true false)
        (Rendering|SetVisibility (Variables|Default|GetSM_LightFixtures_01a_Medium_Candle_low) false false)
        (Rendering|SetVisibility (Variables|Default|GetSM_LightFixtures_01a_Small_Candle_low1) false false))
      (:3
        (Rendering|SetVisibility _sm_lightfixtures_01a_tall_candle_low true false)
        (Rendering|SetVisibility (Variables|Default|GetSM_LightFixtures_01a_Small_Candle_low) true false)
        (Rendering|SetVisibility (Variables|Default|GetSM_LightFixtures_01a_Medium_Candle_low) true false)
        (Rendering|SetVisibility (Variables|Default|GetSM_LightFixtures_01a_Small_Candle_low1) false false))
      (:4
        (Rendering|SetVisibility _sm_lightfixtures_01a_tall_candle_low true false)
        (Rendering|SetVisibility (Variables|Default|GetSM_LightFixtures_01a_Small_Candle_low) true false)
        (Rendering|SetVisibility (Variables|Default|GetSM_LightFixtures_01a_Medium_Candle_low) true false)
        (Rendering|SetVisibility (Variables|Default|GetSM_LightFixtures_01a_Small_Candle_low1) true false)))))