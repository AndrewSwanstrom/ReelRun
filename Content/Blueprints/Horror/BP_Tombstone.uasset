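; Horror tombstone prop that randomizes its appearance on BeginPlay from base, body, top and plate static mesh components.
; It applies a slight random tilt to the base, then either removes the plate and keeps the other default meshes, or randomizes the stone.
; Nested random switches swap meshes or remove pieces, with a rarer variant repositioning body and top.
; Removing the body also removes the top.
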(event EventBeginPlay
  (bind _sm_ctop_01 (Variables|Default|GetSM_CTop_01))
  (bind _sm_cbody_02 (Variables|Default|GetSM_CBody_02))
  (bind _sm_cbase_01 (Variables|Default|GetSM_CBase_01))
  (bind _sm_cbody_02_2 (Variables|Default|GetSM_CBody_02))
  (bind _sm_ctop_01_2 (Variables|Default|GetSM_CTop_01))
  (Utilities|FlowControl|DoOnce false
    (:Completed
      (Transformation|SetRelativeRotation (Variables|Default|GetSM_CBase_01) (Math|Rotator|MakeRotator (Math|Conversions|ToFloat(Integer) (Math|Random|RandomIntegerinRange -5 5)) (Math|Conversions|ToFloat(Integer) (Math|Random|RandomIntegerinRange -5 5)) (+ (Math|Conversions|ToFloat(Integer) (Math|Random|RandomIntegerinRange -5 5)) 9e+01)) false false)
      (switch int (Math|Random|RandomIntegerinRange 0 2)
        (:0
          (switch int (Math|Random|RandomIntegerinRange 0 5) :!label _label
            (:0
              (Utilities|FlowControl|Sequence :!label _label_2
                (:then_0
                  (switch int (Math|Random|RandomIntegerinRange 0 2)
                    (:0
                      (Components|StaticMesh|SetStaticMesh _sm_cbase_01 "/Game/Art/Environment/Horror/Cemetery/Tombstones/SM_CBase_03.SM_CBase_03"))
                    (:1
                      (Components|StaticMesh|SetStaticMesh _sm_cbase_01 "/Game/Art/Environment/Horror/Cemetery/Tombstones/SM_CBase_04.SM_CBase_04"))))
                (:then_1
                  (switch int (Math|Random|RandomIntegerinRange 0 3)
                    (:0
                      (Components|StaticMesh|SetStaticMesh _sm_cbody_02_2 "/Game/Art/Environment/Horror/Cemetery/Tombstones/SM_CBody_03.SM_CBody_03"))
                    (:1
                      (Components|StaticMesh|SetStaticMesh _sm_cbody_02_2 "/Game/Art/Environment/Horror/Cemetery/Tombstones/SM_CBody_04.SM_CBody_04"))
                    (:2
                      (Components|StaticMesh|SetStaticMesh _sm_cbody_02_2 "/Game/Art/Environment/Horror/Cemetery/Tombstones/SM_CBody_05.SM_CBody_05"))
                    (:3
                      (Components|DestroyComponent _sm_cbody_02_2)
                      (Components|DestroyComponent _sm_ctop_01_2 :!label _label_3))))
                (:then_2
                  (Utilities|IsValid (Variables|Default|GetSM_CTop_01)
                    (:Is%20Valid
                      (switch int (Math|Random|RandomIntegerinRange 0 1)
                        (:0
                          (Components|StaticMesh|SetStaticMesh _sm_ctop_01_2 "/Game/Art/Environment/Horror/Cemetery/Tombstones/SM_CTop_02.SM_CTop_02"))
                        (:1
                          (goto _label_3))))))))
            (:1
              (goto _label_2))
            (:2
              (goto _label_2))
            (:3
              (goto _label_2))
            (:4
              (goto _label_2))
            (:5
              (Components|StaticMesh|SetStaticMesh (Variables|Default|GetSM_CBase_01) "/Game/Art/Environment/Horror/Cemetery/Tombstones/SM_CBase_02.SM_CBase_02")
              (Components|StaticMesh|SetStaticMesh _sm_cbody_02 "/Game/Art/Environment/Horror/Cemetery/Tombstones/SM_CBody_01.SM_CBody_01")
              (Transformation|SetRelativeLocation _sm_cbody_02 "0.000000,0.000000,6.000000" false false)
              (Transformation|SetRelativeLocation _sm_ctop_01 "0.000000,0.000000,50.000000" false false)
              (switch int (Math|Random|RandomIntegerinRange 0 2)
                (:0
                  (Components|StaticMesh|SetStaticMesh _sm_ctop_01 "/Game/Art/Environment/Horror/Cemetery/Tombstones/SM_CTop_02.SM_CTop_02"))
                (:1
                  (Components|DestroyComponent _sm_ctop_01))))))
        (:1
          (Components|DestroyComponent (Variables|Default|GetSM_CPlate_01)))
        (:2
          (goto _label))))))

(fn ConstructionScript)