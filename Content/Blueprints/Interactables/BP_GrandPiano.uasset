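; Interactable grand piano that plays a key sound at a random pitch when the player interacts within range.
; Overlapping Box1 sets InRange, shows the interact icon, applies an outline overlay material and enables input.
; Ending the overlap reverses these, calling DisableInput through the player controller.
; BeginPlay fills WhiteKeys and BlackKeys arrays, which the sound logic does not use.
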(event OnComponentBeginOverlap(Box1)
  (params (OverlappedComponent :type Primitive%20Component%20Object%20Reference) (OtherActor :type Actor%20Object%20Reference) (OtherComp :type Primitive%20Component%20Object%20Reference) (OtherBodyIndex :type Integer) (bFromSweep :type Boolean) (SweepResult :type Hit%20Result%20Structure%20%28by%20ref%29))
  (Variables|Default|SetbInRange true)
  (Rendering|SetVisibility (Variables|Default|GetInteractIcon) true false)
  (Rendering|Material|SetOverlayMaterial (Variables|Default|GetStaticMesh) "/Game/Materials/OutlineMat/Mi_OutlineMat_Inst.Mi_OutlineMat_Inst" :!class /Script/Engine.MeshComponent)
  (Input|EnableInput (Game|GetPlayerController 0)))

(event OnComponentEndOverlap(Box1)
  (params (OverlappedComponent :type Primitive%20Component%20Object%20Reference) (OtherActor :type Actor%20Object%20Reference) (OtherComp :type Primitive%20Component%20Object%20Reference) (OtherBodyIndex :type Integer))
  (Variables|Default|SetbInRange false)
  (Rendering|SetVisibility (Variables|Default|GetInteractIcon) false false)
  (Rendering|Material|SetOverlayMaterial (Variables|Default|GetStaticMesh) 0 :!class /Script/Engine.MeshComponent)
  (Input|DisableInput (Game|GetPlayerController 0) 0))

(event EventInteractAction
  (if (Variables|Default|GetbInRange)
    (Audio|PlaySoundatLocation "/Game/Art/SFX/InGame/SW_PianoKey.SW_PianoKey" "0, 0, 0" "0, 0, 0" 1.0 (Math|Random|RandomFloatinRange 0.1 1.5) 0.0 0 0 0 0)))

(event EventBeginPlay
  (Utilities|Array|Add (Variables|Default|GetWhiteKeys) 0)
  (Utilities|Array|Add (Variables|Default|GetBlackKeys) 0))

(fn ConstructionScript)