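; Horror boss enemy Blueprint that provides attack and aim-warning events, triggered from outside these graphs.
; SuperAttack spawns a ground slash at the boss's transform, while NormalAttackShot calls Bullet.
; TurnOnLaser sets the laser's color and AimWarning animates its red channel through a timeline.
; A copied base-enemy shot event, uncalled here, launches a damager from the gun socket toward the player with sound and muzzle flash.
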(event EventBeginPlay
  (|CallParentFunction) ; This node is disabled and will not be called.\nDrag off pins to build functionality.
)

(event Collision|EventActorBeginOverlap
  (params (OtherActor :type Actor%20Object%20Reference))
  (|CallParentFunction OtherActor) ; This node is disabled and will not be called.\nDrag off pins to build functionality.
)

(event EventTick
  (params (DeltaSeconds :type Float%20%28single-precision%29)))

(event Custom|Normal%20Attack%20Shot
  ;[0.4069 0.413 1] normal attack
  (CallFunction|Bullet self 0 (Variables|Character|GetMesh)))

(event Custom|Turn%20On%20Laser
  (Niagara|SetNiagaraVariable(LinearColor) (Variables|Default|GetLaser) "Color" (Utilities|Struct|MakeLinearColor 1.0 0.1 0.1 1.0)))

(event Custom|Aim%20Warning
  (bind _redchannelfloat (Timeline|Timeline PlayFromStart)
    (:Update
      (Niagara|SetNiagaraVariable(LinearColor) (Variables|Default|GetLaser) "Color" (Utilities|Struct|MakeLinearColor _redchannelfloat 0.0 0.0 1.0)))))

(event Custom|Stolen%20Bullet%20Code%20From%20Base%20Enemy
  (params (CharacterRef :type Character%20Object%20Reference) (Flash :type Point%20Light%20Component%20Object%20Reference) (Mesh :type Skeletal%20Mesh%20Component%20Object%20Reference))
  (bind _returnvalue (Transformation|GetSocketLocation Mesh "GunSpawn"))
  (bind _returnvalue_2 (Transformation|GetActorTransform CharacterRef))
  (bind _returnvalue_3 (Game|Player|GetPlayerPawn 0))
  (bind _returnvalue_4 (Transformation|GetActorLocation _returnvalue_3))
  (Collision|LineTraceByChannel _returnvalue _returnvalue_4 "TraceTypeQuery1" false 0 "None" true "(R=1.000000,G=0.000000,B=0.000000,A=1.000000)" "(R=0.000000,G=1.000000,B=0.000000,A=1.000000)" 3.0)
  (bind _returnvalue_5 (Game|SpawnActorfromClass "/Game/Blueprints/Damaging/BP_Damager.BP_Damager_C" (Math|Transform|MakeTransform _returnvalue (.rotation _returnvalue_2) (.scale _returnvalue_2)) "Undefined" "MultiplyWithRoot" 0 0))
  (Audio|PlaySoundatLocation "/Game/Art/SFX/InGame/R_RevolverShots.R_RevolverShots" (Transformation|GetActorLocation CharacterRef) "0, 0, 0" 0.6 1.0 0.0 "/Game/Art/SFX/Attenuations/GunShotAtten.GunShotAtten" 0 0 0)
  (Rendering|SetVisibility Flash false false)
  (Niagara|SpawnSystemAttached "/Game/Art/VFX/NS_MuzzleFlash.NS_MuzzleFlash" 0 "None" "0.000000,35.000000,10.000000" "0.000000,45.000000,0.000000" "KeepRelativeOffset" false)
  (Physics|AddImpulse (Variables|/Game/Blueprints/Damaging/BP_Damager.BP_Damager_C|GetCollider _returnvalue_5) (* (Math|Vector|GetUnitDirection(Vector) (Transformation|GetSocketLocation (Variables|/Script/Engine.Character|GetMesh CharacterRef) "GunSpawn") _returnvalue_4) 3e+03) "None" true))

(event Custom|Super%20Attack
  ;[1 0.2292 0.2292] super attack
  (Game|SpawnActorfromClass "/Game/Art/VFX/NS_KickSlash/BP_GroundSlash.BP_GroundSlash_C" (Transformation|GetActorTransform self) "Undefined" "MultiplyWithRoot" 0 0))

(fn ConstructionScript
  (|CallParentFunction))