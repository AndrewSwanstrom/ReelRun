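; BP_PhotoMode is a possessable photo mode camera actor that shows a camera widget and lets the player take screenshots.
; A very high CustomTimeDilation offsets the global time dilation, which is reset to normal on exit.
; Taking a photo saves a high-res screenshot named from date and counter, with a brief flash widget.
; The photo mode input hands possession back to Base_Character, clears its InPhotoMode flag and destroys this actor.
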(event Input|EnhancedActionEvents|EnhancedInputActionIA_PhotoMode
  (params (ActionValue :type Boolean) (ElapsedSeconds :type Float%20%28double-precision%29) (TriggeredSeconds :type Float%20%28double-precision%29) (InputAction :type Input%20Action%20Object%20Reference :default "/Game/Blueprints/Input/Actions/IA_PhotoMode.IA_PhotoMode"))
  (:Started
    (bind _returnvalue (Actor|GetActorOfClass "/Game/Blueprints/Characters/Base_Character.Base_Character_C"))
    (Variables|/Game/Blueprints/Characters/Base_Character.Base_Character_C|SetbInPhotoMode _returnvalue false)
    (Utilities|Time|SetGlobalTimeDilation 1.0)
    (Pawn|Possess (Game|GetPlayerController 0) _returnvalue)
    (Actor|DestroyActor)))

(event Input|EnhancedActionEvents|EnhancedInputActionIA_TakePhoto
  (params (ActionValue :type Boolean) (ElapsedSeconds :type Float%20%28double-precision%29) (TriggeredSeconds :type Float%20%28double-precision%29) (InputAction :type Input%20Action%20Object%20Reference :default "/Game/Blueprints/Input/Actions/IA_TakePhoto.IA_TakePhoto"))
  (bind _returnvalue (Math|DateTime|Now))
  (bind _photoid (Variables|Default|GetPhotoID))
  (bind (_year _month _day) (Math|DateTime|BreakDateTime _returnvalue))
  (:Triggered
    (bind _returnvalue_2 (UserInterface|CreateWidget "/Game/Blueprints/UI/photomode/BPW_PhotoFlash.BPW_PhotoFlash_C"))
    (UserInterface|Viewport|AddtoViewport _returnvalue_2 0)
    (Utilities|FlowControl|Delay 1.0)
    (Widget|RemovefromParent _returnvalue_2))
  (:Started
    (Class|AutomationBlueprintFunctionLibrary|TakeHighResScreenshot 1920 1080 (Utilities|String|Append (Utilities|String|ToString(Integer) _year) (Utilities|String|ToString(Integer) _month) (Utilities|String|ToString(Integer) _day) (Utilities|String|ToString(Integer) _photoid)) 0 false false "Low" "" 0.0)
    (Math|Integer|IncrementInt _photoid)))

(event EventBeginPlay
  (Input|AddMappingContext (PlayerController|LocalPlayerSubsystems|GetEnhancedInputLocalPlayerSubsystem (Game|GetPlayerController 0)) 0 0 "(bIgnoreAllPressedKeysUntilRelease=True,bForceImmediately=False,bNotifyUserSettings=False)")
  (Variables|Default|SetCustomTimeDilation 1e+04)
  (bind _returnvalue (UserInterface|CreateWidget "/Game/Blueprints/UI/photomode/BPW_Cam.BPW_Cam_C"))
  (UserInterface|Viewport|AddtoViewport _returnvalue 0))

(event EventPossessed
  (params (NewController :type Controller%20Object%20Reference)))

(fn ConstructionScript)