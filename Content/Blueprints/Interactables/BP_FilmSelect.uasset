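; BP_FilmSelect is an interactable film projector actor that builds its projection from three cone lights, one per RGB channel.
; The Construction Script gives each light a dynamic light function material that picks its channel, tinted by LightColor, and applies shared editable intensity, radius, scattering, cone and temperature settings.
; InteractAction and IsInside only print debug text, and the media-opening call is unconnected.
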(event EventBeginPlay
  (|CallParentFunction) ; This node is disabled and will not be called.\nDrag off pins to build functionality.
)

(event Collision|EventActorBeginOverlap
  (params (OtherActor :type Actor%20Object%20Reference)))

(event EventTick
  (params (DeltaSeconds :type Float%20%28single-precision%29)))

(event EventInteractAction
  (Development|PrintString "um. unreal?"))

(event EventIsInside
  (params (IN :type Boolean))
  (Development|PrintString (Utilities|String|ToString(Boolean) IN)))

(fn ConstructionScript
  (bind _projectionsize (Variables|Default|GetProjectionSize))
  ;[1 1 1] Select RGB Channel for each light
  (for _index (range 0 2)
    (bind _returnvalue (Rendering|Material|CreateDynamicMaterialInstance (Variables|Default|GetLightFunctionMaterial) "None" "None" :!class /Script/Engine.KismetMaterialLibrary))
    (Rendering|Material|SetVectorParameterValue _returnvalue "ChannelPick" (* (Utilities|Select :Index _index :Option%200 "(R=1.000000,G=0.000000,B=0.000000,A=1.000000)" :Option%201 "(R=0.000000,G=1.000000,B=0.000000,A=1.000000)" :Option%202 "(R=0.000000,G=0.000000,B=1.000000,A=1.000000)") (Variables|Default|GetLightColor)) :!class /Script/Engine.MaterialInstanceDynamic)
    (Rendering|Components|Light|SetLightFunctionMaterial (Utilities|Select :Index _index :Option%200 (Variables|Default|GetR) :Option%201 (Variables|Default|GetG) :Option%202 (Variables|Default|GetB)) _returnvalue)
    ;[1 1 1] Editable Variables
    (Rendering|Components|Light|SetIntensity (Utilities|Select :Index _index :Option%200 (Variables|Default|GetR) :Option%201 (Variables|Default|GetG) :Option%202 (Variables|Default|GetB)) (Variables|Default|GetNew%20Intensity))
    (Rendering|Lighting|SetAttenuationRadius (Utilities|Select :Index _index :Option%200 (Variables|Default|GetR) :Option%201 (Variables|Default|GetG) :Option%202 (Variables|Default|GetB)) (Variables|Default|GetNew%20Radius))
    (Class|LightComponent|SetVolumetricScatteringIntensity (Utilities|Select :Index _index :Option%200 (Variables|Default|GetR) :Option%201 (Variables|Default|GetG) :Option%202 (Variables|Default|GetB)) (Variables|Default|GetNew%20Volumetric%20Scattering%20Intensity))
    (Rendering|Lighting|SetOuterConeAngle (Utilities|Select :Index _index :Option%200 (Variables|Default|GetR) :Option%201 (Variables|Default|GetG) :Option%202 (Variables|Default|GetB)) _projectionsize)
    (Rendering|Lighting|SetInnerConeAngle (Utilities|Select :Index _index :Option%200 (Variables|Default|GetR) :Option%201 (Variables|Default|GetG) :Option%202 (Variables|Default|GetB)) _projectionsize)
    (Class|LightComponent|SetTemperature (Utilities|Select :Index _index :Option%200 (Variables|Default|GetR) :Option%201 (Variables|Default|GetG) :Option%202 (Variables|Default|GetB)) (Variables|Default|GetNew%20Temperature))))