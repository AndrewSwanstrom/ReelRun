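; BP_Lunchtray is a lunch tray prop that randomizes its look at runtime so placed copies vary.
; On BeginPlay, it gives the tray mesh a slight random yaw and sometimes destroys the apple and plate components.
; It then randomly swaps cutlery for spoons, the water bottle for cans or a cup, and any surviving apple for chips or Spam.
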(event EventBeginPlay
  (bind _sm_waterbottle (Variables|Default|GetSM_WaterBottle))
  (bind _sm_apple_01 (Variables|Default|GetSM_Apple_01))
  (Utilities|FlowControl|DoOnce false
    (:Completed
      (Transformation|SetRelativeRotation (Variables|Default|GetSM_LunchTray) (Math|Rotator|MakeRotator 0.0 0.0 (Math|Conversions|ToFloat(Integer) (Math|Random|RandomIntegerinRange -10 10))) false false)
      (switch int (Math|Random|RandomIntegerinRange 0 2)
        (:Default
          _)
        (:0
          _)
        (:1
          (Components|DestroyComponent (Variables|Default|GetSM_Apple_01))
          (Components|DestroyComponent (Variables|Default|GetSM_Plate)))
        (:2
          _))
      (Utilities|FlowControl|Sequence
        (:then_0
          (switch int (Math|Random|RandomIntegerinRange 0 1)
            (:0
              (Components|StaticMesh|SetStaticMesh (Variables|Default|GetSM_Fork) "/Game/Art/Environment/Horror/Clutter/MessHall/SM_Spoon.SM_Spoon"))))
        (:then_1
          (switch int (Math|Random|RandomIntegerinRange 0 1)
            (:0
              (Components|StaticMesh|SetStaticMesh (Variables|Default|GetSM_Knife) "/Game/Art/Environment/Horror/Clutter/MessHall/SM_Spoon.SM_Spoon"))))
        (:then_2
          (switch int (Math|Random|RandomIntegerinRange 0 3)
            (:0
              (Components|StaticMesh|SetStaticMesh _sm_waterbottle "/Game/Art/Environment/Horror/Clutter/MessHall/SM_SodaCan_02.SM_SodaCan_02"))
            (:1
              (Components|StaticMesh|SetStaticMesh _sm_waterbottle "/Game/Art/Environment/Horror/Clutter/MessHall/SM_SodaCan_01.SM_SodaCan_01"))
            (:2
              (Components|StaticMesh|SetStaticMesh _sm_waterbottle "/Game/Art/Environment/Horror/Clutter/MessHall/SM_PaperCup.SM_PaperCup"))))
        (:then_3
          (Utilities|IsValid (Variables|Default|GetSM_Apple_01)
            (:Is%20Valid
              (switch int (Math|Random|RandomIntegerinRange 0 2)
                (:0
                  (Components|StaticMesh|SetStaticMesh _sm_apple_01 "/Game/Art/Environment/Horror/Clutter/MessHall/SM_OpenChips.SM_OpenChips"))
                (:1
                  (Components|StaticMesh|SetStaticMesh _sm_apple_01 "/Game/Art/Environment/Horror/Clutter/Outside/SM_SpamCan.SM_SpamCan"))))))))))

(fn ConstructionScript)