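; BP_Piano is a piano actor that shows when the character can interact with it.
; Box overlap begin and end toggle InRange, then for a Base_Character set its NearPiano flag, show or hide InteractIcon and apply or clear an outline overlay material on the mesh.
; While InRange, Tick rotates the icon to face the player camera.
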(event OnComponentEndOverlap(Box)
  (params (OverlappedComponent :type Primitive%20Component%20Object%20Reference) (OtherActor :type Actor%20Object%20Reference) (OtherComp :type Primitive%20Component%20Object%20Reference) (OtherBodyIndex :type Integer))
  (Variables|Default|SetInRange false)
  (bind _asbase_character (Utilities|Casting|CastToBase_Character OtherActor))
  (Variables|/Game/Blueprints/Characters/Base_Character.Base_Character_C|SetNearPiano _asbase_character false)
  (Rendering|SetVisibility (Variables|Default|GetInteractIcon) false false)
  (Rendering|Material|SetOverlayMaterial (Variables|Default|GetSM_Piano_01a) 0 :!class /Script/Engine.MeshComponent))

(event OnComponentBeginOverlap(Box)
  (params (OverlappedComponent :type Primitive%20Component%20Object%20Reference) (OtherActor :type Actor%20Object%20Reference) (OtherComp :type Primitive%20Component%20Object%20Reference) (OtherBodyIndex :type Integer) (bFromSweep :type Boolean) (SweepResult :type Hit%20Result%20Structure%20%28by%20ref%29))
  (Variables|Default|SetInRange true)
  (bind _asbase_character (Utilities|Casting|CastToBase_Character OtherActor))
  (Variables|/Game/Blueprints/Characters/Base_Character.Base_Character_C|SetNearPiano _asbase_character true)
  (Rendering|SetVisibility (Variables|Default|GetInteractIcon) true false)
  (Rendering|Material|SetOverlayMaterial (Variables|Default|GetSM_Piano_01a) "/Game/Materials/OutlineMat/Mi_OutlineMat_Inst.Mi_OutlineMat_Inst" :!class /Script/Engine.MeshComponent))

(event EventTick
  (params (DeltaSeconds :type Float%20%28single-precision%29))
  (bind _interacticon (Variables|Default|GetInteractIcon))
  (if (Variables|Default|GetInRange)
    (Transformation|SetWorldRotation _interacticon (Math|Rotator|FindLookatRotation (Transformation|GetWorldLocation _interacticon) (Transformation|GetWorldLocation (Variables|/Script/Engine.PlayerCameraManager|GetTransformComponent (Game|GetPlayerCameraManager 0)))) false false)))

(fn ConstructionScript)